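; Prototype actor for testing hit-damage painting on a skeletal mesh.
; BeginPlay puts a dynamic material instance on slot 0 and sets its RTDamage texture parameter, with no texture shown.
; Paint temporarily swaps in M_UVUnwrap, passes it an offset root position, hit location and radius, then immediately restores the original material.
; The graph contains no capture or draw-to-render-target step between swap and restore.
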(event `self.ReceiveTick`
  (params (DeltaSeconds :type "Float (single-precision)")))

(event `self.ReceiveBeginPlay`
  (bind _skeletal (`self.Skeletal`))
  (bind _returnvalue (`PrimitiveComponent.CreateDynamicMaterialInstance` _skeletal 0 (`PrimitiveComponent.GetMaterial` _skeletal 0) "None"))
  (`PrimitiveComponent.SetMaterial` _skeletal 0 _returnvalue)
  (`MaterialInstanceDynamic.SetTextureParameterValue` _returnvalue "RTDamage" null))

(fn `Paint`
  (params (HitLocation :type "Vector Structure") (Radius :type "Float (double-precision)"))
  (bind _skeletal (`self.Skeletal`))
  (`|ExecutionSequence`
    (:`then_0`
      (set `self.Old_Material` (`PrimitiveComponent.GetMaterial` _skeletal 0))
      (`PrimitiveComponent.SetMaterial` _skeletal 0 "/Game/Materials/BaseMaterials/Misc/M_UVUnwrap.M_UVUnwrap")
      (`MeshComponent.SetVectorParameterValueOnMaterials` _skeletal "Position" (+ (`SceneComponent.K2_GetComponentLocation` (`self.DefaultSceneRoot`)) (0.0 0.0 10.0)))
      (`MeshComponent.SetVectorParameterValueOnMaterials` _skeletal "HitLocation" HitLocation)
      (`MeshComponent.SetScalarParameterValueOnMaterials` _skeletal "Radius" Radius))
    (:`then_1`
      (`PrimitiveComponent.SetMaterial` _skeletal 0 (`self.Old_Material`)))))

(fn `UserConstructionScript`)