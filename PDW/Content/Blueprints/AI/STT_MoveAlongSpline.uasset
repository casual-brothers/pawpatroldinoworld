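; StateTree task that moves an actor along a spline and finishes successfully at the end.
; Each latent tick places the actor at the current world-space distance along the spline, without sweeping, then advances that distance by the movement speed.
; The step is per tick, not scaled by delta time.
; On reaching the spline length, it resets the distance to zero and completes.
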(event `self.ReceiveLatentTick`
  (params (DeltaTime :type "Float (single-precision)"))
  (`Actor.K2_SetActorLocation` (`self.inActor`) (`SplineComponent.GetLocationAtDistanceAlongSpline` (`self.inSpline`) (`self.Distance`) "World") false false)
  (if (< (`self.Distance`) (`SplineComponent.GetSplineLength` (`self.inSpline`)))
    (set `self.Distance` (+ (`self.Distance`) (`self.MovementSpeed`)))
    (else
      (set `self.Distance` 0.0)
      (`self.FinishTask` true))))