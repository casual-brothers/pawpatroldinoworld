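; State Tree task that makes an AI actor find, claim and use a nearby Smart Object.
; On enter, it queries a box around the user actor and claims the first slot returned, without checking the claim handle.
; An async move-and-use gameplay behavior node then finishes the task as succeeded or failed; an empty search fails immediately.
; The GetRandomOne helper picks a random array entry but is not called here.
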(event `self.ReceiveLatentEnterState`
  (params (Transition :type "StateTreeTransitionResult Structure (by ref)"))
  (bind _user_actor (`self.User Actor`))
  (bind _user_actor_2 (`self.User Actor`))
  (bind (_outresults _returnvalue) (`SmartObjectSubsystem.FindSmartObjects_BP` (subsystem `SmartObjectSubsystem`) (make `SmartObjectRequest` (`KismetMathLibrary.MakeBoxWithOrigin` (`Actor.K2_GetActorLocation` _user_actor_2) (1000.0 1000.0 1000.0)) (make `SmartObjectRequestFilter` (struct))) _user_actor_2))
  (if _returnvalue
    (bind _returnvalue_2 (`SmartObjectBlueprintFunctionLibrary.MarkSmartObjectSlotAsClaimed` (`.SlotHandle` (break `SmartObjectRequestResult` (`|GetArrayItem` _outresults))) _user_actor))
    (`AITask_UseGameplayBehaviorSmartObject.MoveToAndUseSmartObjectWithGameplayBehavior` (`AIBlueprintHelperLibrary.GetAIController` _user_actor) _returnvalue_2
      (:`OnSucceeded`
        (`self.FinishTask` true))
      (:`OnFailed`
        (`self.FinishTask` false :!label _label))
      (:`OnMoveToFailed`
        (goto _label)))
    (else
      (`self.FinishTask` false))))

(fn `GetRandomOne`
  (params (inSO :type "Array of SmartObjectRequestResult Structure"))
  (returns (NewParam :type "SmartObjectRequestResult Structure"))
  (return (`|GetArrayItem` inSO (`KismetMathLibrary.RandomInteger` (- (`KismetArrayLibrary.Array_Length` inSO) 1)))))