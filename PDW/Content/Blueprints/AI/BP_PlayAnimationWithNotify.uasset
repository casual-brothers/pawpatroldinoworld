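; State Tree task that plays a tag-selected montage on a dino and fires a Smart Object use event when a chosen notify begins.
; It async-loads the montage looked up from the PDW dino anim instance, then plays it on the owner's skeletal mesh.
; Completion succeeds the task and interruption fails it.
; Without a valid montage, it finishes successfully and sends the event immediately to the claimed slot.
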(event `self.ReceiveLatentEnterState`
  (params (Transition :type "StateTreeTransitionResult Structure (by ref)"))
  (bind (_soclaimhandle_smartobjecthandle _soclaimhandle_slothandle) (break `SmartObjectClaimHandle` (`self.SOClaimHandle`)))
  (bind _returnvalue (`Actor.GetComponentByClass` (`self.Owner`) "/Script/Engine.SkeletalMeshComponent"))
  (bind _aspdwdino_anim_instance (cast `PDWDinoAnimInstance` (`SkeletalMeshComponent.GetAnimInstance` _returnvalue)))
  (bind _returnvalue_2 (`PDWAnimInstance.GetMontageByTag` _aspdwdino_anim_instance (`self.AnimationToPlay`)))
  (if (`KismetSystemLibrary.IsValidSoftObjectReference` _returnvalue_2)
    (bind _object (`|LoadAsset` _returnvalue_2)
      (:`Completed`
        (bind _asanim_montage (cast `AnimMontage` _object))
        (bind _notifyname (`|PlayMontage` _returnvalue _asanim_montage)
          (:`OnCompleted`
            (`self.FinishTask` true))
          (:`OnInterrupted`
            (`self.FinishTask` false))
          (:`OnNotifyBegin`
            (if (== _notifyname (`self.NotifyToWait`))
              (`PDWGameplayFunctionLibrary.SendSmartObjectEvent` self _soclaimhandle_slothandle (`PDWGameplayTagSettings.GetSOUseEvent`) (`self.Owner`) :!label _label))))))
    (else
      (`self.FinishTask` true)
      (goto _label))))