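; Broken button interactable that switches to its fixed appearance once it has been repaired.
; When the InteractionReceiverComponent finishes a behaviour in the Repaired state, it resizes its capsule, hides the Niagara effect and resets the mesh's rotation and relative position.
; The construction script only calls the parent's, and all other events are empty.
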(event `self.InteractionReceiverComponent.OnBehaviourFinished`
  (params (Behaviour :type "PDWInteractionBehaviour Object Reference"))
  (bind _interactionreceivercomponent (`self.InteractionReceiverComponent`))
  (bind _staticmesh (`self.StaticMesh`))
  (if (== (`PDWInteractionReceiverComponent.GetCurrentState` (`self.InteractionReceiverComponent`)) (struct :`TagName` "InteractionState.Repaired"))
    (`CapsuleComponent.SetCapsuleRadius` _interactionreceivercomponent 30.0 true)
    (`CapsuleComponent.SetCapsuleHalfHeight` _interactionreceivercomponent 30.0 true)
    (`SceneComponent.SetHiddenInGame` (`self.Niagara`) true false)
    (`SceneComponent.K2_SetRelativeRotation` :`self` _staticmesh)
    (`SceneComponent.K2_SetRelativeLocation` _staticmesh (0.0 0.0 -15.0) false false)))

(fn `UserConstructionScript`
  (`parent.UserConstructionScript`))