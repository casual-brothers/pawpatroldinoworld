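; Interactable seashell actor that adjusts its interaction capsule once it has been opened.
; When its InteractionReceiverComponent finishes a behaviour in the Opened state, it sets that component's capsule to a fixed radius and half height, updating overlaps.
; BeginPlay, overlap and Tick events are unused, and the construction script only calls its parent.
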(event `self.InteractionReceiverComponent.OnBehaviourFinished`
  (params (Behaviour :type "PDWInteractionBehaviour Object Reference"))
  (bind _interactionreceivercomponent (`self.InteractionReceiverComponent`))
  (if (== (`PDWInteractionReceiverComponent.GetCurrentState` (`self.InteractionReceiverComponent`)) (struct :`TagName` "InteractionState.Opened"))
    (`CapsuleComponent.SetCapsuleRadius` _interactionreceivercomponent 60.0 true)
    (`CapsuleComponent.SetCapsuleHalfHeight` _interactionreceivercomponent 60.0 true)))

(fn `UserConstructionScript`
  (`parent.UserConstructionScript`))