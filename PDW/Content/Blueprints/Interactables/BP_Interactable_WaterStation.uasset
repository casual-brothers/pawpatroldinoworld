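; Interactable water station that Smart Object users can use while its handler still holds water.
; When a Smart Object event matches the use tag, it forwards the interactor and behaviour identifier to the interaction receiver component.
; It adds or removes itself as a Smart Object based on remaining water at init, BeginPlay and slot release.
; The water station handler's update event also toggles that registration, apparently on player interaction.
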(event `self.PDWWaterStationHandler.OnInit`
  (`self.HandleSmartObjectActivity`))

(event `self.ReceiveBeginPlay`
  (add `SmartObjectComponent.OnSmartObjectEvent` (`self.SmartObject`) (delegate `SOEvent`))
  (add `PDWWaterStationHandler.OnSmartObjectUpdate` (`self.PDWWaterStationHandler`) (delegate `SOUpdateOnPlayerInteraction`))
  (`self.HandleSmartObjectActivity`))

(event `SOUpdateOnPlayerInteraction`
  (params (IsActive :type Boolean))
  (`SmartObjectBlueprintFunctionLibrary.AddOrRemoveSmartObject` self IsActive))

(event `SOEvent`
  (params (EventData :type "SmartObjectEventData Structure (by ref)") (Interactor :type "Actor Object Reference"))
  (switch `ESmartObjectChangeReason` EventData_Reason
    (:`OnEvent`
      (if (== (`PDWGameplayTagSettings.GetSOUseEvent`) EventData_Tag)
        (`PDWInteractionReceiverComponent.ProcessInteraction` (`self.InteractionReceiverComponent`) (make `PDWInteractionPayload` Interactor (struct) (`BlueprintGameplayTagLibrary.MakeGameplayTagContainerFromArray` (`|MakeArray` (`self.Behaviour Identifier`)))))))
    (:`OnReleased`
      (`self.HandleSmartObjectActivity`))))

(event `HandleSmartObjectActivity`
  (`SmartObjectBlueprintFunctionLibrary.AddOrRemoveSmartObject` self (not (<= (`PDWWaterStationHandler.GetCurrentWater` (`self.PDWWaterStationHandler`)) 0.0))))

(fn `UserConstructionScript`
  (`parent.UserConstructionScript`))