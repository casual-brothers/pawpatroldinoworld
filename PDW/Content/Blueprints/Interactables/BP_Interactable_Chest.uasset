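; Interactable chest Blueprint that restores its used state on BeginPlay and drops its visual cues after interaction.
; BeginPlay looks up the receiver component's interactable ID; used chests get the inactive tag, single-node animation and hidden Niagara effect.
; Unused chests run their Animation Blueprint.
; When any receiver behaviour finishes, it hides the Niagara effect, clears the overlay material and zeroes the custom depth stencil.
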(event `self.ReceiveBeginPlay`
  (`parent.ReceiveBeginPlay`)
  (bind _returnvalue (`PDWDataFunctionLibrary.IsInteractableUsed` self (`PDWInteractionReceiverComponent.GetInteractableID` (`self.InteractionReceiverComponent`))))
  (if _returnvalue
    (`PDWInteractionReceiverComponent.AddStateTag` (`self.InteractionReceiverComponent`) (`self.InactiveTag`))
    (`SkeletalMeshComponent.SetAnimationMode` (`self.SkeletalMesh`) "AnimationSingleNode" false)
    (`SceneComponent.SetHiddenInGame` (`self.Niagara`) true false)
    (else
      (`SkeletalMeshComponent.SetAnimationMode` (`self.SkeletalMesh`) "AnimationBlueprint" false))))

(event `self.InteractionReceiverComponent.OnBehaviourFinished`
  (params (Behaviour :type "PDWInteractionBehaviour Object Reference"))
  (bind _skeletalmesh (`self.SkeletalMesh`))
  (`SceneComponent.SetHiddenInGame` (`self.Niagara`) true false)
  (`MeshComponent.SetOverlayMaterial` _skeletalmesh null)
  (`PrimitiveComponent.SetCustomDepthStencilValue` _skeletalmesh 0))

(fn `UserConstructionScript`
  (`parent.UserConstructionScript`))