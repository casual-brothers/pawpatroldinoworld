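; BP_Interactable_BouncingLeaf is an interactable bouncing leaf that toggles a Niagara growth-success glow based on its interaction state.
; When its InteractionReceiverComponent finishes a Bouncing behaviour, the glow deactivates and a "Deactive" debug string prints.
; When any other behaviour finishes, the glow activates if the receiver's current state is Grown.
; The other receiver events are empty, and the construction script only calls its parent.
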(event `self.InteractionReceiverComponent.OnBehaviourFinished`
  (params (Behaviour :type "PDWInteractionBehaviour Object Reference"))
  (if (== (`PDWInteractionBehaviour.BehaviourIdentifier` Behaviour) (struct :`TagName` "InteractionBehaviour.Bouncing"))
    (`ActorComponent.SetActive` (`self.NS_Interactable_LeafGrowth_SuccessGlow`) false false)
    (`KismetSystemLibrary.PrintString` "Deactive")
    (elif (== (`PDWInteractionReceiverComponent.GetCurrentState` (`self.InteractionReceiverComponent`)) (struct :`TagName` "InteractionState.Grown"))
      (`ActorComponent.SetActive` (`self.NS_Interactable_LeafGrowth_SuccessGlow`) true false))))

(event `self.InteractionReceiverComponent.OnInteractionSuccessful`
  (params (Payload :type "PDWInteractionPayload Structure (by ref)")))

(event `self.InteractionReceiverComponent.OnInteract`
  (params (Payload :type "PDWInteractionPayload Structure (by ref)")))

(event `self.InteractionReceiverComponent.OnComponentDeactivated`
  (params (Component :type "ActorComponent Object Reference")))

(fn `UserConstructionScript`
  (`parent.UserConstructionScript`))