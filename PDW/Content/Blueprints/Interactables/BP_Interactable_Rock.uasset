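; Interactable rock Blueprint that varies its size and orientation at BeginPlay, after calling the parent's BeginPlay.
; An optional random multiplier scales the InteractionReceiverComponent's relative scale and location together.
; Each rotation axis has its own randomize flag, with SelectFloat keeping the existing angle on axes left off.
; The variation is unseeded and applied only at runtime, as the construction script just calls the parent.
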(event `self.ReceiveBeginPlay`
  (bind _randomizerotationx (`self.RandomizeRotationX`))
  (bind _randomizerotationy (`self.RandomizeRotationY`))
  (bind _randomizerotationz (`self.RandomizeRotationZ`))
  (bind _interactionreceivercomponent (`self.InteractionReceiverComponent`))
  (bind (_relativerotation_roll _relativerotation_pitch _relativerotation_yaw) (`KismetMathLibrary.BreakRotator` (`SceneComponent.RelativeRotation` _interactionreceivercomponent)))
  (`parent.ReceiveBeginPlay`)
  (`|ExecutionSequence`
    (:`then_0`
      (if (`self.RandomizeScale`)
        (set `self.ScaleMultiplier` (`KismetMathLibrary.RandomFloatInRange` 0.7 1.3))
        (`SceneComponent.SetRelativeScale3D` _interactionreceivercomponent (* (`SceneComponent.RelativeScale3D` _interactionreceivercomponent) (`self.ScaleMultiplier`)))
        (`SceneComponent.K2_SetRelativeLocation` _interactionreceivercomponent (* (`SceneComponent.RelativeLocation` _interactionreceivercomponent) (`self.ScaleMultiplier`)) false false)))
    (:`then_1`
      (if (or _randomizerotationx _randomizerotationy _randomizerotationz)
        (`SceneComponent.K2_SetRelativeRotation` _interactionreceivercomponent (`KismetMathLibrary.MakeRotator` (`KismetMathLibrary.SelectFloat` (`KismetMathLibrary.Conv_IntToDouble` (`KismetMathLibrary.RandomIntegerInRange` 0 360)) _relativerotation_roll _randomizerotationx) (`KismetMathLibrary.SelectFloat` (`KismetMathLibrary.Conv_IntToDouble` (`KismetMathLibrary.RandomIntegerInRange` 0 360)) _relativerotation_pitch _randomizerotationy) (`KismetMathLibrary.SelectFloat` (`KismetMathLibrary.Conv_IntToDouble` (`KismetMathLibrary.RandomIntegerInRange` 0 360)) _relativerotation_yaw _randomizerotationz)) false false)))))

(fn `UserConstructionScript`
  (`parent.UserConstructionScript`))