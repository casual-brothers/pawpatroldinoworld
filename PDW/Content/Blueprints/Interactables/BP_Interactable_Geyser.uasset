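; Interactable geyser actor that reacts to a breaking interaction by showing an anticipation effect.
; Its InteractionReceiverComponent reports successful interactions, and a Breaking behaviour identifier activates the NSGeyserAnticipation effect without resetting it.
; The file holds no eruption logic: overlap only calls the parent, and the capsule resize and debug print nodes never run.
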(event `self.ReceiveActorBeginOverlap`
  (params (OtherActor :type "Actor Object Reference"))
  (`parent.ReceiveActorBeginOverlap` OtherActor))

(event `self.InteractionReceiverComponent.OnInteractionSuccessful`
  (params (Payload :type "PDWInteractionPayload Structure (by ref)"))
  (if (== Payload_BehaviourExecutedIdentifier (struct :`TagName` "InteractionBehaviour.Breaking"))
    (`ActorComponent.SetActive` (`self.NS_GeyserAnticipation`) true false)))

(fn `UserConstructionScript`
  (`parent.UserConstructionScript`))