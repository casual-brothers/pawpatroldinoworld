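; Grown variant of the bouncing leaf interactable, which turns off its growth success glow once a bounce interaction finishes.
; It listens for the interaction receiver component's behaviour-finished event and, when the behaviour is Bouncing, deactivates the leaf growth success glow effect.
; BeginPlay, overlap and Tick are disabled stubs, and the construction script only calls the parent.
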(event `self.InteractionReceiverComponent.OnBehaviourFinished`
  (params (Behaviour :type "PDWInteractionBehaviour Object Reference"))
  (if (== (`PDWInteractionBehaviour.BehaviourIdentifier` Behaviour) (struct :`TagName` "InteractionBehaviour.Bouncing"))
    (`ActorComponent.SetActive` (`self.NS_Interactable_LeafGrowth_SuccessGlow`) false false)))

(fn `UserConstructionScript`
  (`parent.UserConstructionScript`))