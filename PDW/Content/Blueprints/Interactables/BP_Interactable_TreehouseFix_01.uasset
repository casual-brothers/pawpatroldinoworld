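; Interactable treehouse repair actor that switches from broken to repaired collision once an interaction completes.
; When its InteractionReceiverComponent reports any finished behaviour, it enables query and physics collision on CollisionRepaired and disables CollisionBroken.
; If that behaviour is Shining, it also resets the static mesh's custom depth stencil value to zero.
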(event `self.InteractionReceiverComponent.OnBehaviourFinished`
  (params (Behaviour :type "PDWInteractionBehaviour Object Reference"))
  (`PrimitiveComponent.SetCollisionEnabled` (`self.CollisionRepaired`) "QueryAndPhysics")
  (`PrimitiveComponent.SetCollisionEnabled` (`self.CollisionBroken`) "NoCollision")
  (if (== (`PDWInteractionBehaviour.BehaviourIdentifier` Behaviour) (struct :`TagName` "InteractionBehaviour.Shining"))
    (`PrimitiveComponent.SetCustomDepthStencilValue` (`self.StaticMesh`) 0)))

(fn `UserConstructionScript`
  (`parent.UserConstructionScript`))