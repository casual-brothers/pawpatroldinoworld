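; BP_Interactable_Heap is an interactable heap that can trigger a follow-up behaviour once it is cleaned.
; When its InteractionReceiverComponent finishes a Cleaning behaviour, it checks for the TriggerInteractionState tag and a non-empty Targets list.
; If both hold, it executes TargetsBehaviourIdentifier through that same component.
; The construction script only calls the parent's.
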(event `self.InteractionReceiverComponent.OnBehaviourFinished`
  (params (Behaviour :type "PDWInteractionBehaviour Object Reference"))
  (if (and (== (`PDWInteractionBehaviour.BehaviourIdentifier` Behaviour) (struct :`TagName` "InteractionBehaviour.Cleaning")) (`PDWInteractionReceiverComponent.HasStateTag` (`self.InteractionReceiverComponent`) (`self.TriggerInteractionState`)) (> (`KismetArrayLibrary.Array_Length` (`self.Targets`)) 0))
    (`PDWInteractionReceiverComponent.ExecuteInteractionBehaviour` (`self.InteractionReceiverComponent`) (`self.TargetsBehaviourIdentifier`) null false false)))

(fn `UserConstructionScript`
  (`parent.UserConstructionScript`))