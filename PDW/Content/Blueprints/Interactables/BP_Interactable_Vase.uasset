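; Interactable vase actor that switches between repaired and broken states through its InteractionReceiverComponent.
; It caches the state tag when an interaction starts and compares it to the current one when the behaviour finishes, reacting only to transitions.
; Becoming repaired shows the static mesh and sets a tall interaction capsule.
; Becoming broken runs a deactivation behaviour, hides the mesh and sets a shorter capsule.
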(event `self.InteractionReceiverComponent.OnInteract`
  (params (Payload :type "PDWInteractionPayload Structure (by ref)"))
  (set `self.PreviousState` (`PDWInteractionReceiverComponent.GetCurrentState` (`self.InteractionReceiverComponent`))))

(event `self.InteractionReceiverComponent.OnBehaviourFinished`
  (params (Behaviour :type "PDWInteractionBehaviour Object Reference"))
  (bind _interactionreceivercomponent (`self.InteractionReceiverComponent`))
  (bind _repairedstate (`self.RepairedState`))
  (bind _brokenstate (`self.BrokenState`))
  (bind _returnvalue (`PDWInteractionReceiverComponent.GetCurrentState` _interactionreceivercomponent))
  (if (and (not (`BlueprintGameplayTagLibrary.MatchesTag` (`self.PreviousState`) _repairedstate)) (`BlueprintGameplayTagLibrary.MatchesTag` _returnvalue _repairedstate))
    (`CapsuleComponent.SetCapsuleSize` (`self.InteractionReceiverComponent`) 100.0 200.0 true)
    (`SceneComponent.SetHiddenInGame` (`self.StaticMesh`) false false)
    (elif (and (`BlueprintGameplayTagLibrary.MatchesTag` _returnvalue _brokenstate) (not (`BlueprintGameplayTagLibrary.MatchesTag` (`self.PreviousState`) _brokenstate)))
      (`PDWInteractionReceiverComponent.ExecuteInteractionBehaviour` _interactionreceivercomponent (`self.DeactivationBehaviourTag`) null false false)
      (`CapsuleComponent.SetCapsuleSize` (`self.InteractionReceiverComponent`) 100.0 100.0 true)
      (`SceneComponent.SetHiddenInGame` (`self.StaticMesh`) true false))))

(fn `UserConstructionScript`
  (`parent.UserConstructionScript`))