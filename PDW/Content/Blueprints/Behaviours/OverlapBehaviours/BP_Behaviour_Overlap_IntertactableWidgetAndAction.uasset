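; Overlap behaviour that shows an interaction widget and adds the interact input map for the player who triggers it.
; It acts only when the receiver component's state matches InteractableState, with a gameplay tag check also gating the start.
; Tagged P1/P2 widget components are assigned to the matching local player for split per-player prompts.
; Ending reverts both, as does minigame initialization after a successful interaction, or success itself when ResetInteractionInputAfterSuccess is set.
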(event `self.BP_ExecuteBehaviour_Implementation`
  (if (`self.CheckState`)
    (bind _conditionmet (`self.GameplayTagCheck`))
    (if (not _conditionmet)
      (`self.ToggleInteractionInputMap` true)
      (`self.ToggleInteractionMessage` false))))

(event `self.BP_EndBehaviour_Implementation`
  (if (`self.CheckState`) :!label _label
    (`self.ToggleInteractionInputMap` false :!label _label_2)
    (`self.ToggleInteractionMessage` true)))

(event `HideUIOnInizialitazionComplete`
  (params (Controllers :type "Array of PDWPlayerController Object Reference (by ref)"))
  (goto _label))

(event `self.BP_OnInteractionSuccessfull_Implementation`
  (if (`self.CheckState`)
    (bind _returnvalue (`self.GetOwnerComponent`))
    (add `PDWMinigameConfigComponent.OnMinigameInitializationComplete` (`Actor.GetComponentByClass` (`ActorComponent.GetOwner` _returnvalue) "/Script/PDW.PDWMinigameConfigComponent") (delegate `HideUIOnInizialitazionComplete`))
    (if (`self.ResetInteractionInputAfterSuccess`)
      (goto _label_2))))

(fn `CheckState`
  (returns (bIsState :type Boolean))
  (bind _interactable_state (`self.Interactable State`))
  (bind _returnvalue (`self.GetOwnerComponent`))
  (bind _returnvalue_2 (`Actor.GetComponentByClass` (`ActorComponent.GetOwner` _returnvalue) "/Game/Blueprints/Pawn/Components/BP_InteractionReceiverComponent.BP_InteractionReceiverComponent_C"))
  (`/Engine/EditorBlueprintResources/StandardMacros.IsValid` _returnvalue_2
    (:`Is Valid`
      (return (or (== _interactable_state (struct)) (== _interactable_state (`PDWInteractionReceiverComponent.GetCurrentState` _returnvalue_2)))))
    (:`Is Not Valid`
      (return true))))