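; Behaviour component that prepares a dynamic material instance on its owner's mesh or decal, for changing that material at runtime.
; On init it creates the instance from the named material slot of the primitive component, or from the first tagged decal component when IsDecal is set.
; On execute it reassigns the instance to the decal, then runs the parent behaviour.
; GetMaterial exposes the stored instance; no material parameters are set here.
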(event `self.BP_InitBehaviour_Implementation`
  (params (NewOwnerComponent :type "SceneComponent Object Reference"))
  (bind _primitivecomponent (`self.GetPrimitiveComponent`))
  (bind _materialslotname (`self.MaterialSlotName`))
  (bind _returnvalue (`PrimitiveComponent.GetMaterialIndex` _primitivecomponent _materialslotname))
  (bind _output (`|GetArrayItem` (`Actor.GetComponentsByTag` (`ActorComponent.GetOwner` (`self.GetOwnerComponent`)) "/Script/Engine.DecalComponent" (`self.MeshTag`))))
  ; Create the dynamic material only the first time
  (if (`self.isDecal`)
    (`/Engine/EditorBlueprintResources/StandardMacros.IsValid` _output
      (:`Is Valid`
        (bind _output_get (set `self.Decal` _output))
        (bind _returnvalue_2 (`DecalComponent.CreateDynamicMaterialInstance` _output_get))
        (set `self.Material` _returnvalue_2))
      (:`Is Not Valid`
        _))
    (else
      (`/Engine/EditorBlueprintResources/StandardMacros.IsValid` _primitivecomponent
        (:`Is Valid`
          (bind _returnvalue_3 (`PrimitiveComponent.CreateDynamicMaterialInstance` _primitivecomponent _returnvalue (`PrimitiveComponent.GetMaterial` _primitivecomponent _returnvalue) _materialslotname))
          (set `self.Material` _returnvalue_3))
        (:`Is Not Valid`
          _))))
  (`parent.BP_InitBehaviour_Implementation` null))

(event `self.BP_ExecuteBehaviour_Implementation`
  (if (`self.isDecal`)
    (`DecalComponent.SetDecalMaterial` (`self.Decal`) (`self.Material`)))
  (`parent.BP_ExecuteBehaviour_Implementation`))

(fn `GetMaterial`
  (returns (Material :type "MaterialInstanceDynamic Object Reference"))
  (return (`self.Material`)))