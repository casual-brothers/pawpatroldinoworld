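; BP_Behaviour_Change2Material is a behaviour that prepares two named material slots on a primitive component for runtime changes.
; On init it creates a dynamic material instance from each slot's current material and caches them as Material and Material2.
; It then calls the parent init, which also runs when the component is invalid.
; GetMaterial returns only the first instance.
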(event `self.BP_InitBehaviour_Implementation`
  (params (NewOwnerComponent :type "SceneComponent Object Reference"))
  (bind _primitivecomponent (`self.GetPrimitiveComponent`))
  (bind _primitivecomponent_2 (`self.GetPrimitiveComponent`))
  (bind _materialslotname (`self.MaterialSlotName`))
  (bind _materialslotname2 (`self.MaterialSlotName2`))
  (bind _returnvalue (`PrimitiveComponent.GetMaterialIndex` _primitivecomponent _materialslotname2))
  (bind _returnvalue_2 (`PrimitiveComponent.GetMaterialIndex` _primitivecomponent_2 _materialslotname))
  (`/Engine/EditorBlueprintResources/StandardMacros.IsValid` (`self.GetPrimitiveComponent`)
    (:`Is Valid`
      (`|ExecutionSequence`
        (:`then_0`
          ; Create the dynamic material only the first time
          (bind _returnvalue_3 (`PrimitiveComponent.CreateDynamicMaterialInstance` _primitivecomponent_2 _returnvalue_2 (`PrimitiveComponent.GetMaterial` _primitivecomponent_2 _returnvalue_2) _materialslotname))
          (set `self.Material` _returnvalue_3))
        (:`then_1`
          (bind _returnvalue_4 (`PrimitiveComponent.CreateDynamicMaterialInstance` _primitivecomponent _returnvalue (`PrimitiveComponent.GetMaterial` _primitivecomponent _returnvalue) _materialslotname2))
          (set `self.Material2` _returnvalue_4))
        (:`then_2`
          (`parent.BP_InitBehaviour_Implementation` null :!label _label))))
    (:`Is Not Valid`
      (goto _label))))

(fn `GetMaterial`
  (returns (Material :type "MaterialInstanceDynamic Object Reference"))
  (return (`self.Material`)))