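; BP_Behaviour_Shine is a behaviour Blueprint, named for a shine effect, whose init, execute, tick and stop events only call their parent implementations.
; Disconnected nodes hold an unused draft that sets a material scalar parameter to zero or one.
; Other unwired nodes attach the NS_Interactable_Shine Niagara system to a primitive component and set its static mesh variable.
; As wired, the asset adds no behaviour of its own.
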(event `self.BP_InitBehaviour_Implementation`
  (params (NewOwnerComponent :type "SceneComponent Object Reference"))
  (`parent.BP_InitBehaviour_Implementation` NewOwnerComponent))

(event `self.BP_ExecuteBehaviour_Implementation`
  (`parent.BP_ExecuteBehaviour_Implementation`))

(event `self.BP_TickBehaviour_Implementation`
  (params (DeltaTime :type "Float (single-precision)"))
  (`parent.BP_TickBehaviour_Implementation` DeltaTime))

(event `self.BP_StopBehaviour_Implementation`
  (`parent.BP_StopBehaviour_Implementation`))