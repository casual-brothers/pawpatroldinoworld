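; Interaction behaviour that attaches a minigame actor's component to whoever executes it, such as a player picking up an item.
; It requires a deployable target component, which it notifies before snapping components found by tag and class, falling back to roots.
; It resets the hint timer and optionally disables physics and collision or randomises rotation.
; For players, it adds the actor to PlayerState items by first tag and disables the interaction receiver's collision.
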(event `self.BP_ExecuteBehaviour_Implementation`
  (bind _owneractor (`self.OwnerActor`))
  (bind _tags (`Actor.Tags` _owneractor))
  (`parent.BP_ExecuteBehaviour_Implementation`)
  (bind _output_get (set `self.OwnerActor` (`ActorComponent.GetOwner` (`self.OwnerComponent`))))
  (bind _aspdwminigame_actor_interface (cast `PDWMinigameActorInterface` _output_get))
  (bind _returnvalue (`PDWMinigameActorInterface.BP_GetMinigameTargetComponent` _aspdwminigame_actor_interface))
  (bind _aspdwdeployable_component (cast `PDWDeployableComponent` _returnvalue))
  (`PDWDeployableComponent.OnObjectAttached` _aspdwdeployable_component)
  (set `self.ComponentToAttach` (`self.GetComponent` (`self.OwnerActor`) (`self.ComponentToAttachTag`) (`self.ComponentToAttachClass`)))
  (set `self.InteracterComponent` (`self.GetComponent` (`self.BehaviourExecutioner`) (`self.InteracterComponentTag`) (`self.InteracterComponentClass`)))
  (`SceneComponent.K2_AttachToComponent` (`self.ComponentToAttach`) (`self.InteracterComponent`) (`self.InteracterSocketName`) "SnapToTarget" "SnapToTarget" "KeepWorld" false)
  (`PDWEventSubsytem.OnResetHintTimerRequestEvent` (subsystem `PDWEventSubsytem`))
  (if (`self.DisablePhysics`)
    (bind _asprimitive_component (cast `PrimitiveComponent` (`self.ComponentToAttach`))
      (:`then`
        (`PrimitiveComponent.SetSimulatePhysics` _asprimitive_component false)
        (`PrimitiveComponent.SetCollisionEnabled` _asprimitive_component "NoCollision"))
      (:`CastFailed`
        _)))
  (if (`self.RandomRotation`)
    (`SceneComponent.K2_SetWorldRotation` (`self.ComponentToAttach`) (`KismetMathLibrary.RandomRotator` true) false false))
  (bind _aspdwplayer_interface (cast `PDWPlayerInterface` (`self.BehaviourExecutioner`))
    (:`then`
      (bind _aspdwinteraction_receiver_component (cast `PDWInteractionReceiverComponent` (`self.OwnerComponent`))
        (:`then`
          (bind _returnvalue_2 (`PDWPlayerInterface.GetPDWPlayerState` _aspdwplayer_interface))
          (if (> (`KismetArrayLibrary.Array_Length` _tags) 0)
            (`PDWPlayerState.AddItem` _returnvalue_2 (`|GetArrayItem` _tags) _owneractor))
          (`PrimitiveComponent.SetCollisionEnabled` _aspdwinteraction_receiver_component "NoCollision"))
        (:`CastFailed`
          _)))
    (:`CastFailed`
      _))
  (`self.StopBehaviour`))

(fn `GetComponent`
  (params (Actor :type "Actor Object Reference") (ComponentTag :type Name) (ComponentClass :type "SceneComponent Class Reference"))
  (returns (Component :type "SceneComponent Object Reference"))
  (bind _output (`|GetArrayItem` (`Actor.GetComponentsByTag` Actor ComponentClass ComponentTag)))
  (if (and (!= ComponentTag "None") (`KismetSystemLibrary.IsValidClass` ComponentClass))
    (`/Engine/EditorBlueprintResources/StandardMacros.IsValid` _output
      (:`Is Valid`
        (return _output))
      (:`Is Not Valid`
        _)))
  (return (`Actor.RootComponent` Actor)))