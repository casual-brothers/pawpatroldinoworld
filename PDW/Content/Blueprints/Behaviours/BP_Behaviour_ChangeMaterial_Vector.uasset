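; Behaviour that drives a vector (color) parameter on a material from a single scalar value, built on a parent behaviour Blueprint.
; On init it derives StartingColor from ParameterColor times the starting value, and each new value writes ParameterColor scaled by that value.
; Starting and current values are read back by projecting the material's color onto the StartingColor-to-ParameterColor line with 4D dot products, yielding a lerp alpha.
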(event `self.BP_InitBehaviour_Implementation`
  (params (NewOwnerComponent :type "SceneComponent Object Reference"))
  (set `self.StartingColor` (* (`self.ParameterColor`) (`self.GetStartingValue`)))
  (`parent.BP_InitBehaviour_Implementation` null))

(fn `GetCurrentValue`
  (returns (CurrentValue :type "Float (double-precision)"))
  (bind _returnvalue (`MaterialInstanceDynamic.K2_GetVectorParameterValueByInfo` (`self.GetMaterial`) (`self.Material Parameter Info`)))
  (return (`self.GetLerpAlpha` _returnvalue)))

(fn `GetLerpAlpha`
  (params (Color :type "LinearColor Structure"))
  (returns (LerpAlpha :type "Float (double-precision)"))
  (bind _startingcolor (`self.StartingColor`))
  (bind (_returnvalue_r _returnvalue_g _returnvalue_b _returnvalue_a) (break `LinearColor` (- (`self.ParameterColor`) _startingcolor)))
  (bind (_returnvalue_r_2 _returnvalue_g_2 _returnvalue_b_2 _returnvalue_a_2) (break `LinearColor` (- Color _startingcolor)))
  (bind _returnvalue (`KismetMathLibrary.MakeVector4` _returnvalue_r _returnvalue_g _returnvalue_b _returnvalue_a))
  (return (/ (`KismetMathLibrary.Vector4_DotProduct` (`KismetMathLibrary.MakeVector4` _returnvalue_r_2 _returnvalue_g_2 _returnvalue_b_2 _returnvalue_a_2) _returnvalue) (`KismetMathLibrary.Vector4_DotProduct` _returnvalue _returnvalue))))

(fn `InitStartingValue`
  (returns (StartingValue :type "Float (double-precision)"))
  (bind _returnvalue (`MaterialInstanceDynamic.K2_GetVectorParameterValueByInfo` (`self.GetMaterial`) (`self.Material Parameter Info`)))
  (return (`self.GetLerpAlpha` _returnvalue)))

(fn `SetNewValue`
  (params (NewValue :type "Float (double-precision)"))
  (`parent.SetNewValue` NewValue)
  (`MaterialInstanceDynamic.SetVectorParameterValueByInfo` (`self.GetMaterial`) (`self.Material Parameter Info`) (* NewValue (`self.ParameterColor`))))