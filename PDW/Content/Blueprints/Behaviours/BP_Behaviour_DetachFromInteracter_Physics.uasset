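; Behaviour Blueprint for items, named for detaching from an interacter, that switches off physics simulation on the item.
; On execute it calls the parent implementation, then, if the item is valid, disables Simulate Physics on each static mesh component tagged PhysicMesh.
; Init, tick and stop are unused placeholder events.
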(event `self.BP_ExecuteBehaviour_Implementation`
  (bind _item (`self.GetItem`))
  (`parent.BP_ExecuteBehaviour_Implementation`)
  (`/Engine/EditorBlueprintResources/StandardMacros.IsValid` _item
    (:`Is Valid`
      (for _array_element (`Actor.GetComponentsByTag` _item "/Script/Engine.StaticMeshComponent" "PhysicMesh")
        (`PrimitiveComponent.SetSimulatePhysics` _array_element false)))))