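; Behaviour that resets a player's Sea Rescue minigame target item.
; On execute, it gets the item matching ItemToRemove from the executioner's PDW player state and caches it for the GetItem accessor.
; If the item is a BP_Minigame_SeaRescue_Target, it resets its PDWDeployable, calls OnMinigameStarted on it and stops the behaviour.
; A failed interface or target cast exits without calling StopBehaviour.
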(event `self.BP_ExecuteBehaviour_Implementation`
  (bind _aspdwplayer_interface (cast `PDWPlayerInterface` (`self.BehaviourExecutioner`)))
  (bind _returnvalue (`PDWPlayerInterface.GetPDWPlayerState` _aspdwplayer_interface))
  (bind _returnvalue_2 (`PDWPlayerState.GetItem` _returnvalue (`self.ItemToRemove`)))
  (bind _output_get (set `self.Item` _returnvalue_2))
  (bind _asbp_minigame_sea_rescue_target (cast `/Game/Blueprints/Actors/MiniGames/SeaRescue/BP_Minigame_SeaRescue_Target` _output_get))
  (bind _pdwdeployable (`/Game/Blueprints/Actors/MiniGames/BP_Minigame_Deployable.PDWDeployable` _asbp_minigame_sea_rescue_target))
  (`PDWMinigameTargetComponent.ResetActor` _pdwdeployable)
  (`PDWMinigameTargetComponent.OnMinigameStarted` _pdwdeployable)
  (`self.StopBehaviour`))

(fn `GetItem`
  (returns (Item :type "Actor Object Reference"))
  (return (`self.Item`)))