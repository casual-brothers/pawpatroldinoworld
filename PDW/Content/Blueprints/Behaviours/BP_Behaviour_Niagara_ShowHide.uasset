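; Behaviour Blueprint that shows or hides a Niagara effect in game.
; On execute it calls the parent implementation, sets the Niagara component's hidden-in-game state from its Hide flag without propagating to children, then stops itself immediately.
; It is a one-shot action: init, tick and stop overrides are disabled placeholders.
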(event `self.BP_ExecuteBehaviour_Implementation`
  (`parent.BP_ExecuteBehaviour_Implementation`)
  (`SceneComponent.SetHiddenInGame` (`self.GetNiagara`) (`self.Hide`) false)
  (`self.StopBehaviour`))