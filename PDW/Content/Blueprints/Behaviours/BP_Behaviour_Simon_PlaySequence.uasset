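; Behaviour that plays back the current sequence of a Simon puzzle interactable by making its echo stones shine.
; On execute it switches to the Simon camera, hides the Niagara effect and waits for the camera delay before disabling the stones.
; Stones shine one by one, chained by behaviour-finished events, or all at once when a reward is due.
; Stopping restores camera and stones; a timer-based tick version remains unconnected.
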(event `self.BP_InitBehaviour_Implementation`
  (params (NewOwnerComponent :type "SceneComponent Object Reference"))
  (`parent.BP_InitBehaviour_Implementation` NewOwnerComponent)
  (bind _asbp_interactable_simon (cast `/Game/Blueprints/Interactables/BP_Interactable_Simon` (`ActorComponent.GetOwner` (`self.OwnerComponent`))))
  (set `self.InteractableSimon` _asbp_interactable_simon))

(event `self.BP_ExecuteBehaviour_Implementation`
  (`parent.BP_ExecuteBehaviour_Implementation`)
  (bind _blendtime (`/Game/Blueprints/Interactables/BP_Interactable_Simon.SimonCameraOn` (`self.InteractableSimon`) (`self.BehaviourExecutioner`)))
  (`KismetSystemLibrary.K2_SetTimerDelegate` (delegate `PlaySumonSequence`) _blendtime)
  (`SceneComponent.SetHiddenInGame` (`Actor.GetComponentByClass` (`self.InteractableSimon`) "/Script/Niagara.NiagaraComponent") true false))

(event `EndReward`
  (params (Behaviour :type "PDWInteractionBehaviour Object Reference"))
  (bind _values (`BlueprintMapLibrary.Map_Values` (`/Game/Blueprints/Interactables/BP_Interactable_Simon.EchoStoneMap` (`self.InteractableSimon`))))
  (remove `PDWInteractionReceiverComponent.OnBehaviourFinished` (`|GetArrayItem` _values) (delegate `EndReward`))
  (`self.StopBehaviour`))

(event `PlaySumonSequence`
  (bind _interactablesimon (`self.InteractableSimon`))
  (bind _interactablesimon_2 (`self.InteractableSimon`))
  (bind _returnvalue (`ActorComponent.GetOwner` (`self.OwnerComponent`)))
  (bind _behaviourshining (`/Game/Blueprints/Interactables/BP_Interactable_Simon.BehaviourShining` (`self.InteractableSimon`)))
  (set `self.Timer` 0.0)
  (set `self.CurrentTimer` 0.0)
  (set `self.CurrentIndex` 0)
  (`/Game/Blueprints/Interactables/BP_Interactable_Simon.DisableEchoStones` _interactablesimon_2 null)
  (bind _values (`BlueprintMapLibrary.Map_Values` (`/Game/Blueprints/Interactables/BP_Interactable_Simon.EchoStoneMap` _interactablesimon_2)))
  (if (`/Game/Blueprints/Interactables/BP_Interactable_Simon.CanGiveReward` _interactablesimon_2)
    (for _array_element _values
      (`PDWInteractionReceiverComponent.ExecuteInteractionBehaviour` _array_element _behaviourshining _returnvalue false false))
    (add `PDWInteractionReceiverComponent.OnBehaviourFinished` (`|GetArrayItem` _values) (delegate `EndReward`))
    (else
      (for _array_element_2 _values
        (add `PDWInteractionReceiverComponent.OnBehaviourFinished` _array_element_2 (delegate `NextBehaviour`)))
      (`PDWInteractionReceiverComponent.ExecuteInteractionBehaviour` (`BlueprintMapLibrary.Map_Find` (`/Game/Blueprints/Interactables/BP_Interactable_Simon.EchoStoneMap` _interactablesimon) (`|GetArrayItem` (`/Game/Blueprints/Interactables/BP_Interactable_Simon.CurrentSequence` _interactablesimon) (`self.CurrentIndex`))) _behaviourshining _returnvalue false false :!label _label))))

(event `NextBehaviour`
  (params (Behaviour :type "PDWInteractionBehaviour Object Reference"))
  (bind _currentindex (`self.CurrentIndex`))
  (`/Engine/EditorBlueprintResources/StandardMacros.IncrementInt` _currentindex
    (:`  `
      (if (< _currentindex (`KismetArrayLibrary.Array_Length` (`/Game/Blueprints/Interactables/BP_Interactable_Simon.CurrentSequence` (`self.InteractableSimon`))))
        (goto _label)
        (else
          (bind _values (`BlueprintMapLibrary.Map_Values` (`/Game/Blueprints/Interactables/BP_Interactable_Simon.EchoStoneMap` (`self.InteractableSimon`))))
          (for _array_element _values
            (remove `PDWInteractionReceiverComponent.OnBehaviourFinished` _array_element (delegate `NextBehaviour`)))
          (`self.StopBehaviour`))))))

(event `self.BP_TickBehaviour_Implementation`
  (params (DeltaTime :type "Float (single-precision)"))
  (`parent.BP_TickBehaviour_Implementation` DeltaTime))

(event `self.BP_StopBehaviour_Implementation`
  (`/Game/Blueprints/Interactables/BP_Interactable_Simon.SimonCameraOff` (`self.InteractableSimon`) (`self.BehaviourExecutioner`))
  (`/Game/Blueprints/Interactables/BP_Interactable_Simon.EnableEchoStones` (`self.InteractableSimon`) null)
  (`parent.BP_StopBehaviour_Implementation`))

(fn `HasTimerEnded`
  (returns (ReturnValue :type Boolean))
  (return (or (`KismetMathLibrary.NearlyEqual_FloatFloat` (`self.CurrentTimer`) (`self.Timer`) 0.02) (> (`self.CurrentTimer`) (`self.Timer`)))))