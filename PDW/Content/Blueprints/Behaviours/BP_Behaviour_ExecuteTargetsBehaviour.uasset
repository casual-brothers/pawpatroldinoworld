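; Interaction behaviour that runs a chosen behaviour on every target of its owning BP_Interactable_Base.
; Each target's interaction receiver component is found by tag, falling back to the first by class, and executes the configured behaviour identifier.
; It stops immediately, or optionally waits on the last target's finished event only.
; When waiting, it can adopt the finished behaviour's new state if that behaviour's receiver has that state tag.
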(event `self.BP_ExecuteBehaviour_Implementation`
  (`parent.BP_ExecuteBehaviour_Implementation`)
  (bind _asbp_interactable_base (cast `/Game/Blueprints/Interactables/BP_Interactable_Base` (`ActorComponent.GetOwner` (`self.GetOwnerComponent`))))
  (bind _targets (`/Game/Blueprints/Interactables/BP_Interactable_Base.Targets` _asbp_interactable_base))
  (set `self.LastIndex` (- (`KismetArrayLibrary.Array_Length` _targets) 1))
  (for (_array_element _array_index) _targets
    (set `self.CurrentIndex` _array_index)
    (bind _returnvalue (`Actor.GetComponentsByTag` _array_element "/Game/Blueprints/Pawn/Components/BP_InteractionReceiverComponent.BP_InteractionReceiverComponent_C" (`self.TargetsInteractionReceiverTag`)))
    (bind _returnvalue_2 (select `bool` (> (`KismetArrayLibrary.Array_Length` _returnvalue) 0) :`false` (`Actor.GetComponentByClass` _array_element "/Game/Blueprints/Pawn/Components/BP_InteractionReceiverComponent.BP_InteractionReceiverComponent_C") :`true` (`|GetArrayItem` _returnvalue)))
    (`PDWInteractionReceiverComponent.ExecuteInteractionBehaviour` _returnvalue_2 (`self.TargetsBehaviourToExecute`) (`ActorComponent.GetOwner` (`self.GetOwnerComponent`)) false false)
    (if (and (`self.WaitTargetsBehaviour`) (== (`self.CurrentIndex`) (`self.LastIndex`)))
      (add `PDWInteractionReceiverComponent.OnBehaviourFinished` _returnvalue_2 (delegate `TargetBehaviourFinished`))))
  (if (not (`self.WaitTargetsBehaviour`))
    (`self.StopBehaviour`)))

(event `TargetBehaviourFinished`
  (params (Behaviour :type "PDWInteractionBehaviour Object Reference"))
  (if (`self.UseTargetsNewState`)
    (bind _asbp_behaviour_base (cast `/Game/Blueprints/Behaviours/BP_Behaviour_Base` Behaviour))
    (bind _aspdwinteraction_receiver_component (cast `PDWInteractionReceiverComponent` (`PDWInteractionBehaviour.OwnerComponent` Behaviour)))
    (bind _newstate (`/Game/Blueprints/Behaviours/BP_Behaviour_Base.NewState` _asbp_behaviour_base))
    (if (`PDWInteractionReceiverComponent.HasStateTag` _aspdwinteraction_receiver_component _newstate)
      (set `self.NewState` _newstate)))
  (`self.StopBehaviour`))