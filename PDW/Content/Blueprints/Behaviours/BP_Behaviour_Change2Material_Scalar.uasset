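; Behaviour Blueprint that changes a scalar parameter on two materials with one shared value.
; It overrides value hooks and leaves execution to its parent class.
; SetNewValue writes to both the material from GetMaterial and Material2, each through its own parameter info.
; InitValues, InitStartingValue and GetCurrentValue use only the first material, so Material2's own value is never read or initialised here.
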(event `self.BP_ExecuteBehaviour_Implementation`
  (`parent.BP_ExecuteBehaviour_Implementation`))

(fn `GetCurrentValue`
  (returns (CurrentValue :type "Float (double-precision)"))
  (bind _returnvalue (`MaterialInstanceDynamic.K2_GetScalarParameterValueByInfo` (`self.GetMaterial`) (`self.Material Parameter Info`)))
  (return _returnvalue))

(fn `InitStartingValue`
  (returns (StartingValue :type "Float (double-precision)"))
  (bind _returnvalue (`MaterialInstanceDynamic.K2_GetScalarParameterValueByInfo` (`self.GetMaterial`) (`self.Material Parameter Info`)))
  (return _returnvalue))

(fn `InitValues`
  (params (NewValue :type "Float (double-precision)" :default 0.0))
  (`MaterialInstanceDynamic.SetScalarParameterValueByInfo` (`self.GetMaterial`) (`self.Material Parameter Info`) NewValue))

(fn `SetNewValue`
  (params (NewValue :type "Float (double-precision)"))
  (`MaterialInstanceDynamic.SetScalarParameterValueByInfo` (`self.GetMaterial`) (`self.Material Parameter Info`) NewValue)
  (`MaterialInstanceDynamic.SetScalarParameterValueByInfo` (`self.Material2`) (`self.Material Parameter Info2`) NewValue))