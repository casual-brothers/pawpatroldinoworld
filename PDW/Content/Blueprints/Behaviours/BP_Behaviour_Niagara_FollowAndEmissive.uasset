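; Behaviour Blueprint that eases an emissive float parameter on a Niagara effect toward a target value while ticking.
; Each tick lerps CurrentValue toward ValueToReach by ProgressPercentage, snaps within ErrorTolerance, then writes it to the named Niagara variable.
; The easing ignores DeltaTime, so its speed depends on tick rate.
; Stopping writes StartingValue back to Niagara without resetting CurrentValue; no follow logic appears in this graph.
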(event `self.BP_TickBehaviour_Implementation`
  (params (DeltaTime :type "Float (single-precision)"))
  (bind _valuetoreach (`self.ValueToReach`))
  (bind _returnvalue (`KismetMathLibrary.Lerp` (`self.CurrentValue`) (`self.ValueToReach`) (`self.ProgressPercentage`)))
  (`parent.BP_TickBehaviour_Implementation` DeltaTime)
  (bind _output_get (set `self.CurrentValue` (`KismetMathLibrary.SelectFloat` _valuetoreach _returnvalue (`KismetMathLibrary.NearlyEqual_FloatFloat` _valuetoreach _returnvalue (`self.ErrorTolerance`)))))
  (`NiagaraComponent.SetVariableFloat` (`self.GetNiagara`) (`self.NiagaraEmissiveVariable`) _output_get))

(event `self.BP_StopBehaviour_Implementation`
  (`parent.BP_StopBehaviour_Implementation`)
  (`NiagaraComponent.SetVariableFloat` (`self.GetNiagara`) (`self.NiagaraEmissiveVariable`) (`self.StartingValue`)))