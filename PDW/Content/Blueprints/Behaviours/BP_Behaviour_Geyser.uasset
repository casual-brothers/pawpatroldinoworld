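; Geyser behaviour that, after a delay, erupts with a Niagara effect and lifts players inside it.
; Execution starts a timer that spawns the effect and enables the owner's FlyCollision box.
; Tick advances each player's elevation-curve value and raises their Z, switching to a sine bob after reaching max height.
; The eruption ends on timeout or when empty, restarting if players remain, otherwise stopping and disabling the collision.
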(event `self.BP_ExecuteBehaviour_Implementation`
  (bind _asbp_interaction_receiver_component (cast `/Game/Blueprints/Pawn/Components/BP_InteractionReceiverComponent` (`self.OwnerComponent`)))
  (set `self.InteractionReceiverComp` _asbp_interaction_receiver_component)
  (`self.StartGeyserDelay`)
  (for _array_element (`PDWGameplayFunctionLibrary.GetPlayers`)
    (`BlueprintMapLibrary.Map_Add` (`self.IsRaising`) _array_element true)))

(event `StartGeyserDelay`
  (`KismetSystemLibrary.K2_SetTimerDelegate` (delegate `Start Geyser`) (`self.ExplosionDelay`)))

(event `Start Geyser`
  (`KismetArrayLibrary.Array_Clear` (`self.PlayersInside`))
  (set `self.AnyPlayerInside` false)
  (bind _returnvalue (`NiagaraFunctionLibrary.SpawnSystemAttached` (`self.System Template`) (`self.GetOwnerComponent`) "None" (0.0 0.0 0.0) (struct) "KeepRelativeOffset" false false))
  (set `self.SpawnedVFX` _returnvalue)
  (`NiagaraComponent.SetVariableFloat` _returnvalue "LoopDuration" (- (/ (`.MaxTime` (`CurveBase.GetTimeRange` (`self.GeyserElevationCurve`))) (`self.CurveSpeed`)) 3.0))
  (`NiagaraComponent.SetVariableFloat` _returnvalue "Velocity" 1.0)
  (`ActorComponent.Activate` _returnvalue true)
  (set `self.GeyserDuration` (`.MaxTime` (`CurveBase.GetTimeRange` (`self.GeyserElevationCurve`))))
  (set `self.CurrentDuration` 0.0)
  (set `self.IsGeyserActive` true)
  (`PrimitiveComponent.SetCollisionEnabled` (`|GetArrayItem` (`Actor.GetComponentsByTag` (`ActorComponent.GetOwner` (`self.OwnerComponent`)) "/Script/Engine.BoxComponent" "FlyCollision")) "QueryAndPhysics"))

(event `self.BP_TickBehaviour_Implementation`
  (params (DeltaTime :type "Float (single-precision)"))
  (bind _tempplayer (`self.TempPlayer`))
  (bind _tempplayer_2 (`self.TempPlayer`))
  (bind _playersinside (`self.PlayersInside`))
  (bind (_returnvalue_x _returnvalue_y _returnvalue_z) (`KismetMathLibrary.BreakVector` (`Actor.K2_GetActorLocation` _tempplayer)))
  (bind _charactermovement (`Character.CharacterMovement` (`self.TempPlayer`)))
  (bind _currentcurvevalue (`self.GetCurveValue` (`PDWCharacter.GetGeyserCurveValue` (`self.TempPlayer`)) (`self.MaxHeight`) (`self.TempDeltaTime`)))
  (bind (_velocity_x _velocity_y _velocity_z) (`KismetMathLibrary.BreakVector` (`MovementComponent.Velocity` _charactermovement)))
  (bind _returnvalue (`KismetMathLibrary.SelectFloat` _currentcurvevalue (+ _currentcurvevalue (* (`KismetMathLibrary.Sin` (* (`self.CurrentDuration`) (`self.OscillationSpeed`))) (`self.OscillationValue`))) (`BlueprintMapLibrary.Map_Find` (`self.IsRaising`) (`self.TempPlayer`))))
  (bind _output_get (set `self.TempDeltaTime` DeltaTime))
  (set `self.CurrentDuration` (+ _output_get (`self.CurrentDuration`)))
  (set `self.AnyPlayerInside` false)
  (if (`self.IsGeyserActive`)
    (for _array_element (`PDWGameplayFunctionLibrary.GetPlayers`)
      (bind _output_get_2 (set `self.TempPlayer` _array_element))
      (`PDWCharacter.SetIsInsideGeyser` _output_get_2 (`self.CheckPlayerIsInside` _array_element (`self.MaxHeight`)))
      (if (`PDWCharacter.GetIsInsideGeyser` _output_get_2)
        (`KismetArrayLibrary.Array_AddUnique` _playersinside _tempplayer_2)
        (`PDWCharacter.SetGeyserCurveValue` _output_get_2 (+ (`PDWCharacter.GetGeyserCurveValue` _tempplayer_2) (`self.TempDeltaTime`)))
        (set `self.AnyPlayerInside` true)
        (if (and (`PDWCharacter.GetIsInsideGeyser` _tempplayer) (< _returnvalue_z _currentcurvevalue)) :!label _label
          (`Actor.K2_SetActorLocation` (`self.TempPlayer`) (`KismetMathLibrary.MakeVector` _returnvalue_x _returnvalue_y _returnvalue) false false)
          (if (>= _returnvalue (`self.MaxHeight`))
            (`BlueprintMapLibrary.Map_Add` (`self.IsRaising`) (`self.TempPlayer`))))
        (else
          (bind _returnvalue_2 (`KismetArrayLibrary.Array_RemoveItem` _playersinside _array_element))
          (if _returnvalue_2
            (if (< _velocity_z 0.0)
              (set `MovementComponent.Velocity` (`KismetMathLibrary.MakeVector` _velocity_x _velocity_y) _charactermovement)
              (`PDWCharacter.SetGeyserCurveValue` _tempplayer 0.0 :!label _label_2)
              (goto _label))
            (else
              (goto _label_2))))))
    (if (or (>= (`self.CurrentDuration`) (`self.GeyserDuration`)) (not (`self.AnyPlayerInside`)))
      (`ActorComponent.Deactivate` (`self.SpawnedVFX`))
      (set `self.IsGeyserActive` false)
      (set `self.CurrentCurveTime` 0.0)
      (if (`self.AnyPlayerInside`)
        (`self.ResetVariables`)
        (`self.StartGeyserDelay`)
        (else
          (`self.StopBehaviour`))))))

(event `self.BP_StopBehaviour_Implementation`
  (`self.ResetVariables`)
  (`PrimitiveComponent.SetCollisionEnabled` (`|GetArrayItem` (`Actor.GetComponentsByTag` (`ActorComponent.GetOwner` (`self.OwnerComponent`)) "/Script/Engine.BoxComponent" "FlyCollision")) "NoCollision")
  (`parent.BP_StopBehaviour_Implementation`))

(event `ResetVariables`
  (for _array_element (`PDWGameplayFunctionLibrary.GetPlayers`)
    (if (`self.CheckPlayerIsInside` _array_element (`self.MaxHeight`))
      (`PDWCharacter.SetIsInsideGeyser` _array_element false)
      (`PDWCharacter.SetGeyserCurveValue` _array_element 0.0)
      (bind _charactermovement (`Character.CharacterMovement` _array_element))
      (bind (_velocity_x _velocity_y _velocity_z) (`KismetMathLibrary.BreakVector` (`MovementComponent.Velocity` _charactermovement)))
      (if (< _velocity_z 0.0)
        (set `MovementComponent.Velocity` (`KismetMathLibrary.MakeVector` _velocity_x _velocity_y) _charactermovement)))))