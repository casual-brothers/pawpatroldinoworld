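; Base behaviour Blueprint that gives access to the owning actor's main Niagara component.
; On init, it runs the parent initialisation, then caches the first Niagara component tagged "MainNiagara" on the owner component's actor, if one exists.
; A GetNiagara function returns that cached reference, while the execute, tick and stop events are left as disabled placeholders.
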(event `self.BP_InitBehaviour_Implementation`
  (params (NewOwnerComponent :type "SceneComponent Object Reference"))
  (bind _returnvalue (`Actor.GetComponentsByTag` (`ActorComponent.GetOwner` (`self.OwnerComponent`)) "/Script/Niagara.NiagaraComponent" "MainNiagara"))
  (`parent.BP_InitBehaviour_Implementation` NewOwnerComponent)
  (if (> (`KismetArrayLibrary.Array_Length` _returnvalue) 0)
    (set `self.Niagara` (`|GetArrayItem` _returnvalue))))

(fn `GetNiagara`
  (returns (Niagara :type "NiagaraComponent Object Reference"))
  (return (`self.Niagara`)))