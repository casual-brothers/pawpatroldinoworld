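; Behaviour Blueprint that shows or hides mesh components on the actor owning its behaviour component.
; On execute, it gathers that actor's meshes by TagMeshToShow, or all meshes when the tag is None.
; It applies NewHidden to each mesh and its children, setting the mesh's collision to NoCollision when hidden and QueryAndPhysics when shown.
; It then stops itself immediately, acting as a one-shot behaviour.
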(event `self.BP_ExecuteBehaviour_Implementation`
  (bind _tagmeshtoshow (`self.TagMeshToShow`))
  (bind _newhidden (`self.NewHidden`))
  (bind _returnvalue (`ActorComponent.GetOwner` (`self.OwnerComponent`)))
  (`parent.BP_ExecuteBehaviour_Implementation`)
  (for _array_element (select `bool` (!= _tagmeshtoshow "None") :`false` (`Actor.K2_GetComponentsByClass` _returnvalue "/Script/Engine.MeshComponent") :`true` (`Actor.GetComponentsByTag` _returnvalue "/Script/Engine.MeshComponent" _tagmeshtoshow))
    (`SceneComponent.SetHiddenInGame` _array_element _newhidden true)
    (if _newhidden
      (`PrimitiveComponent.SetCollisionEnabled` _array_element "NoCollision")
      (else
        (`PrimitiveComponent.SetCollisionEnabled` _array_element "QueryAndPhysics"))))
  (`self.StopBehaviour`))