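; Behaviour that unlocks the items listed on its owning actor's BP_ItemsToUnlockComponent once the behaviour animation ends.
; It adds one of each unlockable to the inventory with a notification, then flags the set as pending review.
; It then triggers an action named from the reward gameplay tag and stops itself.
; Without that component, the animation-end event does nothing, including not stopping the behaviour.
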(event `self.OnBehaviourAnimationEnd`
  (bind _returnvalue (`Actor.GetComponentByClass` (`ActorComponent.GetOwner` (`self.GetOwnerComponent`)) "/Game/Blueprints/Components/BP_ItemsToUnlockComponent.BP_ItemsToUnlockComponent_C"))
  (bind _itemstounlock_unlocakbles (break `PDWUnlockableContainer` (`/Game/Blueprints/Components/BP_ItemsToUnlockComponent.ItemsToUnlock` _returnvalue)))
  (`/Engine/EditorBlueprintResources/StandardMacros.IsValid` _returnvalue
    (:`Is Valid`
      (for _array_element _itemstounlock_unlocakbles
        (`PDWGameplayFunctionLibrary.AddItemsToInventory` self (`|MakeMap` (`PDWUnlockableData.ID` _array_element) 1)))
      (`PDWUIFunctionLibrary.SetPendingReview` self (`/Game/Blueprints/Components/BP_ItemsToUnlockComponent.ItemsToUnlock` _returnvalue))
      (`NebulaFlowCoreFunctionLibrary.TriggerAction` (`BlueprintGameplayTagLibrary.GetDebugStringFromGameplayTag` (`FlowDeveloperSettings.GetRewardTag`)) "" null)
      (`self.StopBehaviour`))))

(event `self.BP_ExecuteBehaviour_Implementation`
  (`parent.BP_ExecuteBehaviour_Implementation`))