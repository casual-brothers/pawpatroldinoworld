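; Behaviour that links a water station's current water level to the inherited value logic, named for changing the station's material.
; On init it finds the owner's PDWWaterStationHandler and seeds InitValues with the current water, re-seeding whenever the handler's OnInit fires.
; SetNewValue writes the new amount back to the handler before calling the parent, which is left to handle any material update.
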(event `self.BP_InitBehaviour_Implementation`
  (params (NewOwnerComponent :type "SceneComponent Object Reference"))
  (bind _returnvalue (`Actor.GetComponentByClass` (`ActorComponent.GetOwner` NewOwnerComponent) "/Script/PDW.PDWWaterStationHandler"))
  (`parent.BP_InitBehaviour_Implementation` NewOwnerComponent)
  (set `self.WaterStationHandler` _returnvalue)
  (add `PDWWaterStationHandler.OnInit` _returnvalue (delegate `OnInit`))
  (`self.InitValues` (`PDWWaterStationHandler.GetCurrentWater` (`self.WaterStationHandler`))))

(event `OnInit`
  (`self.InitValues` (`PDWWaterStationHandler.GetCurrentWater` (`self.WaterStationHandler`))))

(fn `SetNewValue`
  (params (NewValue :type "Float (double-precision)"))
  (`PDWWaterStationHandler.SetCurrentWater` (`self.WaterStationHandler`) NewValue)
  (`parent.SetNewValue` NewValue))