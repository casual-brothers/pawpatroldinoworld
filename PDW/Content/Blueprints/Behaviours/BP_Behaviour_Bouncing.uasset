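; Interaction behaviour that repeatedly bounces the player's pup upward, like a trampoline.
; It stops immediately if the player has a vehicle, the pup is flying, or the interaction component sits above the pawn.
; Otherwise a looping timer launches the pup with a Z override, boosted by a multiplier while jump is held.
; Bouncing ends when the component stops being interactable, and stopping clears the timer.
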(event `self.BP_InitBehaviour_Implementation`
  (params (NewOwnerComponent :type "SceneComponent Object Reference")))

(event `self.BP_ExecuteBehaviour_Implementation`
  (bind (_returnvalue_x _returnvalue_y _returnvalue_z) (`KismetMathLibrary.BreakVector` (`Actor.K2_GetActorLocation` (`Controller.K2_GetPawn` (`self.Controller`)))))
  (bind _aspdwplayer_interface (cast `PDWPlayerInterface` (`self.BehaviourExecutioner`)))
  (bind _returnvalue (`PDWPlayerInterface.GetPDWPlayerController` _aspdwplayer_interface))
  (bind _asbp_player_controller (cast `/Game/Blueprints/Pawn/BP_PlayerController` _returnvalue))
  (bind _returnvalue_2 (`PDWPlayerController.GetVehicleInstance` _returnvalue))
  (`/Engine/EditorBlueprintResources/StandardMacros.IsValid` _returnvalue_2
    (:`Is Valid`
      (set `self.bSkip` true :!label _label)
      (`self.StopBehaviour` :!label _label_2))
    (:`Is Not Valid`
      (bind _returnvalue_3 (`PDWPlayerController.GetPupInstance` _returnvalue))
      (`/Engine/EditorBlueprintResources/StandardMacros.IsValid` _returnvalue_3
        (:`Is Valid`
          (set `self.Controller` _asbp_player_controller)
          (if (`PDWCharacter.bFlying` _returnvalue_3)
            (goto _label)
            (else
              (bind _aspdwinteraction_receiver_component (cast `PDWInteractionReceiverComponent` (`self.OwnerComponent`)))
              (bind (_returnvalue_x_2 _returnvalue_y_2 _returnvalue_z_2) (`KismetMathLibrary.BreakVector` (`SceneComponent.K2_GetComponentLocation` _aspdwinteraction_receiver_component)))
              (if (> _returnvalue_z_2 _returnvalue_z)
                (goto _label)
                (else
                  (bind _returnvalue_4 (`KismetSystemLibrary.K2_SetTimerDelegate` (delegate `Jump`) (`self.Duration`) true))
                  (set `self.Timer` _returnvalue_4)
                  (add `PDWInteractionReceiverComponent.OnStopBeingInteractable` _aspdwinteraction_receiver_component (delegate `CustomEvent`))
                  (`parent.BP_ExecuteBehaviour_Implementation`))))))))))

(event `CustomEvent`
  (params (Component :type "PDWInteractionComponent Object Reference"))
  (goto _label_2))

(event `self.BP_StopBehaviour_Implementation`
  (if (`KismetSystemLibrary.K2_IsValidTimerHandle` (`self.Timer`))
    (`KismetSystemLibrary.K2_ClearTimer` null "Jump")
    (`parent.BP_StopBehaviour_Implementation`)))

(event `Jump`
  (bind _jumpingforce (`self.JumpingForce`))
  (if (`/Game/Blueprints/Pawn/BP_PlayerController.JumpPressed` (`self.Controller`))
    (`Character.LaunchCharacter` (stale `self.BP_ExecuteBehaviour_Implementation` _returnvalue_3) (`KismetMathLibrary.MakeVector` 0.0 0.0 (* (`self.HoldJumpMultiplier`) _jumpingforce)) false true)
    (else
      (`Character.LaunchCharacter` (stale `self.BP_ExecuteBehaviour_Implementation` _returnvalue_3) (`KismetMathLibrary.MakeVector` 0.0 0.0 _jumpingforce) false true))))