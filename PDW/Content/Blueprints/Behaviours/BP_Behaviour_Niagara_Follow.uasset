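; Behaviour that makes a Niagara effect follow the controlled pawn of the player who executes it.
; On execute it caches that pawn and sets the follow speed parameter, then each tick writes the pawn's location into the follow location parameter.
; On init and stop it resets both parameters to the owner's initial location and the starting speed.
; Parameter names are configurable variables, and writes are skipped when a name is None.
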(event `self.BP_InitBehaviour_Implementation`
  (params (NewOwnerComponent :type "SceneComponent Object Reference"))
  (`parent.BP_InitBehaviour_Implementation` NewOwnerComponent)
  (set `self.StartingLocation` (`Actor.K2_GetActorLocation` (`ActorComponent.GetOwner` (`self.OwnerComponent`))))
  (`self.BackToStart`))

(event `self.BP_ExecuteBehaviour_Implementation`
  (`parent.BP_ExecuteBehaviour_Implementation`)
  (bind _aspdwplayer_interface (cast `PDWPlayerInterface` (`self.BehaviourExecutioner`)))
  (bind _returnvalue (`PDWPlayerInterface.GetPDWPlayerController` _aspdwplayer_interface))
  (set `self.ControlledPawn` (`Controller.K2_GetPawn` _returnvalue))
  (`self.SetNiagaraVariableFloat` (`self.GetNiagara`) (`self.NiagaraFollowSpeedVariable`) (`self.NiagaraFollowSpeed`)))

(event `self.BP_TickBehaviour_Implementation`
  (params (DeltaTime :type "Float (single-precision)"))
  (`parent.BP_TickBehaviour_Implementation` DeltaTime)
  (`self.SetNiagaraVariableVector3` (`self.GetNiagara`) (`self.NiagaraFollowLocationVariable`) (`Actor.K2_GetActorLocation` (`self.ControlledPawn`))))

(event `self.BP_StopBehaviour_Implementation`
  (`parent.BP_StopBehaviour_Implementation`)
  (`self.BackToStart`))

(fn `BackToStart`
  (bind _niagara (`self.GetNiagara`))
  (`self.SetNiagaraVariableVector3` _niagara (`self.NiagaraFollowLocationVariable`) (`self.StartingLocation`))
  (`self.SetNiagaraVariableFloat` _niagara (`self.NiagaraFollowSpeedVariable`) (`self.StartingSpeed`)))

(fn `SetNiagaraVariableFloat`
  (params (Target :type "NiagaraComponent Object Reference") (InVariableName :type Name) (InValue :type "Float (double-precision)"))
  (if (!= InVariableName "None")
    (`NiagaraComponent.SetVariableFloat` Target InVariableName InValue)))

(fn `SetNiagaraVariableVector3`
  (params (Target :type "NiagaraComponent Object Reference") (InVariableName :type Name) (InValue :type "Vector Structure"))
  (if (!= InVariableName "None")
    (`NiagaraComponent.SetVariableVec3` Target InVariableName InValue)))