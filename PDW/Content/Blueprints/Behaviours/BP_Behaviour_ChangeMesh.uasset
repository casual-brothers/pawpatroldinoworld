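; Behaviour Blueprint that swaps the mesh of a static mesh component through an ordered list of mesh and scale entries.
; Each execution applies the entry at the current index and advances it, stopping the behaviour when no duration is set or the list is exhausted.
; State changes and hiding are allowed only once every mesh has been applied and the parent checks also pass.
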(event `self.BP_ExecuteBehaviour_Implementation`
  (bind _currentmeshindex (`self.CurrentMeshIndex`))
  (bind _newmeshes (`self.NewMeshes`))
  (bind (_output_staticmesh _output_scale) (break `/Game/Blueprints/Behaviours/CustomStructs/STRUCT_MeshWithScale` (`|GetArrayItem` _newmeshes _currentmeshindex)))
  (`parent.BP_ExecuteBehaviour_Implementation`)
  (bind _asstatic_mesh_component (cast `StaticMeshComponent` (`self.GetPrimitiveComponent`)))
  (if (> (`KismetArrayLibrary.Array_Length` _newmeshes) _currentmeshindex)
    (`StaticMeshComponent.SetStaticMesh` _asstatic_mesh_component _output_staticmesh)
    (`SceneComponent.SetRelativeScale3D` _asstatic_mesh_component _output_scale)
    (`/Engine/EditorBlueprintResources/StandardMacros.IncrementInt` (`self.CurrentMeshIndex`)
      (:`  `
        (if (<= (`self.BehaviourDuration`) 0.0)
          (`self.StopBehaviour`))))
    (else
      (`self.StopBehaviour`))))

(fn `CanChangeState`
  (returns (CanChangeState :type Boolean))
  (bind _canchangestate (`parent.CanChangeState`))
  (return (and _canchangestate (`self.IsFinalMesh`))))

(fn `CanHide`
  (returns (CanDestroy :type Boolean))
  (return (and (`parent.CanHide`) (`self.IsFinalMesh`))))

(fn `IsFinalMesh`
  (returns (ReturnValue :type Boolean))
  (return (<= (`KismetArrayLibrary.Array_Length` (`self.NewMeshes`)) (`self.CurrentMeshIndex`))))