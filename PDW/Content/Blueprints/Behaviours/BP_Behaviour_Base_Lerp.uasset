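; Base behaviour that lerps a float from a starting value to ValueToReach in equal steps, one per execution.
; Tick eases between steps along ProgressionCurve and feeds SetNewValue, an empty hook for children alongside InitStartingValue.
; Stopping plays step or end audio, VFX and sequences; success notification, hiding and state changes are gated on the final step.
; Options skip steps, override the start, or reset after completion, including a timed return.
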(event `self.BP_InitBehaviour_Implementation`
  (params (NewOwnerComponent :type "SceneComponent Object Reference"))
  (`parent.BP_InitBehaviour_Implementation` NewOwnerComponent)
  (set `self.StartingValue` (`self.InitStartingValue`))
  (`self.InitValueIncrement`)
  (set `self.DefaultNotifySuccess` (`self.bNotifySuccess`)))

(event `self.BP_ExecuteBehaviour_Implementation`
  (bind _returnvalue (+ (`self.GetCurrentStepValue`) (`self.ValueIncrement`)))
  (set `self.ElapsedTime` 0.0)
  (`self.SetCurrentStep` (`self.GetCurrentValue`))
  (if (== (`self.NumberOfSteps`) (`self.CurrentStep`))
    (if (`self.KeepPlayingEffects`)
      (`self.PlayBaseEffects`))
    (set `self.bNotifySuccess` false)
    (`self.StopBehaviour`)
    (else
      (set `self.NewValue` (`KismetMathLibrary.SelectFloat` _returnvalue _returnvalue))
      (`parent.BP_ExecuteBehaviour_Implementation`))))

(event `self.BP_TickBehaviour_Implementation`
  (params (DeltaTime :type "Float (single-precision)"))
  (bind _returnvalue (`self.GetCurrentStepValue`))
  (bind _newvalue (`self.NewValue`))
  (bind _returnvalue_2 (+ (* (`CurveFloat.GetFloatValue` (`self.ProgressionCurve`) (`self.ElapsedTime`)) (- (`self.NewValue`) _returnvalue)) _returnvalue))
  (bind _returnvalue_3 (`KismetMathLibrary.NearlyEqual_FloatFloat` _newvalue _returnvalue_2 (`self.ErrorTolerance`)))
  (if (not (`self.IsWaitingForReset`))
    (set `self.ElapsedTime` (+ DeltaTime (`self.ElapsedTime`)))
    (bind _output_get (set `self.CurrentValue` (`KismetMathLibrary.SelectFloat` _newvalue _returnvalue_2 _returnvalue_3)))
    (`self.SetNewValue` _output_get)
    (if _returnvalue_3
      (if (`self.IsResetting`)
        (set `self.CurrentStep` 0)
        (else
          (`/Engine/EditorBlueprintResources/StandardMacros.IncrementInt` (`self.CurrentStep`)
            (:`  `
              _))))
      (bind _output_get_2 (set `self.CurrentValue` (`self.GetCurrentStepValue`)))
      (`self.SetNewValue` _output_get_2)
      (if (and (`self.ResetOnCompletion`) (not (`self.IsResetting`)) (`self.IsFinalStep`))
        (set `self.IsWaitingForReset` true)
        (`KismetSystemLibrary.K2_SetTimerDelegate` (`|CreateDelegate` :!event `ResetValues`) (`self.ResetTimer`))
        (else
          (set `self.IsResetting` false)
          (if (`self.IsFinalStep`)
            (set `self.bNotifySuccess` (`self.DefaultNotifySuccess`))
            (else
              (set `self.bNotifySuccess` false)))
          (`self.StopBehaviour`))))))

(event `self.BP_StopBehaviour_Implementation`
  (`self.PlayStepEffects`)
  (`self.PlayEndEffects`)
  (`parent.BP_StopBehaviour_Implementation`)
  (if (and (`self.IsFinalStep`) (`self.CanReset`))
    (set `self.CurrentValue` (`self.GetStartingValue`))
    (set `self.CurrentStep` 0)))

(fn `CanChangeState`
  (returns (CanChangeState :type Boolean))
  (bind _canchangestate (`parent.CanChangeState`))
  (return (and (`self.IsFinalStep`) _canchangestate)))

(fn `CanHide`
  (returns (CanDestroy :type Boolean))
  (return (and (`self.IsFinalStep`) (`parent.CanHide`))))

(fn `GetCurrentStepValue`
  (returns (ReturnValue :type "Float (double-precision)"))
  (return (`KismetMathLibrary.SelectFloat` (`self.ValueToReach`) (+ (* (`self.ValueIncrement`) (`self.CurrentStep`)) (`KismetMathLibrary.SelectFloat` (`self.ForcedStartingValue`) (`self.GetStartingValue`) (`self.OverrideStartingValue`))) (== (`self.NumberOfSteps`) (`self.CurrentStep`)))))

(fn `GetCurrentValue`
  (returns (CurrentValue :type "Float (double-precision)"))
  (return (`self.CurrentValue`)))

(fn `GetStartingValue`
  (returns (StartingValue :type "Float (double-precision)"))
  (return (`self.StartingValue`)))

(fn `InitStartingValue`
  (returns (StartingValue :type "Float (double-precision)"))
  (return 0.0))

(fn `InitValueIncrement`
  (bind _numberofsteps (`self.NumberOfSteps`))
  (set `self.ValueIncrement` (/ (- (`self.ValueToReach`) (`KismetMathLibrary.SelectFloat` (`self.ForcedStartingValue`) (`self.GetStartingValue`) (`self.OverrideStartingValue`))) (`KismetMathLibrary.SelectInt` _numberofsteps 1 (!= _numberofsteps 0)))))

(fn `IsFinalStep`
  (returns (ReturnValue :type Boolean))
  (return (== (`self.NumberOfSteps`) (`self.CurrentStep`))))

(fn `PlayBaseAudio`
  (`self.PlayAudio` (`self.Audio`) (`self.OwnerComponent`) (`self.InteractionType`) (`self.InteractionTypeValue`) (`self.Phase`) (`KismetMathLibrary.SelectFloat` (`KismetMathLibrary.Conv_IntToDouble` (`self.CurrentStep`)) (`self.PhaseValue`) (`self.UseStepNumber`))))

(fn `PlayEndAudio`
  (`self.PlayAudio` (`self.EndAudio`) (`self.OwnerComponent`) (`self.EndInteractionType`) (`self.EndInteractionTypeValue`) (`self.EndPhase`) (`KismetMathLibrary.SelectFloat` (`KismetMathLibrary.Conv_IntToDouble` (`self.CurrentStep`)) (`self.EndPhaseValue`) (`self.EndUseStepNumber`))))

(fn `PlayEndEffects`
  (bind _defaultnotifysuccess (`self.DefaultNotifySuccess`))
  (if (and (`self.IsFinalStep`) (or (not _defaultnotifysuccess) (and _defaultnotifysuccess (`self.bNotifySuccess`))))
    (`self.PlayEndAudio`)
    (`self.PlayEndVFX`)
    (`self.PlayEndSequence`)))

(fn `PlayEndSequence`
  (`self.PlaySequence` (`self.EndLevelSequence`) (`self.EndSettings`) (`self.EndBindingTag`) (`|MakeArray` (`ActorComponent.GetOwner` (`self.OwnerComponent`)))))

(fn `PlayEndVFX`
  (bind _ownercomponent (`self.OwnerComponent`))
  (`self.PlayVFX` (`self.EndVFX`) _ownercomponent (`self.EndVFXRotation`) (+ (`SceneComponent.K2_GetComponentLocation` _ownercomponent) (`self.EndVFXOffset`))))

(fn `PlayStepAudio`
  (`self.PlayAudio` (`self.StepAudio`) (`self.OwnerComponent`) (`self.StepInteractionType`) (`self.StepInteractionTypeValue`) (`self.StepPhase`) (`KismetMathLibrary.SelectFloat` (`KismetMathLibrary.Conv_IntToDouble` (`self.CurrentStep`)) (`self.StepPhaseValue`) (`self.StepUseStepNumber`))))

(fn `PlayStepEffects`
  (if (not (`self.IsFinalStep`))
    (`self.PlayStepAudio`)
    (`self.PlayStepVFX`)
    (`self.PlayStepSequence`)))

(fn `PlayStepSequence`
  (`self.PlaySequence` (`self.StepLevelSequence`) (`self.StepSettings`) (`self.StepBindingTag`) (`|MakeArray` (`ActorComponent.GetOwner` (`self.OwnerComponent`)))))

(fn `PlayStepVFX`
  (bind _ownercomponent (`self.OwnerComponent`))
  (`self.PlayVFX` (`self.StepVFX`) _ownercomponent (`self.StepVFXRotation`) (+ (`SceneComponent.K2_GetComponentLocation` _ownercomponent) (`self.StepVFXOffset`))))

(fn `ResetValues`
  (set `self.IsWaitingForReset` false)
  (set `self.IsResetting` true)
  (set `self.NewValue` (`self.GetStartingValue`)))

(fn `SetCurrentStep`
  (params (CurrentValue :type "Float (double-precision)"))
  (bind _forcedstartingvalue (`self.ForcedStartingValue`))
  (bind _numberofsteps (`self.NumberOfSteps`))
  (bind _returnvalue (- (`self.ValueToReach`) _forcedstartingvalue))
  (set `self.CurrentStep` (`KismetMathLibrary.SelectInt` (- _numberofsteps 1) (`KismetMathLibrary.SelectInt` (`KismetMathLibrary.Round` (* (/ (- CurrentValue _forcedstartingvalue) (`KismetMathLibrary.SelectFloat` _returnvalue 1.0 (!= _returnvalue 0.0))) _numberofsteps)) (`self.CurrentStep`) (`self.OverrideStartingValue`)) (`self.bSkipSteps`))))

(fn `SetNewValue`
  (params (NewValue :type "Float (double-precision)")))

(fn `ValueReached`
  (returns (ValueReached :type Boolean))
  (return (`KismetMathLibrary.NearlyEqual_FloatFloat` (`self.CurrentValue`) (`self.ValueToReach`) 0.02)))