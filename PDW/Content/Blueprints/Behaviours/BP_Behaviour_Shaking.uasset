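; Behaviour that shakes its owning actor around the location captured when it executes, for a set Duration.
; Each tick it lerps the actor toward that location plus a per-axis Shake offset, with alpha from DeltaTime and ShakeSpeed.
; The offset sign flips on every axis evaluation, so neighbouring axes oppose and each reverses every frame.
; A timer restores the captured location and stops the behaviour.
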(event `self.BP_ExecuteBehaviour_Implementation`
  (`parent.BP_ExecuteBehaviour_Implementation`)
  (set `self.ElapsedTime` 0.0)
  (set `self.ActorLocation` (`Actor.K2_GetActorLocation` (`ActorComponent.GetOwner` (`self.GetOwnerComponent`))))
  (`KismetSystemLibrary.K2_SetTimerDelegate` (delegate `EndEvent`) (`self.Duration`)))

(event `EndEvent`
  (`Actor.K2_SetActorRelativeLocation` (`ActorComponent.GetOwner` (`self.GetOwnerComponent`)) (`self.ActorLocation`) false false)
  (`self.StopBehaviour`))

(event `self.BP_TickBehaviour_Implementation`
  (params (DeltaTime :type "Float (single-precision)"))
  (bind (_actorlocation_x _actorlocation_y _actorlocation_z) (`KismetMathLibrary.BreakVector` (`self.ActorLocation`)))
  (bind (_shake_x _shake_y _shake_z) (`KismetMathLibrary.BreakVector` (`self.Shake`)))
  (`parent.BP_TickBehaviour_Implementation` DeltaTime)
  (bind _shakeresult (`self.AlternateShake` _shake_x))
  (bind _shakeresult_2 (`self.AlternateShake` _shake_y))
  (bind _shakeresult_3 (`self.AlternateShake` _shake_z))
  (`Actor.K2_SetActorRelativeLocation` (`ActorComponent.GetOwner` (`self.GetOwnerComponent`)) (`KismetMathLibrary.VLerp` (`Actor.K2_GetActorLocation` (`ActorComponent.GetOwner` (`self.GetOwnerComponent`))) (`KismetMathLibrary.MakeVector` (+ _shakeresult _actorlocation_x) (+ _shakeresult_2 _actorlocation_y) (+ _shakeresult_3 _actorlocation_z)) (* DeltaTime (`self.ShakeSpeed`))) false false))

(fn `AlternateShake`
  (params (ShakeValue :type "Float (double-precision)"))
  (returns (ShakeResult :type "Float (double-precision)"))
  (bind _alternate (`self.Alternate`))
  (set `self.Alternate` (* _alternate -1.0))
  (return (* ShakeValue _alternate)))