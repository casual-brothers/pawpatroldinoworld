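; Minigame behaviour for a water hose on the player's vehicle that sprays and paints at hit points.
; Tick plays the hose montage, whose notify spawns socket-attached Niagara tinted per player; stopping plays the end section and destroys it.
; Paint feeds hit point and distance-scaled lifetime to Niagara, briefly swaps in an unwrap material to set brush parameters, and triggers interactions on WaterHoseTarget hits, turning the owner component toward them.
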(event `self.BP_InitBehaviour_Implementation`
  (params (NewOwnerComponent :type "SceneComponent Object Reference")))

(event `self.BP_StopBehaviour_Implementation`
  (`|PlayMontage` (`self.SpawnerMesh`) "/Game/Art/Vehicles/Vh_01_Marshall/Animation/AM_VH_01_WaterHose.AM_VH_01_WaterHose" 1.0 0.0 "End"
    (:`then`
      (`ActorComponent.K2_DestroyComponent` (`self.NiagaraComponent`))
      (set `self.SpawnerMesh` null))))

(event `self.BP_ExecuteBehaviour_Implementation`)

(event `self.BP_TickBehaviour_Implementation`
  (params (DeltaTime :type "Float (single-precision)"))
  (`/Engine/EditorBlueprintResources/StandardMacros.IsValid` (`self.SpawnerMesh`)
    (:`Is Not Valid`
      (bind _aspdwplayer_controller (cast `PDWPlayerController` (`self.BehaviourExecutioner`)))
      (bind _returnvalue (`PDWPlayerController.GetVehicleInstance` _aspdwplayer_controller))
      (bind _output (`|GetArrayItem` (`Actor.GetComponentsByTag` _returnvalue "/Script/Engine.SkeletalMeshComponent" "ComponentTag.VehicleMesh")))
      (if (`KismetSystemLibrary.IsValid` _output)
        (bind _notifyname (`|PlayMontage` _output "/Game/Art/Vehicles/Vh_01_Marshall/Animation/AM_VH_01_WaterHose.AM_VH_01_WaterHose")
          (:`then`
            (set `self.SpawnerMesh` _output))
          (:`OnNotifyBegin`
            (if (== _notifyname "SpawnNiagara")
              (bind _returnvalue_2 (`NiagaraFunctionLibrary.SpawnSystemAttached` "/Game/Art/VFX/NiagaraSystem/MiniGame/NS_MG_MArshall_WaterHose.NS_MG_MArshall_WaterHose" _output "socket_water_hose" (0.0 0.0 0.0) (struct) "KeepRelativeOffset"))
              (set `self.NiagaraComponent` _returnvalue_2)
              (if (== _aspdwplayer_controller (`PDWGameplayFunctionLibrary.GetPlayerControllerTwo`))
                (`NiagaraComponent.SetVariableLinearColor` _returnvalue_2 "TargetColor" (make `LinearColor` 5.0 0.1 0.0 1.0))
                (else
                  (`NiagaraComponent.SetVariableLinearColor` _returnvalue_2 "TargetColor" (make `LinearColor` 0.0 1.177 3.0 1.0)))))))))))

(event `self.BP_Paint`
  (params (inHit :type "HitResult Structure (by ref)"))
  (bind _returnvalue (`self.GetOwnerComponent`))
  (bind _hitpoint (`self.HitPoint`))
  (bind _niagaracomponent (`self.NiagaraComponent`))
  (bind _comp (`self.Comp`))
  (bind _oldmaterialinstancedynamic (`self.OldMaterialInstanceDynamic`))
  (bind _comp_2 (`self.Comp`))
  (`KismetSystemLibrary.PrintString` (`KismetSystemLibrary.GetDisplayName` inHit_HitComponent) true true (struct :`G` 0.66 :`B` 1.0 :`A` 1.0) 0.0 "5151515")
  ; Valid Niagara
  (`/Engine/EditorBlueprintResources/StandardMacros.IsValid` (`self.NiagaraComponent`)
    (:`Is Valid`
      ; ValidHit Position
      (`/Engine/EditorBlueprintResources/StandardMacros.IsValid` inHit_HitActor
        (:`Is Valid`
          (set `self.HitPoint` inHit_ImpactPoint))
        (:`Is Not Valid`
          (set `self.HitPoint` inHit_TraceEnd)))
      (`NiagaraComponent.SetVariableVec3` _niagaracomponent "HitPoint" _hitpoint)
      (`NiagaraComponent.SetVariableFloat` _niagaracomponent "LifeTime" (`KismetMathLibrary.MapRangeClamped` (`KismetMathLibrary.Vector_Distance` (`SceneComponent.GetSocketLocation` (`self.SpawnerMesh`) "socket_water_hose") _hitpoint) 0.0 1000.0 0.0 1.0))
      (set `self.OldMaterialInstanceDynamic` (`self.CachedMaterialInstanceDynamic`))
      (`PrimitiveComponent.SetMaterial` _comp_2 0 (`self.UnwrapMaterial`))
      (`MeshComponent.SetVectorParameterValueOnMaterials` _comp_2 "Position" _hitpoint)
      (`MeshComponent.SetScalarParameterValueOnMaterials` _comp "Radius" (`self.BrushRadius`))
      (set `self.CachedMaterialInstanceDynamic` _oldmaterialinstancedynamic)
      (`PrimitiveComponent.SetMaterial` _comp 0 _oldmaterialinstancedynamic)
      (if (`Actor.ActorHasTag` inHit_HitActor "WaterHoseTarget")
        (bind _aspdwinteraction_receiver_component (cast `PDWInteractionReceiverComponent` inHit_HitComponent))
        (`SceneComponent.K2_SetWorldRotation` _returnvalue (`KismetMathLibrary.FindLookAtRotation` (`SceneComponent.K2_GetComponentLocation` _returnvalue) (`SceneComponent.K2_GetComponentLocation` _aspdwinteraction_receiver_component)) false false)
        (`PDWInteractionReceiverComponent.ExecuteInteractionBehaviour` _aspdwinteraction_receiver_component (`self.Behaviour Identifier`) (`self.BehaviourExecutioner`) false false)))))