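; Minigame behaviour for repeated button presses that plays a level sequence when press progress is non-zero.
; It creates the sequence, optionally binds the minigame owner's actor by tag, and sets the transform origin to that actor's PlayerStart_0 arrow.
; A CanPlay flag blocks retriggering until the sequence finishes.
; Before uninit, it unbinds the finish callback and stops the sequence.
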(event `self.BP_OnInit`
  (set `self.CanPlay` true))

(event `self.BP_ButtonPressProgress`
  (params (inInputInstance :type "InputActionInstance Structure (by ref)") (PreviousTime :type "Float (single-precision)") (CurrentTime :type "Float (single-precision)"))
  (bind _bindingtagid (`self.BindingTagID`))
  (bind _returnvalue (`ActorComponent.GetOwner` (`self.GetMiniGameOwner`)))
  (if (and (`self.CanPlay`) (!= CurrentTime 0.0))
    (set `self.CanPlay` false)
    (bind (_outactor _returnvalue_2) (`PDWGameplayFunctionLibrary.PDWCreateLevelSequence` (`self.GetControllerOwner`) (`self.In Level Sequence`) (`self.Settings`)))
    (bind _asdefault_level_sequence_instance_data (cast `DefaultLevelSequenceInstanceData` (`LevelSequenceActor.DefaultInstanceData` _outactor)))
    (if (!= _bindingtagid "None")
      (`LevelSequenceActor.SetBindingByTag` _outactor _bindingtagid (`|MakeArray` _returnvalue) false))
    (set `DefaultLevelSequenceInstanceData.TransformOrigin` (`SceneComponent.K2_GetComponentToWorld` (`|GetArrayItem` (`Actor.GetComponentsByTag` _returnvalue "/Script/Engine.ArrowComponent" "PlayerStart_0"))) _asdefault_level_sequence_instance_data)
    (`MovieSceneSequencePlayer.Play` _returnvalue_2)
    (add `MovieSceneSequencePlayer.OnFinished` _returnvalue_2 (delegate `End Sequence`))))

(event `End Sequence`
  (set `self.CanPlay` true))

(event `self.BP_BeforeUninit`
  (`/Engine/EditorBlueprintResources/StandardMacros.IsValid` (stale `self.BP_ButtonPressProgress` _returnvalue_2)
    (:`Is Valid`
      (remove `MovieSceneSequencePlayer.OnFinished` (stale `self.BP_ButtonPressProgress` _returnvalue_2) (delegate `End Sequence`))
      (`MovieSceneSequencePlayer.Stop` (stale `self.BP_ButtonPressProgress` _returnvalue_2))
      (set `self.CanPlay` false))))