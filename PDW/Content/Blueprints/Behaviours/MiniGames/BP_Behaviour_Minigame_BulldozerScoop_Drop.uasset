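; Behaviour for the bulldozer scoop minigame that handles dropping the scoop's load onto an interaction receiver.
; If the receiver is not busy, it hides the executioner's tagged mesh and plays an effect there.
; It then marks the receiver busy, spawns an actor attached to the receiver's "SpawnLocation" component and plays a second effect.
; The behaviour stops itself only when that tagged mesh is found on a non-busy receiver.
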(event `self.BP_ExecuteBehaviour_Implementation`
  (bind _ownercomponent (`self.OwnerComponent`))
  (bind _returnvalue (`ActorComponent.GetOwner` (`self.OwnerComponent`)))
  (bind _output (`|GetArrayItem` (`Actor.GetComponentsByTag` (`self.BehaviourExecutioner`) "/Script/Engine.StaticMeshComponent" (`self.Tag`))))
  (bind (_returnvalue_location _returnvalue_rotation) (`KismetMathLibrary.BreakTransform` (`SceneComponent.K2_GetComponentToWorld` (`Actor.RootComponent` _returnvalue))))
  (bind _aspdwinteraction_receiver_component (cast `PDWInteractionReceiverComponent` _ownercomponent))
  (if (!= (`PDWInteractionReceiverComponent.GetCurrentState` _aspdwinteraction_receiver_component) (`self.BusyTag`))
    (if (`KismetSystemLibrary.IsValid` _output)
      (`SceneComponent.SetVisibility` _output false false)
      (`NiagaraFunctionLibrary.SpawnSystemAtLocation` (`self.System Template`) (`SceneComponent.K2_GetComponentLocation` _output))
      (if (`KismetSystemLibrary.IsValid` _ownercomponent)
        (`PDWInteractionReceiverComponent.AddStateTag` _aspdwinteraction_receiver_component (`self.BusyTag`))
        (bind _returnvalue_2 (`|SpawnActorFromClass` (`self.Class`) (`KismetMathLibrary.MakeTransform` _returnvalue_location _returnvalue_rotation) "AlwaysSpawn" "MultiplyWithRoot" _returnvalue null))
        (`Actor.K2_AttachToComponent` _returnvalue_2 (`|GetArrayItem` (`Actor.GetComponentsByTag` _returnvalue "/Script/Engine.SceneComponent" "SpawnLocation")) "None" "SnapToTarget" "SnapToTarget" "SnapToTarget" true)
        (`NiagaraFunctionLibrary.SpawnSystemAtLocation` (`self.System Template`) _returnvalue_location _returnvalue_rotation))
      (`self.StopBehaviour`))))