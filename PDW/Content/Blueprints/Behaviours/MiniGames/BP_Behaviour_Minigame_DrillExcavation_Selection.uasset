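; Minigame behaviour that handles a selection in the drill excavation minigame.
; When executed, it asks the owning BP_Minigame_DrillExcavation to play an animation for the controller owner and triggers vibration feedback on that controller, using the vehicle-change tag.
; It then forwards a configured behaviour to the interaction receiver component of each valid current target, with the controller owner as executioner.
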(event `self.BP_ExecuteBehaviour_Implementation`
  (params (inInputInstance :type "InputActionInstance Structure (by ref)"))
  (bind _returnvalue (`self.GetControllerOwner`))
  (bind _asbp_minigame_drill_excavation (cast `/Game/Blueprints/Minigames/PupSpecific/BP_Minigame_DrillExcavation` (`ActorComponent.GetOwner` (`self.GetMiniGameOwner`)))
    (:`then`
      (`/Game/Blueprints/Minigames/PupSpecific/BP_Minigame_DrillExcavation.OnAnimationRequest_Event` _asbp_minigame_drill_excavation _returnvalue)
      (`PDWGameplayFunctionLibrary.PlayForceFeedback` (`|MakeArray` _returnvalue) (struct :`TagName` "ID.Vibration.ChangeToVehicle")))
    (:`CastFailed`
      _))
  (for _array_element (`self.CurrentTarget`)
    (`/Engine/EditorBlueprintResources/StandardMacros.IsValid` _array_element
      (:`Is Valid`
        (`PDWInteractionReceiverComponent.ExecuteInteractionBehaviour` (`Actor.GetComponentByClass` _array_element "/Game/Blueprints/Pawn/Components/BP_InteractionReceiverComponent.BP_InteractionReceiverComponent_C") (`self.BehaviourToExecute`) _returnvalue false false)))))