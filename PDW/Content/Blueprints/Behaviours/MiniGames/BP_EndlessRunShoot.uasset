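; Minigame behaviour that fires a tennis-ball skill projectile in the endless-run chase.
; When not already playing, it runs a shoot montage on the owner's "BackPack"-tagged skeletal mesh.
; The "Trigger" notify spawns the projectile at the skill socket, owned by player two, homing on any component hit by a forward sphere trace.
; The "CheckInput" notify clears the playing flag, allowing another shot.
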(event `self.BP_ExecuteBehaviour_Implementation`
  (params (inInputInstance :type "InputActionInstance Structure (by ref)"))
  (bind _in_skeletal_mesh_component (`self.In Skeletal Mesh Component`))
  (bind _returnvalue (`SceneComponent.GetSocketLocation` _in_skeletal_mesh_component "Socket_Skill"))
  (if (not (`self.PlayingMontage`))
    (bind _in_skeletal_mesh_component_2 (`self.In Skeletal Mesh Component`)
      (:`then`
        _)
      (:`else`
        (set `self.In Skeletal Mesh Component` (`|GetArrayItem` (`Actor.GetComponentsByTag` (`ActorComponent.GetOwner` (`self.GetMiniGameOwner`)) "/Script/Engine.SkeletalMeshComponent" "BackPack")))))
    (bind _notifyname (`|PlayMontage` _in_skeletal_mesh_component_2 "/Game/Art/Characters/CH_03_Chase/Animation/Backpack_Skill/AM_CH_03_Chase_Skill_TennisBall_EndlessRun.AM_CH_03_Chase_Skill_TennisBall_EndlessRun" 1.0 0.4 "0")
      (:`then`
        (set `self.PlayingMontage` true))
      (:`OnNotifyBegin`
        (if (== _notifyname "Trigger")
          (bind (_outhit _returnvalue_2) (`KismetSystemLibrary.SphereTraceSingle` _returnvalue (+ _returnvalue (* (`SceneComponent.GetForwardVector` _in_skeletal_mesh_component) 1000.0)) 50.0 "TraceTypeQuery3"))
          (bind _returnvalue_3 (`|SpawnActorFromClass` "/Game/Blueprints/Actors/Skills/BP_Skill_TennisBall_Projectile_EndlessRun.BP_Skill_TennisBall_Projectile_EndlessRun_C" (`SceneComponent.GetSocketTransform` _in_skeletal_mesh_component "Socket_Skill" "RTS_World") "Undefined" "MultiplyWithRoot" (`PDWGameplayFunctionLibrary.GetPlayerTwo`) null))
          (if _returnvalue_2
            (bind _projectilemovement1 (`/Game/Blueprints/Actors/Skills/BP_Skill_TennisBall_Projectile_EndlessRun.ProjectileMovement1` _returnvalue_3))
            (set `ProjectileMovementComponent.bIsHomingProjectile` true _projectilemovement1)
            (set `ProjectileMovementComponent.HomingTargetComponent` (`.HitComponent` (`GameplayStatics.BreakHitResult` _outhit)) _projectilemovement1)
            (set `ProjectileMovementComponent.HomingAccelerationMagnitude` 1000.0 _projectilemovement1))
          (elif (== _notifyname "CheckInput")
            (set `self.PlayingMontage` false)))))))