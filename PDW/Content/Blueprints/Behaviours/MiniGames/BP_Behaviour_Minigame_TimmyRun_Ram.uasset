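; Minigame behaviour that drives Timmy's ram animation in the TimmyRun minigame.
; On ram mode start, it casts the minigame owner's owner to BP_Minigame_TimmyRun, caches its Timmy reference and plays the ram montage.
; On ram mode stop, it jumps that montage to its End section if Timmy is still valid, so the animation finishes through its ending rather than being cut.
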(event `self.BP_OnRamModeStart`
  (bind _asbp_minigame_timmy_run (cast `/Game/Blueprints/Minigames/PupSpecific/BP_Minigame_TimmyRun` (`ActorComponent.GetOwner` (`self.GetMiniGameOwner`))))
  (bind _output_get (set `self.Timmy` (`/Game/Blueprints/Minigames/PupSpecific/BP_Minigame_TimmyRun.Timmy` _asbp_minigame_timmy_run)))
  (`Character.PlayAnimMontage` _output_get "/Game/Art/Characters/NPC_15_Timmy/Animation/AM_CH_Timmy_Ram.AM_CH_Timmy_Ram" 1.0 "None"))

(event `self.BP_OnRamModeStop`
  (bind _timmy (`self.Timmy`))
  (`/Engine/EditorBlueprintResources/StandardMacros.IsValid` _timmy
    (:`Is Valid`
      (`AnimInstance.Montage_JumpToSection` (`SkeletalMeshComponent.GetAnimInstance` (`Character.Mesh` _timmy)) "End" "/Game/Art/Characters/NPC_15_Timmy/Animation/AM_CH_Timmy_Ram.AM_CH_Timmy_Ram"))))