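; Ray trace behaviour for the drill excavation minigame that detects, highlights and reports targets under the trace.
; On each trace result it rebuilds a unique list of blocking-hit actors whose hit component is a PDWTargetingComponent.
; When the list changes, it switches custom depth and stencil on meshes tagged ActivateRender, clearing old targets and marking current ones.
; It sends the list through the event subsystem's grappling hook target event, with the moving mesh's controller as sender.
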(event `self.OnRayTraceHits`
  (params (Hits :type "Array of HitResult Structure (by ref)") (DeltaTime :type "Float (single-precision)"))
  (bind _actors (`self.Actors`))
  (bind _oldactors (`self.OldActors`))
  (bind _actors_2 (`self.Actors`))
  (`parent.OnRayTraceHits` Hits DeltaTime)
  (set `self.OldActors` _actors)
  (`KismetArrayLibrary.Array_Clear` _actors)
  (for _array_element Hits
    (if (`GameplayStatics.BreakHitResult` _array_element)
      (`/Engine/EditorBlueprintResources/StandardMacros.IsValid` (`.HitComponent` (`GameplayStatics.BreakHitResult` _array_element))
        (:`Is Valid`
          (cast `PDWTargetingComponent` (`.HitComponent` (`GameplayStatics.BreakHitResult` _array_element)))
          (bind _aspdwminigame_moving_mesh (cast `PDWMinigameMovingMesh` (`self.OwnerComponent`)))
          (`KismetArrayLibrary.Array_AddUnique` (`self.Actors`) (`.HitActor` (`GameplayStatics.BreakHitResult` _array_element)))))))
  (if (not (`KismetArrayLibrary.Array_Identical` _oldactors _actors_2))
    (`self.SetRender` _oldactors)
    (`self.SetRender` _actors_2 true 1))
  (`PDWEventSubsytem.OnGrapplingHookTargetAquiredEvent` (subsystem `PDWEventSubsytem`) _actors_2 (`PDWMinigameMovingMesh.ControllerOwner` _aspdwminigame_moving_mesh)))

(fn `SetRender`
  (params (Array :type "Array of Actor Object Reference") (CustmDepth :type Boolean) (VustomDepthStencil :type Integer))
  (for _array_element Array
    (bind _returnvalue (`Actor.GetComponentsByTag` _array_element "/Script/Engine.StaticMeshComponent" "ActivateRender"))
    (if (`KismetArrayLibrary.Array_IsNotEmpty` _returnvalue)
      (for _array_element_2 _returnvalue
        (`PrimitiveComponent.SetRenderCustomDepth` _array_element_2 CustmDepth)
        (`PrimitiveComponent.SetCustomDepthStencilValue` _array_element_2 VustomDepthStencil)))))