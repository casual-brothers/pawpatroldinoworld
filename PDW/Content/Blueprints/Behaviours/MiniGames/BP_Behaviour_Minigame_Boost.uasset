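; Minigame behaviour Blueprint that gives the owning controller's vehicle a speed boost when executed.
; After the parent implementation runs, it checks that the controller owner and its vehicle instance are valid, then calls SpeedBoost on the vehicle with the configured multiplier, duration and acceleration.
; A timer-based boost cooldown using a CanBoost flag exists in the graph but is disconnected, so the behaviour itself applies no cooldown.
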(event `self.BP_ExecuteBehaviour_Implementation`
  (params (inInputInstance :type "InputActionInstance Structure (by ref)"))
  (bind _returnvalue (`self.GetControllerOwner`))
  (`parent.BP_ExecuteBehaviour_Implementation` inInputInstance)
  (`/Engine/EditorBlueprintResources/StandardMacros.IsValid` _returnvalue
    (:`Is Valid`
      (bind _returnvalue_2 (`PDWPlayerController.GetVehicleInstance` _returnvalue))
      (`/Engine/EditorBlueprintResources/StandardMacros.IsValid` _returnvalue_2
        (:`Is Valid`
          (`PDWVehiclePawn.SpeedBoost` _returnvalue_2 (`self.Speed Multiplier`) (`self.BoostTimer`) (`self.Acceleration Value`)))))))

(event `CustomEvent`
  (set `self.bCanBoost` true))