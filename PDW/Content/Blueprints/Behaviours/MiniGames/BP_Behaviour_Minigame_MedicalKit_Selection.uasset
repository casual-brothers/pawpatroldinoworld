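; Minigame behaviour for Marshall's medical kit that treats a selected target through a shuffled button sequence.
; The first execution caches the target and its "BrokenBone"-tagged mesh, then each later one steps that bone toward zero relative transform and updates the bind.
; Niagara effects accompany each step.
; Completion disables collision, then after a short timer hides the target and notifies success.
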(event `self.BP_OnComplete`
  (`KismetSystemLibrary.K2_SetTimerDelegate` (delegate `End`) 0.75)
  (`Actor.SetActorEnableCollision` (`self.CachedActor`) false)
  (`NiagaraFunctionLibrary.SpawnSystemAttached` "/Game/Art/VFX/NiagaraSystem/MiniGame/NS_MG_Marshall_MedicalKit.NS_MG_Marshall_MedicalKit" (`Actor.RootComponent` (`|GetArrayItem` (`self.CurrentTarget`))) "None" (0.0 0.0 0.0) (struct) "KeepRelativeOffset"))

(event `End`
  (set `self.bTargetAttached` false)
  (`Actor.SetActorHiddenInGame` (`self.CachedActor`) true)
  (`NiagaraFunctionLibrary.SpawnSystemAtLocation` "/Game/Art/VFX/NiagaraSystem/MiniGame/NS_MG_Marshall_MedicalKit.NS_MG_Marshall_MedicalKit")
  (set `self.CachedActor` null)
  (`self.NotifySuccess`))

(event `self.BP_ExecuteBehaviour_Implementation`
  (params (inInputInstance :type "InputActionInstance Structure (by ref)"))
  (bind _numberofsteps (`self.NumberOfSteps`))
  (bind _brokenbone (`self.BrokenBone`))
  (bind _returnvalue (`SceneComponent.GetRelativeTransform` _brokenbone))
  (bind _output (`|GetArrayItem` (`Actor.GetComponentsByTag` (`|GetArrayItem` (`self.CurrentTarget`)) "/Script/Engine.StaticMeshComponent" "BrokenBone")))
  (if (`self.bIsValidTarget`)
    (if (`self.bTargetAttached`)
      (`/Engine/EditorBlueprintResources/StandardMacros.IsValid` _brokenbone
        (:`Is Valid`
          (`SceneComponent.K2_SetRelativeTransform` _brokenbone (`KismetMathLibrary.MakeTransform` (- (.location _returnvalue) (`self.LocationStep`)) (`KismetMathLibrary.MakeRotator` (- (.roll (.rotation _returnvalue)) (`self.RotationXStep`)) (- (.pitch (.rotation _returnvalue)) (`self.RotationYStep`)) (- (.yaw (.rotation _returnvalue)) (`self.RotationZStep`)))) false true))
        (:`Is Not Valid`
          _))
      (`NiagaraFunctionLibrary.SpawnSystemAttached` "/Game/Art/VFX/NiagaraSystem/MiniGame/NS_MG_Marshall_MedicalKit.NS_MG_Marshall_MedicalKit" (`Actor.RootComponent` (`|GetArrayItem` (`self.CurrentTarget`))) "None" (0.0 0.0 0.0) (struct) "KeepRelativeOffset")
      (`self.UpdateBind`)
      (else
        (`/Engine/EditorBlueprintResources/StandardMacros.IsValid` _output
          (:`Is Valid`
            (bind _output_get (set `self.BrokenBone` _output))
            (bind _returnvalue_2 (`SceneComponent.GetRelativeTransform` _output_get))
            (set `self.LocationStep` (/ (.location _returnvalue_2) _numberofsteps))
            (set `self.RotationXStep` (/ (.roll (.rotation _returnvalue_2)) _numberofsteps))
            (set `self.RotationYStep` (/ (.pitch (.rotation _returnvalue_2)) _numberofsteps))
            (set `self.RotationZStep` (/ (.yaw (.rotation _returnvalue_2)) _numberofsteps)))
          (:`Is Not Valid`
            _))
        (set `self.bTargetAttached` true)
        (`NiagaraFunctionLibrary.SpawnSystemAttached` "/Game/Art/VFX/NiagaraSystem/MiniGame/NS_MG_Marshall_MedicalKit.NS_MG_Marshall_MedicalKit" (`Actor.RootComponent` (`|GetArrayItem` (`self.CurrentTarget`))) "None" (0.0 0.0 0.0) (struct) "KeepRelativeOffset")
        (bind _output_get_2 (set `self.CachedActor` (`|GetArrayItem` (`self.CurrentTarget`))))
        (`self.ShuffleButtonSequence`)
        (`self.UpdateBind`)))))