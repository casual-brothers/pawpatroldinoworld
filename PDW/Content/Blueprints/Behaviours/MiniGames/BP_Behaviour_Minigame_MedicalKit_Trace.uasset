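; Ray trace behaviour for the medical kit minigame that reports when a moving mesh's trace gains or loses a target.
; On a new hit it sends the grappling-hook target-acquired event for the mesh's controller owner and plays a vibration.
; Losing the hit sends the same event once with the invalid actor, using Targeted and EventSent flags as latches.
; While a target is held, it only prints the owner component's name for debugging.
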(event `self.OnRayTraceHit`
  (params (inHitResult :type "HitResult Structure (by ref)") (DeltaTime :type "Float (single-precision)"))
  (bind _returnvalue (subsystem `PDWEventSubsytem`))
  (bind _returnvalue_2 (`KismetSystemLibrary.GetDisplayName` (`self.GetOwnerComponent`)))
  (`/Engine/EditorBlueprintResources/StandardMacros.IsValid` inHitResult_HitActor
    (:`Is Valid`
      (`/Engine/EditorBlueprintResources/StandardMacros.IsValid` inHitResult_HitComponent
        (:`Is Valid`
          (if (`self.bTargeted`)
            (`KismetSystemLibrary.PrintString` _returnvalue_2 true true (struct :`G` 0.66 :`B` 1.0 :`A` 1.0) 0.0 (`KismetStringLibrary.Conv_StringToName` _returnvalue_2))
            (else
              (bind _aspdwminigame_moving_mesh (cast `PDWMinigameMovingMesh` (`self.OwnerComponent`)))
              (bind _controllerowner (`PDWMinigameMovingMesh.ControllerOwner` _aspdwminigame_moving_mesh))
              (`PDWEventSubsytem.OnGrapplingHookTargetAquiredEvent` _returnvalue (`|MakeArray` inHitResult_HitActor) _controllerowner)
              (set `self.bTargeted` true)
              (set `self.bEventSent` false)
              (`PDWGameplayFunctionLibrary.PlayForceFeedback` (`|MakeArray` _controllerowner) (struct :`TagName` "ID.Vibration.ChangeToVehicle")))))))
    (:`Is Not Valid`
      (set `self.bTargeted` false)
      (if (not (`self.bEventSent`))
        (bind _aspdwminigame_moving_mesh_2 (cast `PDWMinigameMovingMesh` (`self.OwnerComponent`)))
        (`PDWEventSubsytem.OnGrapplingHookTargetAquiredEvent` _returnvalue (`|MakeArray` inHitResult_HitActor) (`PDWMinigameMovingMesh.ControllerOwner` _aspdwminigame_moving_mesh_2))
        (set `self.bEventSent` true)))))