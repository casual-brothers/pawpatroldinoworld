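; Grappling hook minigame behaviour that lets the player's vehicle hook a valid target and yank it loose.
; The first execution attaches a Niagara beam from a vehicle socket with looping rumble; the next impulses the physics-enabled target mesh toward the vehicle.
; Tick keeps the beam end on the pulled actor until a timer hides it, spawns rubble VFX, clears the hook effects and notifies success unless the target is fake.
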(event `self.BP_ExecuteBehaviour_Implementation`
  (params (inInputInstance :type "InputActionInstance Structure (by ref)"))
  (bind _output (`|GetArrayItem` (`self.CurrentTarget`)))
  (bind _array (`|MakeArray` (`self.GetControllerOwner`)))
  (bind _returnvalue (`SceneComponent.K2_GetComponentLocation` (`Actor.RootComponent` (`|GetArrayItem` (`self.CurrentTarget`)))))
  (bind _returnvalue_2 (`PDWPlayerController.GetVehicleInstance` (`self.GetControllerOwner`)))
  (if (`self.bIsValidTarget`)
    (if (`self.bTargetAttached`)
      (bind _output_get (set `self.TargetMesh` (`Actor.FindComponentByTag` _output "/Script/Engine.StaticMeshComponent" (`self.TargetMeshName`))))
      (`PrimitiveComponent.SetSimulatePhysics` _output_get true)
      (`PrimitiveComponent.AddImpulse` _output_get (* (`KismetMathLibrary.Normal` (- (`Actor.K2_GetActorLocation` _returnvalue_2) (`Actor.K2_GetActorLocation` _output))) (`self.AttractionFOrce`)) "None" true)
      (set `self.bTargetAttached` false)
      (set `self.CachedActor` (`|GetArrayItem` (`self.CurrentTarget`)))
      (`PDWGameplayFunctionLibrary.StopForceFeedback` _array)
      (`PDWGameplayFunctionLibrary.PlayForceFeedback` _array (struct :`TagName` "ID.Vibration.ChangeToVehicle"))
      (`KismetSystemLibrary.K2_SetTimerDelegate` (delegate `CustomEvent`) (`self.Time`))
      (else
        (bind (_returnvalue_location _returnvalue_rotation) (`KismetMathLibrary.BreakTransform` (`PDWGameplayFunctionLibrary.GetSocketTransformFromSpecificMesh` _returnvalue_2 (`self.In Socket Name`) (`self.In Mesh Tag`))))
        (bind _returnvalue_3 (`NiagaraFunctionLibrary.SpawnSystemAtLocation` "/Game/Art/VFX/NiagaraSystem/MiniGame/NS_MG_Chase_GrapplingHook1.NS_MG_Chase_GrapplingHook1" _returnvalue_location _returnvalue_rotation))
        (set `self.HookVFX` _returnvalue_3)
        (set `self.Winch` _returnvalue_3)
        (set `self.bTargetAttached` true)
        (`NiagaraComponent.SetNiagaraVariableVec3` _returnvalue_3 "BeamEndPoint" _returnvalue)
        (`NiagaraComponent.SetNiagaraVariableVec3` _returnvalue_3 "BeamStartPoint" _returnvalue_location)
        (`self.UpdateBind`)
        (bind _returnvalue_4 (`NiagaraFunctionLibrary.SpawnSystemAtLocation` (`self.GrapplingVfx`) _returnvalue))
        (set `self.IvyShakeVfx` _returnvalue_4)
        (`FMODBlueprintStatics.PlayEvent2D` "/Game/FMOD/Events/MINI_GAME/Chase/minigame_grabbling_hook_shot.minigame_grabbling_hook_shot")
        (`PDWGameplayFunctionLibrary.PlayForceFeedback` (`|MakeArray` (`self.GetControllerOwner`)) (struct :`TagName` "ID.Vibration.Bark") "None" true)))))

(event `CustomEvent`
  (bind _cachedactor (`self.CachedActor`))
  (bind _winch (`self.Winch`))
  (bind _cachedactor_2 (`self.CachedActor`))
  (bind _ivyshakevfx (`self.IvyShakeVfx`))
  (`Actor.SetActorHiddenInGame` _cachedactor true)
  (`NiagaraFunctionLibrary.SpawnSystemAtLocation` "/Game/Art/VFX/NiagaraSystem/MiniGame/NS_MG_Rubble_BulldozerScoop_Pickup.NS_MG_Rubble_BulldozerScoop_Pickup" (`SceneComponent.K2_GetComponentLocation` (`Actor.RootComponent` _cachedactor)))
  (`Actor.SetActorEnableCollision` _cachedactor false)
  (`/Engine/EditorBlueprintResources/StandardMacros.IsValid` _ivyshakevfx
    (:`Is Valid`
      (`ActorComponent.K2_DestroyComponent` _ivyshakevfx))
    (:`Is Not Valid`
      _))
  (`/Engine/EditorBlueprintResources/StandardMacros.IsValid` _winch
    (:`Is Valid`
      (`ActorComponent.K2_DestroyComponent` _winch)
      (`/Engine/EditorBlueprintResources/StandardMacros.IsValid` _cachedactor_2
        (:`Is Valid`
          (`self.UpdateBind`)
          (`PrimitiveComponent.SetSimulatePhysics` (`self.TargetMesh`) false)
          (if (not (`PDWTargetingComponent.IsFakeTarget` (`Actor.FindComponentByTag` _cachedactor_2 "/Script/PDW.PDWTargetingComponent" "TargetingComp")))
            (`self.NotifySuccess`))
          (set `self.CachedActor` null))))))

(event `self.BP_UninitializeBehaviour`
  (bind _hookvfx (`self.HookVFX`))
  (`/Engine/EditorBlueprintResources/StandardMacros.IsValid` _hookvfx
    (:`Is Valid`
      (`ActorComponent.K2_DestroyComponent` _hookvfx)
      (`ActorComponent.K2_DestroyComponent` (`self.IvyShakeVfx`))
      (set `self.bTargetAttached` false))))

(event `self.BP_CustomTick_Implementation`
  (params (inDeltaTime :type "Float (single-precision)"))
  (bind _winch (`self.Winch`))
  (bind _cachedactor (`self.CachedActor`))
  (`/Engine/EditorBlueprintResources/StandardMacros.IsValid` _cachedactor
    (:`Is Valid`
      (`/Engine/EditorBlueprintResources/StandardMacros.IsValid` _winch
        (:`Is Valid`
          (`NiagaraComponent.SetNiagaraVariableVec3` _winch "BeamEndPoint" (`SceneComponent.K2_GetComponentLocation` (`Actor.RootComponent` _cachedactor))))))))