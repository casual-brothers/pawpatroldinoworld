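; Behaviour Blueprint for the grappling hook minigame that reports when its ray trace gains or loses a target.
; A hit on a PDW targeting component sends the hit actor through the PDW event subsystem's target-acquired event, along with the owning moving mesh's controller.
; Any other result clears the targeted state and sends the same event with an empty target.
; Two flags stop repeat events while the state is unchanged.
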(event `self.OnRayTraceHit`
  (params (inHitResult :type "HitResult Structure (by ref)") (DeltaTime :type "Float (single-precision)"))
  (bind _returnvalue (subsystem `PDWEventSubsytem`))
  (`/Engine/EditorBlueprintResources/StandardMacros.IsValid` inHitResult_HitComponent
    (:`Is Valid`
      (cast `PDWTargetingComponent` inHitResult_HitComponent
        (:`then`
          (if (not (`self.bTargeted`))
            (bind _aspdwminigame_moving_mesh (cast `PDWMinigameMovingMesh` (`self.OwnerComponent`)))
            (`PDWEventSubsytem.OnGrapplingHookTargetAquiredEvent` _returnvalue (`|MakeArray` inHitResult_HitActor) (`PDWMinigameMovingMesh.ControllerOwner` _aspdwminigame_moving_mesh))
            (set `self.bTargeted` true)
            (set `self.bEventSent` false)))
        (:`CastFailed`
          (set `self.bTargeted` false :!label _label)
          (if (not (`self.bEventSent`))
            (bind _aspdwminigame_moving_mesh_2 (cast `PDWMinigameMovingMesh` (`self.OwnerComponent`)))
            (`PDWEventSubsytem.OnGrapplingHookTargetAquiredEvent` _returnvalue (`|MakeArray` null :!type "Actor Object Reference") (`PDWMinigameMovingMesh.ControllerOwner` _aspdwminigame_moving_mesh_2))
            (set `self.bEventSent` true)))))
    (:`Is Not Valid`
      (goto _label))))