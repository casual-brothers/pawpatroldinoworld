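; Behaviour that releases a specified item from the interacting player, used for minigame objects such as sea rescue targets.
; On execute, it looks up the item in the executioner's player state, detaches it and disables collision on its interaction receiver.
; Sea rescue targets snap to their unload point when valid, and deployable minigame components are notified of the detach.
; The behaviour stops immediately and exposes the detached item through GetItem.
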(event `self.BP_ExecuteBehaviour_Implementation`
  (bind _item (`self.Item`))
  (bind _itemtoremove (`self.ItemToRemove`))
  (bind _aspdwplayer_interface (cast `PDWPlayerInterface` (`self.BehaviourExecutioner`))
    (:`then`
      (bind _returnvalue (`PDWPlayerInterface.GetPDWPlayerState` _aspdwplayer_interface))
      (bind _returnvalue_2 (`PDWPlayerState.CheckItem` _returnvalue _itemtoremove))
      (if _returnvalue_2
        (bind _returnvalue_3 (`PDWPlayerState.GetItem` _returnvalue _itemtoremove))
        (set `self.Item` _returnvalue_3)
        (`Actor.K2_DetachFromActor` _item "KeepWorld" "KeepWorld" "KeepRelative")
        (bind _asbp_minigame_sea_rescue_target (cast `/Game/Blueprints/Actors/MiniGames/SeaRescue/BP_Minigame_SeaRescue_Target` _item)
          (:`then`
            (bind _unloadtargetpoint (`/Game/Blueprints/Actors/MiniGames/SeaRescue/BP_Minigame_SeaRescue_Target.UnloadTargetPoint` _asbp_minigame_sea_rescue_target))
            (`/Engine/EditorBlueprintResources/StandardMacros.IsValid` _unloadtargetpoint
              (:`Is Valid`
                (`Actor.K2_AttachToActor` _item _unloadtargetpoint "None" "SnapToTarget" "SnapToTarget" "SnapToTarget" true))
              (:`Is Not Valid`
                _)))
          (:`CastFailed`
            _))
        (`PrimitiveComponent.SetCollisionEnabled` (`Actor.GetComponentByClass` _item "/Script/PDW.PDWInteractionReceiverComponent") "NoCollision")
        (bind _aspdwminigame_actor_interface (cast `PDWMinigameActorInterface` (`self.Item`))
          (:`then`
            (bind _returnvalue_4 (`PDWMinigameActorInterface.BP_GetMinigameTargetComponent` _aspdwminigame_actor_interface))
            (bind _aspdwdeployable_component (cast `PDWDeployableComponent` _returnvalue_4)
              (:`then`
                (`PDWDeployableComponent.OnObjectDetached` _aspdwdeployable_component))
              (:`CastFailed`
                _)))
          (:`CastFailed`
            _))))
    (:`CastFailed`
      _))
  (`self.StopBehaviour`))

(fn `GetItem`
  (returns (Item :type "Actor Object Reference"))
  (return (`self.Item`)))