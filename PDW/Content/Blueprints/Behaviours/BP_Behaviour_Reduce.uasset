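; BP_Behaviour_Reduce is a behaviour Blueprint that drives the uniform relative scale of a primitive component, presumably to shrink it as the name suggests.
; Initialisation runs the parent logic, then resets a valid component's scale to one.
; It overrides the value hooks: the starting value is one, new values set all three axes, and the current value reads relative X scale, or zero without a valid component.
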(event `self.BP_InitBehaviour_Implementation`
  (params (NewOwnerComponent :type "SceneComponent Object Reference"))
  (bind _primitivecomponent (`self.GetPrimitiveComponent`))
  (`parent.BP_InitBehaviour_Implementation` NewOwnerComponent)
  (`/Engine/EditorBlueprintResources/StandardMacros.IsValid` _primitivecomponent
    (:`Is Valid`
      (`SceneComponent.SetRelativeScale3D` _primitivecomponent (1.0 1.0 1.0)))))

(fn `GetCurrentValue`
  (returns (CurrentValue :type "Float (double-precision)"))
  (bind _primitivecomponent (`self.GetPrimitiveComponent`))
  (bind _relativescale3d_x (`KismetMathLibrary.BreakVector` (`SceneComponent.RelativeScale3D` _primitivecomponent)))
  (`/Engine/EditorBlueprintResources/StandardMacros.IsValid` _primitivecomponent
    (:`Is Valid`
      (return _relativescale3d_x))
    (:`Is Not Valid`
      (return 0.0))))

(fn `InitStartingValue`
  (returns (StartingValue :type "Float (double-precision)"))
  (return 1.0))

(fn `SetNewValue`
  (params (NewValue :type "Float (double-precision)"))
  (`SceneComponent.SetRelativeScale3D` (`self.GetPrimitiveComponent`) (`KismetMathLibrary.Conv_DoubleToVector` NewValue)))