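; Interaction behaviour that runs a timed countdown on its owner, showing progress on a tinted, optionally hidden circular loading-icon widget.
; Tick advances the timer and feeds the icon material's Percentage parameter, notifying success and stopping on completion.
; The executioner ending overlap or the receiver losing collision interrupts it, skipping end audio, VFX and sequence.
; Interruption also blocks state change and hiding through parent-check overrides.
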(event `self.BP_ExecuteBehaviour_Implementation`
  (bind _returnvalue (`ActorComponent.GetOwner` (`self.OwnerComponent`)))
  (bind _output (`|GetArrayItem` (`Actor.GetComponentsByTag` _returnvalue "/Game/Blueprints/UI/WidgetComponent/BP_BaseWidgetComponent.BP_BaseWidgetComponent_C" "LoadingIcon")))
  (`parent.BP_ExecuteBehaviour_Implementation`)
  (set `self.bNotifySuccess` false)
  (set `self.TimerInterrupted` false)
  (set `self.CurrentTimer` 0.0)
  (set `self.ActiveTimer` true)
  (`/Engine/EditorBlueprintResources/StandardMacros.IsValid` _output
    (:`Is Valid`
      (bind _output_get (set `self.LoadingIconComponent` _output))
      (bind _asbpw_loading_icon (cast `/Game/Blueprints/UI/Widgets/BPW_LoadingIcon` (`WidgetComponent.GetWidget` _output_get)))
      (`Image.SetBrushTintColor` (`/Game/Blueprints/UI/Widgets/BPW_LoadingIcon.CircularProgress` _asbpw_loading_icon) (`self.CustomTint`))
      (`SceneComponent.SetHiddenInGame` _output_get (`self.HideUI`) false)
      (`self.SetLoadingIcon` 0.0))
    (:`Is Not Valid`
      (`KismetSystemLibrary.PrintText` " WIDGET NOT FOUND")))
  ; Stop Timer if Overlap Ends
  (add `PrimitiveComponent.OnComponentEndOverlap` (`Actor.GetComponentByClass` _returnvalue "/Game/Blueprints/Pawn/Components/BP_InteractionReceiverComponent.BP_InteractionReceiverComponent_C") (delegate `CancelTimer`)))

(event `CancelTimer`
  (params (OverlappedComponent :type "PrimitiveComponent Object Reference") (OtherActor :type "Actor Object Reference") (OtherComp :type "PrimitiveComponent Object Reference") (OtherBodyIndex :type Integer))
  ; Stop Timer if Overlap Ends
  (if (== OtherActor (`self.BehaviourExecutioner`))
    (`self.InterruptBehaviour`)))

(event `self.BP_TickBehaviour_Implementation`
  (params (DeltaTime :type "Float (single-precision)"))
  (`parent.BP_TickBehaviour_Implementation` DeltaTime)
  (if (`PrimitiveComponent.K2_IsCollisionEnabled` (`Actor.GetComponentByClass` (`ActorComponent.GetOwner` (`self.OwnerComponent`)) "/Game/Blueprints/Pawn/Components/BP_InteractionReceiverComponent.BP_InteractionReceiverComponent_C"))
    (if (`self.ActiveTimer`)
      (set `self.CurrentTimer` (+ DeltaTime (`self.CurrentTimer`)))
      (`self.SetLoadingIcon` (`KismetMathLibrary.SelectFloat` 1.0 (/ (`self.CurrentTimer`) (`self.Timer`)) (`self.HasTimerEnded`)))
      (if (`self.HasTimerEnded`)
        (set `self.bNotifySuccess` true)
        (`self.StopBehaviour`)))
    (else
      (`self.InterruptBehaviour`))))

(event `self.BP_StopBehaviour_Implementation`
  (remove `PrimitiveComponent.OnComponentEndOverlap` (`Actor.GetComponentByClass` (`ActorComponent.GetOwner` (`self.OwnerComponent`)) "/Game/Blueprints/Pawn/Components/BP_InteractionReceiverComponent.BP_InteractionReceiverComponent_C") (delegate `CancelTimer`))
  (if (not (`self.TimerInterrupted`))
    (`self.PlayEndEffects`))
  (set `self.ActiveTimer` false)
  (`SceneComponent.SetHiddenInGame` (`self.LoadingIconComponent`) true false)
  (`parent.BP_StopBehaviour_Implementation`))

(fn `CanChangeState`
  (returns (CanChangeState :type Boolean))
  (bind _canchangestate (`parent.CanChangeState`))
  (return (and _canchangestate (not (`self.TimerInterrupted`)))))

(fn `CanHide`
  (returns (CanDestroy :type Boolean))
  (return (and (`parent.CanHide`) (not (`self.TimerInterrupted`)))))

(fn `HasTimerEnded`
  (returns (ReturnValue :type Boolean))
  (bind _timer (`self.Timer`))
  (bind _currenttimer (`self.CurrentTimer`))
  (return (or (`KismetMathLibrary.NearlyEqual_FloatFloat` _currenttimer _timer (`self.ErrorTolerance`)) (>= _currenttimer _timer))))

(fn `InterruptBehaviour`
  (set `self.TimerInterrupted` true)
  (set `self.ActiveTimer` false)
  (`SceneComponent.SetHiddenInGame` (`self.LoadingIconComponent`) true false)
  (`self.StopBehaviour`))

(fn `IsTimerInterrupted`
  (returns (TimerInterrupted :type Boolean))
  (return (`self.TimerInterrupted`)))

(fn `PlayEndAudio`
  (`self.PlayAudio` (`self.EndAudio`) (`self.OwnerComponent`) (`self.EndInteractionType`) (`self.EndInteractionTypeValue`) (`self.EndPhase`) (`self.EndPhaseValue`)))

(fn `PlayEndEffects`
  (`self.PlayEndAudio`)
  (`self.PlayEndVFX`)
  (`self.PlayEndSequence`))

(fn `PlayEndSequence`
  (`self.PlaySequence` (`self.EndLevelSequence`) (`self.EndSettings`) (`self.EndBindingTag`) (`|MakeArray` (`ActorComponent.GetOwner` (`self.OwnerComponent`)))))

(fn `PlayEndVFX`
  (bind _ownercomponent (`self.OwnerComponent`))
  (`self.PlayVFX` (`self.EndVFX`) _ownercomponent (`self.EndVFXRotation`) (+ (`SceneComponent.K2_GetComponentLocation` _ownercomponent) (`self.EndVFXOffset`))))

(fn `SetLoadingIcon`
  (params (Value :type "Float (single-precision)"))
  (bind _asbpw_loading_icon (cast `/Game/Blueprints/UI/Widgets/BPW_LoadingIcon` (`WidgetComponent.GetWidget` (`self.LoadingIconComponent`))))
  (bind _returnvalue (`Image.GetDynamicMaterial` (`/Game/Blueprints/UI/Widgets/BPW_LoadingIcon.CircularProgress` _asbpw_loading_icon)))
  (`MaterialInstanceDynamic.SetScalarParameterValue` _returnvalue "Percentage" Value))