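; A behaviour Blueprint that toggles a named boolean variable on a Niagara effect as the behaviour runs.
; Init writes the inverse of the configured value, Execute writes the value itself, and Stop restores the inverse, each after calling the parent implementation.
; The tick override is disabled, so the variable changes only on those lifecycle events.
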(event `self.BP_InitBehaviour_Implementation`
  (params (NewOwnerComponent :type "SceneComponent Object Reference"))
  (`parent.BP_InitBehaviour_Implementation` NewOwnerComponent)
  (`NiagaraComponent.SetVariableBool` (`self.GetNiagara`) (`self.VariableName`) (not (`self.ValueToSet`))))

(event `self.BP_ExecuteBehaviour_Implementation`
  (`parent.BP_ExecuteBehaviour_Implementation`)
  (`NiagaraComponent.SetVariableBool` (`self.GetNiagara`) (`self.VariableName`) (`self.ValueToSet`)))

(event `self.BP_StopBehaviour_Implementation`
  (`parent.BP_StopBehaviour_Implementation`)
  (`NiagaraComponent.SetVariableBool` (`self.GetNiagara`) (`self.VariableName`) (not (`self.ValueToSet`))))