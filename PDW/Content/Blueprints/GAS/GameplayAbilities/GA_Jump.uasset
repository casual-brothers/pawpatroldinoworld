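; GA_Jump is a Gameplay Ability that makes the player-controlled PDWCharacter jump.
; After a cooldown check, it commits, binds the character's landed delegate and calls Jump.
; Landing unbinds the delegate and ends the ability.
; A tag-wait task watches for GAS.DisableSkills, removing GE_DisableSkill and cancelling the ability if that tag is added.
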(event `self.K2_ActivateAbility`
  (bind _returnvalue (`self.K2_CheckAbilityCooldown`))
  (if _returnvalue
    (`self.K2_CommitAbility`)
    (`AbilityTask_WaitGameplayTagAdded.WaitGameplayTagAdd` (struct :`TagName` "GAS.DisableSkills") null
      (:`then`
        (bind _aspdwcharacter (cast `PDWCharacter` (`Controller.K2_GetPawn` (`self.PlayerController`))))
        (set `self.PDWCharacter` _aspdwcharacter)
        (add `Character.LandedDelegate` _aspdwcharacter (delegate `LandedDelegate_Event`))
        (`Character.Jump` _aspdwcharacter))
      (:`Added`
        (`AbilitySystemComponent.RemoveActiveGameplayEffectBySourceEffect` (`self.GetAbilitySystemComponentFromActorInfo`) "/Game/Blueprints/GAS/GameplayEffects/GE_DisableSkill.GE_DisableSkill_C" null -1)
        (`self.K2_CancelAbility`)))))

(event `LandedDelegate_Event`
  (params (Hit :type "HitResult Structure (by ref)"))
  (remove `Character.LandedDelegate` (`self.PDWCharacter`) (delegate `LandedDelegate_Event`))
  (`self.K2_EndAbility`))