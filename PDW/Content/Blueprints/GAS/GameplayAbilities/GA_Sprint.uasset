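; GA_Sprint is a gameplay ability that applies a boost effect while the player's pawn moves fast along a steady line.
; On activation, unless sprint is disabled, a looping half-second timer compares pawn speed to an attribute threshold and current direction to the last sample using an absolute dot product.
; The effect toggles only on state changes through the PlayerController's GAS component.
; Ending the ability clears the timer and removes the effect.
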(event `self.K2_OnEndAbility`
  (params (bWasCancelled :type Boolean))
  (`KismetSystemLibrary.K2_InvalidateTimerHandle` (`self.NewVar`))
  (`AbilitySystemComponent.RemoveActiveGameplayEffect` (`PDWPlayerController.GASComponent` (`self.PlayerController`)) (`self.Handle`) -1))

(event `self.K2_ActivateAbility`
  (if (not (`PDWPlayerController.GetSprintDisabled` (`self.PlayerController`)))
    (bind _returnvalue (`KismetSystemLibrary.K2_SetTimerDelegate` (delegate `CustomEvent`) 0.5 true))
    (set `self.NewVar` _returnvalue)))

(event `CustomEvent`
  (bind _playercontroller (`self.PlayerController`))
  (if (`PDWPlayerController.GetSprintDisabled` (`self.PlayerController`))
    _
    (elif (> (* (`KismetMathLibrary.VSize` (`Actor.GetVelocity` (`Controller.K2_GetPawn` _playercontroller))) 0.01) (* (`.ReturnValue` (`AbilitySystemBlueprintLibrary.GetFloatAttribute` _playercontroller (struct :`AttributeName` "CharacterSpeed" :`Attribute` "/Script/PDW.PDWAttributeSet:CharacterSpeed" :`AttributeOwner` "/Script/CoreUObject.Class'/Script/PDW.PDWAttributeSet'"))) 0.9))
      (if (> (`KismetMathLibrary.Abs` (`KismetMathLibrary.Dot_VectorVector` (`KismetMathLibrary.Normal` (`self.LastSpeed`)) (`KismetMathLibrary.Normal` (`Actor.GetVelocity` (`Controller.K2_GetPawn` (`self.PlayerController`)))))) (- 1.0 (`self.Tollerance`)))
        (`self.SetEffectActive` true)
        (else
          (`self.SetEffectActive` false)))
      (set `self.LastSpeed` (`Actor.GetVelocity` (`Controller.K2_GetPawn` (`self.PlayerController`))))
      (else
        (`self.SetEffectActive` false)))))

(event `SetEffectActive`
  (params (bValue :type Boolean))
  (bind _playercontroller (`self.PlayerController`))
  (if (!= (`self.bEffectActive`) bValue)
    (bind _output_get (set `self.bEffectActive` bValue))
    (if _output_get
      (bind _returnvalue (`AbilitySystemComponent.BP_ApplyGameplayEffectToSelf` :`self` (`PDWPlayerController.GASComponent` _playercontroller) :`GameplayEffectClass` (`self.BoostEffect`)))
      (set `self.Handle` _returnvalue)
      (else
        (`AbilitySystemComponent.RemoveActiveGameplayEffect` (`PDWPlayerController.GASComponent` _playercontroller) (`self.Handle`) -1)))))