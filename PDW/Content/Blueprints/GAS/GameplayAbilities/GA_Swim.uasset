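; GA_Swim is a Gameplay Ability that puts a character into the swimming state.
; On activation it adds its player-state container, sets the PDWAnimInstance animation state to Swimming, commits and applies GE_Swim to itself.
; Cancel and end share cleanup that removes those player states and restores the Walking animation state.
; Only the end path also removes active effects granting the InteractionState.Swimming tag.
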(event `self.K2_ActivateAbility`
  (bind _returnvalue (`self.GetAbilitySystemComponentFromActorInfo`))
  (bind _playerstate (`self.PlayerState`))
  (`/Engine/EditorBlueprintResources/StandardMacros.IsValid` _playerstate
    (:`Is Valid`
      (`PDWPlayerState.AddPlayerStates` _playerstate (`self.PlayerStateContainer`))
      (bind _returnvalue_2 (`self.GetAnimInstance`))
      (bind _aspdwanim_instance (cast `PDWAnimInstance` _returnvalue_2))
      (`PDWAnimInstance.SetAnimationState` _aspdwanim_instance "Swimming")
      (`self.K2_CommitAbility`)
      (`AbilitySystemComponent.BP_ApplyGameplayEffectToSelf` _returnvalue "/Game/Blueprints/GAS/GameplayEffects/GE_Swim.GE_Swim_C" 0.0 (`AbilitySystemComponent.MakeEffectContext` _returnvalue)))))

(event `self.BP_OnCancelAbility`
  (bind _playerstate (`self.PlayerState`))
  (`/Engine/EditorBlueprintResources/StandardMacros.IsValid` _playerstate :!label _label
    (:`Is Valid`
      (`PDWPlayerState.RemovePlayerStates` _playerstate (`self.PlayerStateContainer`))
      (bind _returnvalue (`self.GetAnimInstance`))
      (bind _aspdwanim_instance (cast `PDWAnimInstance` _returnvalue))
      (`PDWAnimInstance.SetAnimationState` _aspdwanim_instance "Walking"))))

(event `self.K2_OnEndAbility`
  (params (bWasCancelled :type Boolean))
  (`AbilitySystemComponent.RemoveActiveEffectsWithGrantedTags` (`self.GetAbilitySystemComponentFromActorInfo`) (struct :`GameplayTags` (struct :`(TagName` "InteractionState.Swimming"))))
  (goto _label))