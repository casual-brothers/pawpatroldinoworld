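; Gameplay Ability that plays the vehicle horn (clacson) while its input is held.
; On activation it plays the FMOD-style Vehicle_clacson event at the controlled pawn's location and sets its clacson_type parameter from the vehicle instance's type.
; Releasing the input cancels the ability, and ending it stops and releases the stored event instance.
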(event `self.K2_ActivateAbility`
  (bind _playercontroller (`self.PlayerController`))
  (bind _returnvalue (`FMODBlueprintStatics.PlayEventAtLocation` "/Game/FMOD/Events/VEHICLE/Clacson/vehicle_clacson.vehicle_clacson" (`Actor.GetTransform` (`Controller.K2_GetPawn` _playercontroller))))
  (bind _output_get (set `self.NewVar` _returnvalue))
  (bind _returnvalue_2 (`PDWPlayerController.GetVehicleInstance` _playercontroller))
  (switch `EVehicleType` (`PDWVehiclePawn.VehicleType` _returnvalue_2)
    (:`Vehicle`
      (set `self.Value` 0.0))
    (:`Truck`
      (set `self.Value` 1.0))
    (:`Special`
      (set `self.Value` 2.0))
    (:`WithSiren`
      (set `self.Value` 3.0)))
  (`FMODBlueprintStatics.EventInstanceSetParameter` _output_get "clacson_type" (`self.Value`)))

(event `self.BP_OnReleaseInput`
  (`self.K2_CancelAbility`))

(event `self.K2_OnEndAbility`
  (params (bWasCancelled :type Boolean))
  (`FMODBlueprintStatics.EventInstanceStop` (`self.NewVar`) true))