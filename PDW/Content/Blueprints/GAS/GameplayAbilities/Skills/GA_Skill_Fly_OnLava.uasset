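; GA_Skill_Fly_OnLava is a skill gameplay ability, named for flying on lava, that manages actors spawned during the skill.
; After the parent trigger logic runs, it attaches SpawnedActor to PlayerController with world transforms kept and records it uniquely in SpawnedActors.
; When the ability ends, it calls the parent end logic and destroys every recorded actor.
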(event `self.K2_OnEndAbility`
  (params (bWasCancelled :type Boolean))
  (`parent.K2_OnEndAbility` false)
  (for _array_element (`self.SpawnedActors`)
    (`Actor.K2_DestroyActor` _array_element)))

(event `self.TriggerAbilityLogic`
  (bind _spawnedactor (`self.SpawnedActor`))
  (`parent.TriggerAbilityLogic`)
  (`Actor.K2_AttachToActor` _spawnedactor (`self.PlayerController`) "None" "KeepWorld" "KeepWorld" "KeepWorld" true)
  (`KismetArrayLibrary.Array_AddUnique` (`self.SpawnedActors`) _spawnedactor))