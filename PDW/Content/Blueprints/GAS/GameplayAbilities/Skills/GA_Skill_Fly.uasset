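; GA_Skill_Fly is a flight skill gameplay ability that builds on its parent's trigger and end logic.
; On trigger it snaps the spawned actor to the mesh component and binds to the teleport-confirm event, which cancels the ability.
; On end it destroys each spawned actor and unbinds that event inside the same loop, so unbinding only runs when spawned actors exist.
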(event `self.K2_OnEndAbility`
  (params (bWasCancelled :type Boolean))
  (`parent.K2_OnEndAbility` false)
  (for _array_element (`self.SpawnedActors`)
    (`Actor.K2_DestroyActor` _array_element)
    (remove `PDWEventSubsytem.OnTeleportConfirm` (subsystem `PDWEventSubsytem`) (delegate `CustomEvent`))))

(event `self.TriggerAbilityLogic`
  (`parent.TriggerAbilityLogic`)
  (`Actor.K2_AttachToComponent` (`self.SpawnedActor`) (`self.MeshComp`) "None" "SnapToTarget" "SnapToTarget" "KeepRelative" true)
  (add `PDWEventSubsytem.OnTeleportConfirm` (subsystem `PDWEventSubsytem`) (delegate `CustomEvent`)))

(event `CustomEvent`
  (`self.K2_CancelAbility`))