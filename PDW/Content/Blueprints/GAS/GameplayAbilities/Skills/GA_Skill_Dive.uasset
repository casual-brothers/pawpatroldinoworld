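; Dive skill ability that puts the character and its backpack mesh into diving mode for a limited swim time.
; On trigger it sets DivingState, makes the capsule block a custom channel and attaches the spawned actor.
; Tick counts down the duration, which loop requests reset, then plays an emersion montage back to walking.
; A leaving-swimming-area event or close hit from a downward spine trace ends the dive without that montage.
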(event `self.TriggerAbilityLogic`
  (`parent.TriggerAbilityLogic`)
  (`PDWPlayerState.AddPlayerStates` (`self.PlayerState`) (`self.DivingState`))
  (bind _returnvalue (`self.GetAnimInstance`))
  (bind _aspdwanim_instance (cast `PDWAnimInstance` _returnvalue))
  (bind _output_get (set `self.As PDWAnim Instance` _aspdwanim_instance))
  (`PDWAnimInstance.SetDivingMode` _output_get true)
  (bind _ascapsule_collision (cast `CapsuleComponent` (`Actor.RootComponent` (`Controller.K2_GetPawn` (`self.PlayerController`)))))
  (bind _output_get_2 (set `self.As Capsule Collision` _ascapsule_collision))
  (`PrimitiveComponent.SetCollisionResponseToChannel` _output_get_2 "ECC_GameTraceChannel7" "ECR_Block")
  (`Actor.K2_AttachToActor` (`self.SpawnedActor`) (`self.PlayerController`) "None" "KeepWorld" "KeepWorld" "KeepWorld" true)
  (bind _aspdwanim_instance_2 (cast `PDWAnimInstance` (`SkeletalMeshComponent.GetAnimInstance` (`|GetArrayItem` (`Actor.GetComponentsByTag` (`Controller.K2_GetPawn` (`self.PlayerController`)) "/Script/Engine.SkeletalMeshComponent" "ComponentTag.SkillMesh")))))
  (set `self.BackpackAnimInstance` _aspdwanim_instance_2)
  (`PDWAnimInstance.SetDivingMode` _aspdwanim_instance_2 true)
  (`Actor.K2_AttachToComponent` (`self.SpawnedActor`) (`self.MeshComp`) "None" "SnapToTarget" "SnapToTarget" "KeepRelative" true)
  (bind (_asynctaskproxy _payload) (`AbilityTask_WaitGameplayEvent.WaitGameplayEvent` (struct :`TagName` "Event.LeavingSwimmingArea") null)
    (:`EventReceived`
      (if (== (`.Target` (break `GameplayEventData` _payload)) (`self.PlayerController`))
        (bind _returnvalue_2 (`self.GetAnimInstance` :!label _label))
        (`AnimInstance.Montage_Stop` _returnvalue_2 0.0 null)
        (`PDWPlayerState.RemovePlayerStates` (`self.PlayerState`) (`self.DivingState`))
        (`PDWAnimInstance.SetDivingMode` (`self.As PDWAnim Instance`) false)
        (`PDWAnimInstance.SetDivingMode` (`self.BackpackAnimInstance`) false)
        (set `self.bStopTick` true)
        (`self.K2_EndAbility`)))))

(event `self.K2_ActivateAbility`)

(event `self.K2_Tick`
  (params (DeltaTime :type "Float (single-precision)"))
  (bind _returnvalue (`SceneComponent.GetSocketLocation` (`self.MeshComp`) "spine_02_skin"))
  (`|ExecutionSequence`
    (:`then_0`
      (if (not (`self.bStopTick`))
        (set `self.SwimDuration` (- (`self.SwimDuration`) DeltaTime))
        (if (<= (`self.SwimDuration`) 0.0)
          (`self.HandleEmersion`))))
    (:`then_1`
      (bind _returnvalue_2 (`self.GetAnimInstance`))
      (bind _outhit (`KismetSystemLibrary.LineTraceSingle` _returnvalue (+ _returnvalue (0.0 0.0 -200.0)) "TraceTypeQuery1" false (`|MakeArray` (`AnimInstance.GetOwningActor` _returnvalue_2)) "None" true (struct :`R` 0.878393 :`B` 1.0 :`A` 1.0)))
      (if (< (`KismetMathLibrary.VSize` (- (`.ImpactPoint` (`GameplayStatics.BreakHitResult` _outhit)) (`SceneComponent.GetSocketLocation` (`self.MeshComp`) "spine_02_skin"))) 20.0)
        (goto _label)))))

(event `self.BP_OnLoopRequest`
  (set `self.SwimDuration` (`self.SwimIncrementDuration`)))

(event `HandleEmersion`
  (`PDWPlayerState.RemovePlayerStates` (`self.PlayerState`) (`self.DivingState`))
  (`PDWAnimInstance.SetDivingMode` (`self.As PDWAnim Instance`) false)
  (`PDWAnimInstance.SetDivingMode` (`self.BackpackAnimInstance`) false)
  (bind _ascharacter_movement_component (cast `CharacterMovementComponent` (`Pawn.GetMovementComponent` (`Controller.K2_GetPawn` (`self.PlayerController`)))))
  (`CharacterMovementComponent.SetMovementMode` _ascharacter_movement_component "MOVE_Walking" 0)
  (`|PlayMontage` (`self.MeshComp`) "/Game/Art/Characters/CH_05_Zuma/Animation/AM_CH_05_Zuma_Emersion.AM_CH_05_Zuma_Emersion"
    (:`then`
      (set `self.bStopTick` true))
    (:`OnCompleted`
      (`CharacterMovementComponent.SetMovementMode` _ascharacter_movement_component "MOVE_Walking" 0 :!label _label_2)
      (`PrimitiveComponent.SetCollisionResponseToChannel` (`self.As Capsule Collision`) "ECC_GameTraceChannel7" "ECR_Block")
      (`self.K2_EndAbility`))
    (:`OnBlendOut`
      (goto _label_2))
    (:`OnInterrupted`
      (goto _label_2))))