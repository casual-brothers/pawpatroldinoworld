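; GA_Skill_WaterGun is a Gameplay Ability for the Water Gun skill, building on a parent ability's activation and trigger logic.
; On trigger, it attaches the SpawnedActor to the first player's pawn, keeping its world transform.
; While active, it listens for the GAS.DisableSkills tag; when added, it removes the GE_DisableSkill effect and cancels itself.
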(event `self.K2_ActivateAbility`
  (`parent.K2_ActivateAbility`)
  (bind _asynctaskproxy (`AbilityTask_WaitGameplayTagAdded.WaitGameplayTagAdd` (struct :`TagName` "GAS.DisableSkills") null)
    (:`then`
      (set `self.Async Task` _asynctaskproxy))
    (:`Added`
      (`AbilitySystemComponent.RemoveActiveGameplayEffectBySourceEffect` (`self.GetAbilitySystemComponentFromActorInfo`) "/Game/Blueprints/GAS/GameplayEffects/GE_DisableSkill.GE_DisableSkill_C" null -1)
      (`self.K2_CancelAbility`))))

(event `self.TriggerAbilityLogic`
  (`parent.TriggerAbilityLogic`)
  (`Actor.K2_AttachToActor` (`self.SpawnedActor`) (`GameplayStatics.GetPlayerPawn` 0) "None" "KeepWorld" "KeepWorld" "KeepWorld" true))