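; Zuma vehicle Blueprint that swaps its Niagara surface and trail effects to match the ground beneath it.
; BeginPlay binds the physics constraint to the VHSK component.
; Each tick compares the Nebula surface control's ground surface with the stored one; on a mismatch it deactivates both effects and attaches new ones to VHSK, using dust for unlisted surfaces.
; Disconnected Tick logic for easing rotation and position by angular speed and velocity never runs.
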(event `self.ReceiveBeginPlay`
  (`parent.ReceiveBeginPlay`)
  (`PhysicsConstraintComponent.SetConstrainedComponents` (`self.PhysicsConstraint`) (`self.VH_SK`) "None" null "None"))

(event `self.ReceiveTick`
  (params (DeltaSeconds :type "Float (single-precision)"))
  (`parent.ReceiveTick` DeltaSeconds)
  (`self.SpawnVfxOnSurfaceZuma`))

(fn `SpawnSystemZuma`
  (params (SurfaceSystem :type "NiagaraSystem Object Reference") (AttachToComponent :type "SceneComponent Object Reference") (Location :type "Vector Structure") (SurfaceTrail :type "NiagaraSystem Object Reference"))
  (bind _returnvalue (`NiagaraFunctionLibrary.SpawnSystemAttached` SurfaceSystem AttachToComponent "None" Location (struct) "KeepRelativeOffset" true))
  (set `self.VfxReference` _returnvalue)
  (bind _returnvalue_2 (`NiagaraFunctionLibrary.SpawnSystemAttached` SurfaceTrail AttachToComponent "None" (0.0 0.0 10.0) (struct) "KeepRelativeOffset" true))
  (set `self.TrailVfxReference` _returnvalue_2))

(fn `SpawnVfxOnSurfaceZuma`
  (bind _trailvfxreference (`self.TrailVfxReference`))
  (bind _vh_sk (`self.VH_SK`))
  (bind _location (`self.Location`))
  (bind _vfxreference (`self.VfxReference`))
  (bind _returnvalue (`NebulaGameplaySurfaceControlComponent.GetCurrentGroundSurface` (`self.NebulaGameplaySurfaceControl`)))
  (if (`|EnumInequality` (`self.CurrentSurface`) _returnvalue)
    (`/Engine/EditorBlueprintResources/StandardMacros.IsValid` _vfxreference
      (:`Is Valid`
        (`ActorComponent.Deactivate` _vfxreference))
      (:`Is Not Valid`
        _))
    (`/Engine/EditorBlueprintResources/StandardMacros.IsValid` _trailvfxreference
      (:`Is Valid`
        (`ActorComponent.Deactivate` _trailvfxreference))
      (:`Is Not Valid`
        _))
    (switch `EPhysicalSurface` _returnvalue
      (:`SurfaceType_Default`
        (set `self.CurrentSurface` "SurfaceType1" :!label _label)
        (`self.SpawnSystemZuma` "/Game/Art/VFX/NiagaraSystem/Skill/Vehicles/Zuma/NS_ZumaVehicle_Dust.NS_ZumaVehicle_Dust" _vh_sk _location "/Game/Art/VFX/NiagaraSystem/Skill/Vehicles/Zuma/NS_ZumaVehicle_Trail.NS_ZumaVehicle_Trail"))
      (:`SurfaceType1`
        (goto _label))
      (:`SurfaceType2`
        (set `self.CurrentSurface` "SurfaceType2")
        (`self.SpawnSystemZuma` "/Game/Art/VFX/NiagaraSystem/Skill/Vehicles/Zuma/NS_ZumaVehicle_Mud.NS_ZumaVehicle_Mud" _vh_sk _location "/Game/Art/VFX/NiagaraSystem/Skill/Vehicles/Zuma/NS_ZumaVehicle_Trail.NS_ZumaVehicle_Trail"))
      (:`SurfaceType3`
        (set `self.CurrentSurface` "SurfaceType3")
        (`self.SpawnSystemZuma` "/Game/Art/VFX/NiagaraSystem/Skill/Vehicles/Zuma/NS_ZumaVehicle_Dust.NS_ZumaVehicle_Dust" (`self.VH_SK`) (`self.Location`) "/Game/Art/VFX/NiagaraSystem/Skill/Vehicles/Zuma/NS_ZumaVehicle_Trail.NS_ZumaVehicle_Trail"))
      (:`SurfaceType6`
        (set `self.CurrentSurface` "SurfaceType6")
        (`self.SpawnSystemZuma` "/Game/Art/VFX/NiagaraSystem/Skill/Vehicles/Zuma/NS_ZumaVehicle_Grass.NS_ZumaVehicle_Grass" (`self.VH_SK`) (`self.Location`) "/Game/Art/VFX/NiagaraSystem/Skill/Vehicles/Zuma/NS_ZumaVehicle_Grass.NS_ZumaVehicle_Grass"))
      (:`SurfaceType7`
        (set `self.CurrentSurface` "SurfaceType7")
        (`self.SpawnSystemZuma` "/Game/Art/VFX/NiagaraSystem/Skill/Vehicles/Zuma/NS_ZumaVehicle_Water.NS_ZumaVehicle_Water" (`self.VH_SK`) (`self.Location`) "/Game/Art/VFX/NiagaraSystem/Skill/Vehicles/Zuma/NS_ZumaVehicle_WaterTrail.NS_ZumaVehicle_WaterTrail")))))

(fn `UserConstructionScript`
  (`parent.UserConstructionScript`))