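; Rubble vehicle pawn, a child Blueprint that adds a physics constraint and animated track material on top of its parent vehicle logic.
; On BeginPlay it binds the constraint to the VHSK mesh and swaps the wheel material for a dynamic instance.
; Tick, marked WIP, feeds speed into that material's TrackSpeed parameter, zeroing it within a low-speed range.
; Unconnected logic would ease a Scene component's yaw and offset from angular and linear speed.
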(event `self.ReceiveBeginPlay`
  (`parent.ReceiveBeginPlay`)
  (`PhysicsConstraintComponent.SetConstrainedComponents` (`self.PhysicsConstraint`) (`self.VH_SK`) "None" null "None")
  (bind _returnvalue (`KismetMaterialLibrary.CreateDynamicMaterialInstance` (`PrimitiveComponent.GetMaterialByName` (`self.VH_SK`) "SN_Wheels")))
  (bind _output_get (set `self.WheelsMID` _returnvalue))
  (`PrimitiveComponent.SetMaterial` (`self.VH_SK`) 2 _output_get))

(event `self.ReceiveTick`
  (params (DeltaSeconds :type "Float (single-precision)"))
  (bind _returnvalue (`self.GetSpeedKPH`))
  (bind _wheelsmid (`self.WheelsMID`))
  ;[0.8229 0 0 0.5] WIP
  (`parent.ReceiveTick` DeltaSeconds)
  (if (`KismetMathLibrary.InRange_FloatFloat` _returnvalue -1.0)
    (`MaterialInstanceDynamic.SetScalarParameterValue` _wheelsmid "TrackSpeed" 0.0)
    (else
      (`MaterialInstanceDynamic.SetScalarParameterValue` _wheelsmid "TrackSpeed" _returnvalue))))

(fn `UserConstructionScript`
  (`parent.UserConstructionScript`))