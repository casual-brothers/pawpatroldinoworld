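; Base vehicle pawn that handles surface-driven wheel effects and collision feedback.
; For four-wheel vehicles, Tick reads the ground surface, swaps attached Niagara effects when it changes (rear-only for tracked vehicles), and zeroes trail alpha on hard surfaces or in air.
; Hits spawn impact VFX and controller vibration, throttled by a resetting DoOnce.
; Movement input is empty, its steering and slope-speed logic is disconnected, and possession events add then immediately remove the mapping context.
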(event `EnhancedInput|/Game/Input/Actions/Character/IA_Move`
  (params (ActionValue :type "Vector2D Structure") (ElapsedSeconds :type "Float (double-precision)") (TriggeredSeconds :type "Float (double-precision)") (InputAction :type "InputAction Object Reference" :default "/Game/Input/Actions/Character/IA_Move.IA_Move")))

(event `self.ReceiveTick`
  (params (DeltaSeconds :type "Float (single-precision)"))
  (`parent.ReceiveTick` DeltaSeconds)
  (`self.SpawnVfxOnSurface`))

(event `self.ReceivePossessed`
  (params (NewController :type "Controller Object Reference"))
  (bind _asplayer_controller (cast `PlayerController` NewController))
  (bind _returnvalue (pcsubsystem `EnhancedInputLocalPlayerSubsystem` _asplayer_controller))
  (`EnhancedInputSubsystemInterface.AddMappingContext` _returnvalue "/Game/Input/IMC_Default.IMC_Default" 0 (struct))
  (`EnhancedInputSubsystemInterface.RemoveMappingContext` _returnvalue "/Game/Input/IMC_Default.IMC_Default" (struct)))

(event `self.ReceiveUnpossessed`
  (params (OldController :type "Controller Object Reference"))
  (bind _asplayer_controller (cast `PlayerController` OldController))
  (bind _returnvalue (pcsubsystem `EnhancedInputLocalPlayerSubsystem` _asplayer_controller))
  (`EnhancedInputSubsystemInterface.AddMappingContext` _returnvalue "/Game/Input/IMC_Default.IMC_Default" 0 (struct))
  (`EnhancedInputSubsystemInterface.RemoveMappingContext` _returnvalue "/Game/Input/IMC_Default.IMC_Default" (struct)))

(event `self.PrimitiveComponent.OnComponentHit`
  (params (HitComponent :type "PrimitiveComponent Object Reference") (OtherActor :type "Actor Object Reference") (OtherComp :type "PrimitiveComponent Object Reference") (NormalImpulse :type "Vector Structure") (Hit :type "HitResult Structure (by ref)"))
  (`/Engine/EditorBlueprintResources/StandardMacros.IsValid` OtherActor
    (:`Is Valid`
      (`/Engine/EditorBlueprintResources/StandardMacros.DoOnce` false :!label _label
        (:`Completed`
          (`NiagaraFunctionLibrary.SpawnSystemAtLocation` "/Game/Art/VFX/NiagaraSystem/Generic/NS_Vehicle_Hit.NS_Vehicle_Hit" (`.ImpactPoint` (`GameplayStatics.BreakHitResult` Hit)))
          (`PDWGameplayFunctionLibrary.PlayForceFeedback` (`|MakeArray` (`self.GetPDWPlayerController`)) (struct :`TagName` "ID.Vibration.VehicleImpact"))
          (`KismetSystemLibrary.Delay` 0.5)
          (goto _label :!via `Reset`))))))

(fn `CleanSurfaceVFX`
  (bind _surfacevfxbl (`self.SurfaceVfxBL`))
  (`/Engine/EditorBlueprintResources/StandardMacros.IsValid` _surfacevfxbl
    (:`Is Valid`
      (`/Engine/EditorBlueprintResources/StandardMacros.IsValid` (`self.SurfaceVfxFL`)
        (:`Is Valid`
          (`/Engine/EditorBlueprintResources/StandardMacros.IsValid` (`self.SurfaceVfxFR`)
            (:`Is Valid`
              (`/Engine/EditorBlueprintResources/StandardMacros.IsValid` (`self.SurfaceVfxBR`)
                (:`Is Valid`
                  (`ActorComponent.Deactivate` _surfacevfxbl)
                  (`ActorComponent.Deactivate` (`self.SurfaceVfxFL`))
                  (`ActorComponent.Deactivate` (`self.SurfaceVfxFR`))
                  (`ActorComponent.Deactivate` (`self.SurfaceVfxBR`)))))))))))

(fn `SetNiagaraVariable`
  (params (Alpha :type "Float (double-precision)" :default 1.0) (Kill :type Boolean) (Activate :type Boolean :default true))
  (`NiagaraComponent.SetVariableLinearColor` (`self.NS_Vehicle_Trail_BL`) "Alpha" (make `LinearColor` 0.0 0.0 0.0 Alpha))
  (`NiagaraComponent.SetVariableLinearColor` (`self.NS_Vehicle_Trail_BR`) "Alpha" (make `LinearColor` 0.0 0.0 0.0 Alpha))
  (`NiagaraComponent.SetVariableLinearColor` (`self.NS_Vehicle_Trail_FL`) "Alpha" (make `LinearColor` 0.0 0.0 0.0 Alpha))
  (`NiagaraComponent.SetVariableLinearColor` (`self.NS_Vehicle_Trail_FR`) "Alpha" (make `LinearColor` 0.0 0.0 0.0 Alpha))
  (`NiagaraComponent.SetVariableBool` (`self.NS_Vehicle_Trail_BR`) "Kill" Kill)
  (`NiagaraComponent.SetVariableBool` (`self.NS_Vehicle_Trail_BL`) "Kill" Kill)
  (`NiagaraComponent.SetVariableBool` (`self.NS_Vehicle_Trail_FL`) "Kill" Kill)
  (`NiagaraComponent.SetVariableBool` (`self.NS_Vehicle_Trail_FR`) "Kill" Kill))

(fn `SpawnSystem`
  (params (Niagara :type "NiagaraSystem Object Reference") (MeshComponent :type "SceneComponent Object Reference"))
  (if (`self.IsTrackVehicle`)
    (bind _returnvalue (`NiagaraFunctionLibrary.SpawnSystemAttached` Niagara (`self.NS_Vehicle_Trail_BL`) "None" (0.0 0.0 0.0) (struct) "KeepRelativeOffset" true))
    (set `self.SurfaceVfxBL` _returnvalue)
    (bind _returnvalue_2 (`NiagaraFunctionLibrary.SpawnSystemAttached` Niagara (`self.NS_Vehicle_Trail_BR`) "None" (0.0 0.0 0.0) (struct) "KeepRelativeOffset" true))
    (set `self.SurfaceVfxBR` _returnvalue_2)
    (else
      (bind _returnvalue_3 (`NiagaraFunctionLibrary.SpawnSystemAttached` Niagara (`self.NS_Vehicle_Trail_BL`) "None" (0.0 0.0 0.0) (struct) "KeepRelativeOffset" true))
      (set `self.SurfaceVfxBL` _returnvalue_3)
      (bind _returnvalue_4 (`NiagaraFunctionLibrary.SpawnSystemAttached` Niagara (`self.NS_Vehicle_Trail_FL`) "None" (0.0 0.0 0.0) (struct) "KeepRelativeOffset" true))
      (set `self.SurfaceVfxFL` _returnvalue_4)
      (bind _returnvalue_5 (`NiagaraFunctionLibrary.SpawnSystemAttached` Niagara (`self.NS_Vehicle_Trail_FR`) "None" (0.0 0.0 0.0) (struct) "KeepRelativeOffset" true))
      (set `self.SurfaceVfxFR` _returnvalue_5)
      (bind _returnvalue_6 (`NiagaraFunctionLibrary.SpawnSystemAttached` Niagara (`self.NS_Vehicle_Trail_BR`) "None" (0.0 0.0 0.0) (struct) "KeepRelativeOffset" true))
      (set `self.SurfaceVfxBR` _returnvalue_6))))

(fn `SpawnVfxOnSurface`
  (if (`self.Is4WheelsVehicle`)
    (if (`self.IsOnAir`)
      (`NiagaraComponent.SetVariableLinearColor` (`self.NS_Vehicle_Trail_BL`) "Alpha" (make `LinearColor` 0.0))
      (`NiagaraComponent.SetVariableLinearColor` (`self.NS_Vehicle_Trail_BR`) "Alpha" (make `LinearColor` 0.0))
      (`NiagaraComponent.SetVariableLinearColor` (`self.NS_Vehicle_Trail_FL`) "Alpha" (make `LinearColor` 0.0))
      (`NiagaraComponent.SetVariableLinearColor` (`self.NS_Vehicle_Trail_FR`) "Alpha" (make `LinearColor` 0.0)))
    (bind _returnvalue (`NebulaGameplaySurfaceControlComponent.GetCurrentGroundSurface` (`self.NebulaGameplaySurfaceControl`)))
    (if (`|EnumInequality` (`self.CurrentSurface`) _returnvalue)
      (`self.CleanSurfaceVFX`)
      (switch `EPhysicalSurface` _returnvalue
        (:`SurfaceType_Default`
          (set `self.CurrentSurface` "SurfaceType1" :!label _label)
          (`self.SetNiagaraVariable` 1.0)
          (`self.SpawnSystem` "/Game/Art/VFX/NiagaraSystem/Generic/NS_Vehicle_Dirt.NS_Vehicle_Dirt"))
        (:`SurfaceType1`
          (goto _label))
        (:`SurfaceType2`
          (set `self.CurrentSurface` "SurfaceType2")
          (`self.SetNiagaraVariable` 1.0)
          (`self.SpawnSystem` "/Game/Art/VFX/NiagaraSystem/Generic/NS_Vehicle_Mud.NS_Vehicle_Mud"))
        (:`SurfaceType3`
          (set `self.CurrentSurface` "SurfaceType3")
          (`self.SetNiagaraVariable` 1.0)
          (`self.SpawnSystem` "/Game/Art/VFX/NiagaraSystem/Generic/NS_Vehicle_Dust.NS_Vehicle_Dust"))
        (:`SurfaceType4`
          (set `self.CurrentSurface` "SurfaceType4")
          (`self.SetNiagaraVariable` 0.0 false false :!label _label_2))
        (:`SurfaceType5`
          (set `self.CurrentSurface` "SurfaceType5")
          (goto _label_2))
        (:`SurfaceType6`
          (set `self.CurrentSurface` "SurfaceType6")
          (`self.SetNiagaraVariable` 1.0)
          (`self.SpawnSystem` "/Game/Art/VFX/NiagaraSystem/Generic/NS_Vehicle_Grass.NS_Vehicle_Grass"))
        (:`SurfaceType7`
          (set `self.CurrentSurface` "SurfaceType7")
          (`self.SetNiagaraVariable` 0.0 false false)
          (`self.SpawnSystem` "/Game/Art/VFX/NiagaraSystem/Generic/NS_Vehicle_Water.NS_Vehicle_Water"))
        (:`SurfaceType8`
          (set `self.CurrentSurface` "SurfaceType8")
          (goto _label_2))
        (:`SurfaceType9`
          (set `self.CurrentSurface` "SurfaceType9")
          (goto _label_2))
        (:`SurfaceType10`
          (set `self.CurrentSurface` "SurfaceType10")
          (goto _label_2))
        (:`SurfaceType11`
          (set `self.CurrentSurface` "SurfaceType11")
          (goto _label_2))
        (:`SurfaceType12`
          (set `self.CurrentSurface` "SurfaceType12")
          (goto _label_2))))))

(fn `UserConstructionScript`
  (if (not (`self.Is4WheelsVehicle`))
    (`ActorComponent.K2_DestroyComponent` (`self.NS_Vehicle_Trail_FL`))
    (`ActorComponent.K2_DestroyComponent` (`self.NS_Vehicle_Trail_BL`))
    (`ActorComponent.K2_DestroyComponent` (`self.NS_Vehicle_Trail_BR`))
    (`ActorComponent.K2_DestroyComponent` (`self.NS_Vehicle_Trail_FR`))))