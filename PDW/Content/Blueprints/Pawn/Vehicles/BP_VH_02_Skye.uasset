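; Skye's vehicle pawn, which banks with steering and shows surface-specific ground effects.
; Tick eases the VHSK roll toward steering input, while minigame turn events snap it to the turn direction.
; On a ground surface change, it deactivates old Niagara effects and attaches dirt, mud, dust or water below the mesh.
; Unhandled surfaces fall back to dirt and store that type, so the effect respawns every tick there.
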(event `self.ReceiveTick`
  (params (DeltaSeconds :type "Float (single-precision)"))
  (bind _vh_sk (`self.VH_SK`))
  (bind (_relativerotation_roll _relativerotation_pitch _relativerotation_yaw) (`KismetMathLibrary.BreakRotator` (`SceneComponent.RelativeRotation` _vh_sk)))
  (`parent.ReceiveTick` DeltaSeconds)
  (`SceneComponent.K2_SetRelativeRotation` _vh_sk (`|EaseFunction` "Linear" (* DeltaSeconds 3.0) (`KismetMathLibrary.MakeRotator` _relativerotation_roll _relativerotation_pitch _relativerotation_yaw) (`KismetMathLibrary.MakeRotator` (`KismetMathLibrary.MapRangeClamped` (`self.GetSteeringInput`) -1.0 1.0 -30.0 30.0) _relativerotation_pitch _relativerotation_yaw)) false false)
  (`self.Skye_SpawnVfxOnSurface`))

(event `self.BP_OnTurnDuringMinigame`
  (params (Direction :type Integer))
  (bind _vh_sk (`self.VH_SK`))
  (bind (_relativerotation_roll _relativerotation_pitch _relativerotation_yaw) (`KismetMathLibrary.BreakRotator` (`SceneComponent.RelativeRotation` _vh_sk)))
  (`SceneComponent.K2_SetRelativeRotation` _vh_sk (`|EaseFunction` "Linear" 1.0 (`KismetMathLibrary.MakeRotator` _relativerotation_roll _relativerotation_pitch _relativerotation_yaw) (`KismetMathLibrary.MakeRotator` (`KismetMathLibrary.MapRangeClamped` (`KismetMathLibrary.Conv_IntToDouble` Direction) -1.0 1.0 -30.0 30.0) _relativerotation_pitch _relativerotation_yaw)) false false))

(fn `Skye_CleanSurfaceVfx`
  (bind _dirtsurfacevfxref (`self.DirtSurfaceVfxRef`))
  (bind _sandsurfacevfxref (`self.SandSurfaceVfxRef`))
  (bind _mudsurfacevfxref (`self.MudSurfaceVfxRef`))
  (bind _watersurfacevfxref (`self.WaterSurfaceVfxRef`))
  (`|ExecutionSequence`
    (:`then_0`
      (`/Engine/EditorBlueprintResources/StandardMacros.IsValid` _dirtsurfacevfxref
        (:`Is Valid`
          (`ActorComponent.Deactivate` _dirtsurfacevfxref))))
    (:`then_1`
      (`/Engine/EditorBlueprintResources/StandardMacros.IsValid` _sandsurfacevfxref
        (:`Is Valid`
          (`ActorComponent.Deactivate` _sandsurfacevfxref))))
    (:`then_2`
      (`/Engine/EditorBlueprintResources/StandardMacros.IsValid` _mudsurfacevfxref
        (:`Is Valid`
          (`ActorComponent.Deactivate` _mudsurfacevfxref))))
    (:`then_3`
      (`/Engine/EditorBlueprintResources/StandardMacros.IsValid` _watersurfacevfxref
        (:`Is Valid`
          (`ActorComponent.Deactivate` _watersurfacevfxref))))))

(fn `Skye_SpawnVfxOnSurface`
  (bind _staticmeshref (`self.StaticMeshRef`))
  (bind _staticmeshref_2 (`self.StaticMeshRef`))
  (bind _returnvalue (`NebulaGameplaySurfaceControlComponent.GetCurrentGroundSurface` (`self.NebulaGameplaySurfaceControl`)))
  (if (`|EnumInequality` (`self.SkyCurrentSurface`) _returnvalue)
    (`self.Skye_CleanSurfaceVfx`)
    (switch `EPhysicalSurface` _returnvalue
      (:`SurfaceType_Default`
        (set `self.SkyCurrentSurface` "SurfaceType1" :!label _label)
        (bind _returnvalue_2 (`NiagaraFunctionLibrary.SpawnSystemAttached` "/Game/Art/VFX/NiagaraSystem/Generic/NS_VehicleSkye_Dirt.NS_VehicleSkye_Dirt" _staticmeshref_2 "None" (0.0 0.0 -200.0) (struct) "KeepRelativeOffset"))
        (set `self.DirtSurfaceVfxRef` _returnvalue_2))
      (:`SurfaceType1`
        (goto _label))
      (:`SurfaceType2`
        (set `self.SkyCurrentSurface` "SurfaceType2")
        (bind _returnvalue_3 (`NiagaraFunctionLibrary.SpawnSystemAttached` "/Game/Art/VFX/NiagaraSystem/Generic/NS_VehicleSkye_Mud.NS_VehicleSkye_Mud" _staticmeshref "None" (0.0 0.0 -180.0) (struct) "KeepRelativeOffset"))
        (set `self.MudSurfaceVfxRef` _returnvalue_3))
      (:`SurfaceType3`
        (set `self.SkyCurrentSurface` "SurfaceType3")
        (bind _returnvalue_4 (`NiagaraFunctionLibrary.SpawnSystemAttached` "/Game/Art/VFX/NiagaraSystem/Generic/NS_VehicleSkye_Dust.NS_VehicleSkye_Dust" _staticmeshref_2 "None" (0.0 0.0 -200.0) (struct) "KeepRelativeOffset"))
        (set `self.SandSurfaceVfxRef` _returnvalue_4))
      (:`SurfaceType7`
        (set `self.SkyCurrentSurface` "SurfaceType7")
        (bind _returnvalue_5 (`NiagaraFunctionLibrary.SpawnSystemAttached` "/Game/Art/VFX/NiagaraSystem/Generic/NS_VehicleSkye_Water.NS_VehicleSkye_Water" _staticmeshref "None" (0.0 0.0 -50.0) (struct) "KeepRelativeOffset"))
        (set `self.WaterSurfaceVfxRef` _returnvalue_5)))))

(fn `UserConstructionScript`
  (`parent.UserConstructionScript`))