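; Player controller that restores its last configuration on possession and turns Enhanced Input actions into gameplay calls, each gated by IsInputActionDisabled.
; Movement routes to camera-relative minigame movement, vehicle input or on-foot movement, alongside jump, look, interact, skill and a cooldown-limited vehicle swap.
; Character change, pause and debug keys for cutscene skip and Ryder menu fire named TriggerAction events, mostly FSM ones.
; An unconnected steering/throttle conversion remains unused.
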(event Input|EnhancedActionEvents|EnhancedInputActionIA_GameplayPause
  (params (ActionValue :type Boolean) (ElapsedSeconds :type Float%20%28double-precision%29) (TriggeredSeconds :type Float%20%28double-precision%29) (InputAction :type Input%20Action%20Object%20Reference :default "/Game/Input/Actions/Character/IA_GameplayPause.IA_GameplayPause"))
  (bind _returnvalue (Class|PDWGameplayFunctionLibrary|IsInputActionDisabled InputAction))
  (if (not _returnvalue)
    (Class|NebulaFlowCoreFunctionLibrary|TriggerAction "FSM.PauseGame" "" self)))

(event Input|EnhancedActionEvents|EnhancedInputActionIA_Skill
  (params (ActionValue :type Boolean) (ElapsedSeconds :type Float%20%28double-precision%29) (TriggeredSeconds :type Float%20%28double-precision%29) (InputAction :type Input%20Action%20Object%20Reference :default "/Game/Input/Actions/Character/IA_Skill.IA_Skill"))
  (bind _returnvalue (Class|PDWGameplayFunctionLibrary|IsInputActionDisabled InputAction))
  (if (not _returnvalue)
    (Class|PDWPlayerController|ActivateSkill ActionValue 0)))

(event Input|EnhancedActionEvents|EnhancedInputActionIA_Jump
  (params (ActionValue :type Boolean) (ElapsedSeconds :type Float%20%28double-precision%29) (TriggeredSeconds :type Float%20%28double-precision%29) (InputAction :type Input%20Action%20Object%20Reference :default "/Game/Input/Actions/Character/IA_Jump.IA_Jump"))
  (:Triggered
    (bind _output_get (Variables|Default|SetJumpPressed ActionValue :!label _label))
    (if _output_get
      (bind _returnvalue (Class|PDWGameplayFunctionLibrary|IsInputActionDisabled InputAction))
      (if (not _returnvalue)
        (Class|PDWPlayerController|CharacterJump))))
  (:Completed
    (goto _label)))

(event Input|EnhancedActionEvents|EnhancedInputActionIA_Interact
  (params (ActionValue :type Boolean) (ElapsedSeconds :type Float%20%28double-precision%29) (TriggeredSeconds :type Float%20%28double-precision%29) (InputAction :type Input%20Action%20Object%20Reference :default "/Game/Input/Actions/Character/IA_Interact.IA_Interact"))
  (bind _returnvalue (Class|PDWGameplayFunctionLibrary|IsInputActionDisabled InputAction))
  (if (not _returnvalue)
    (Class|PDWPlayerController|Interact)))

(event Input|EnhancedActionEvents|EnhancedInputActionIA_ChangeCharacter
  (params (ActionValue :type Boolean) (ElapsedSeconds :type Float%20%28double-precision%29) (TriggeredSeconds :type Float%20%28double-precision%29) (InputAction :type Input%20Action%20Object%20Reference :default "/Game/Input/Actions/Character/IA_ChangeCharacter.IA_ChangeCharacter"))
  (bind _returnvalue (Class|PDWGameplayFunctionLibrary|IsInputActionDisabled InputAction))
  (if (not _returnvalue)
    (Class|NebulaFlowCoreFunctionLibrary|TriggerAction "ChangePup" "" self)))

(event Input|EnhancedActionEvents|EnhancedInputActionIA_SwapVehicle
  (params (ActionValue :type Boolean) (ElapsedSeconds :type Float%20%28double-precision%29) (TriggeredSeconds :type Float%20%28double-precision%29) (InputAction :type Input%20Action%20Object%20Reference :default "/Game/Input/Actions/Character/IA_SwapVehicle.IA_SwapVehicle"))
  (:Completed
    (bind _returnvalue (Class|PDWGameplayFunctionLibrary|IsInputActionDisabled InputAction))
    (if (not _returnvalue)
      (Utilities|FlowControl|DoOnce false :!label _label
        (:Completed
          (Class|PDWPlayerController|ChangeVehicle false true)
          (Utilities|FlowControl|Delay (Variables|Default|GetSwapVehicleCooldown))
          (goto _label Reset))))))

(event Input|EnhancedActionEvents|EnhancedInputActionIA_Look
  (params (ActionValue :type Vector%202D%20Structure) (ElapsedSeconds :type Float%20%28double-precision%29) (TriggeredSeconds :type Float%20%28double-precision%29) (InputAction :type Input%20Action%20Object%20Reference :default "/Game/Input/Actions/Character/IA_Look.IA_Look"))
  (bind _returnvalue (Class|PDWGameplayFunctionLibrary|IsInputActionDisabled InputAction))
  (if (not _returnvalue)
    (Class|PDWPlayerController|Look ActionValue)))

(event Input|EnhancedActionEvents|EnhancedInputActionIA_Pause
  (params (ActionValue :type Boolean) (ElapsedSeconds :type Float%20%28double-precision%29) (TriggeredSeconds :type Float%20%28double-precision%29) (InputAction :type Input%20Action%20Object%20Reference :default "/Game/Input/Actions/Character/IA_Pause.IA_Pause"))
  (bind _returnvalue (Class|PDWGameplayFunctionLibrary|IsInputActionDisabled InputAction))
  (if (not _returnvalue)
    (Class|NebulaFlowCoreFunctionLibrary|TriggerAction "FSM.PauseGame" "" self)))

(event Input|EnhancedActionEvents|EnhancedInputActionIA_Move
  (params (ActionValue :type Vector%202D%20Structure) (ElapsedSeconds :type Float%20%28double-precision%29) (TriggeredSeconds :type Float%20%28double-precision%29) (InputAction :type Input%20Action%20Object%20Reference :default "/Game/Input/Actions/Character/IA_Move.IA_Move"))
  (:Triggered
    (bind _returnvalue (Class|PDWGameplayFunctionLibrary|IsInputActionDisabled InputAction :!label _label))
    (if (not _returnvalue)
      (if (Variables|Default|GetMovementCameraBase)
        (Class|PDWPlayerController|MiniGameMove ActionValue (Variables|Default|GetCameraForwardVector) (Variables|Default|GetCameraRightVector))
        (elif (Class|PDWPlayerController|GetIsonVehicle)
          (bind _returnvalue_2 (Class|PDWPlayerController|GetVehicleInstance))
          ;[0.15 0.15 0.15 0.5] capire perchè se agganciato qua non va più avanti
          (Class|PDWVehiclePawn|AnalyzeInput _returnvalue_2 ActionValue)
          (else
            (Class|PDWPlayerController|Move ActionValue))))))
  (:Completed
    (goto _label)))

(event EventPossess
  (params (PossessedPawn :type Pawn%20Object%20Reference))
  (Class|PDWInputSubsystem|RestoreLastConfiguration self))

(event Input|KeyboardEvents|DebugKeyK
  (params (Key :type Key%20Structure :default "None") (ActionValue :type Input%20Action%20Value%20Structure))
  (:Pressed
    (Class|NebulaFlowCoreFunctionLibrary|TriggerAction "FSM.SkipCutscene" "" 0)))

(event Input|KeyboardEvents|DebugKeyMultiply
  (params (Key :type Key%20Structure :default "None") (ActionValue :type Input%20Action%20Value%20Structure))
  (:Pressed
    (Class|NebulaFlowCoreFunctionLibrary|TriggerAction "FSM.RyderMenu" "" 0)))

(fn ConstructionScript)