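; Pup character Blueprint for Marshall, whose lifecycle events and construction script add nothing beyond calls to the parent class.
; CleanFunction line-traces forward from the actor, draws a debug sphere at the hit location and calls Paint on a hit BP_TEST_CLEAN, apparently a cleaning prototype.
; Nothing in this file calls CleanFunction, and the nodes adding Water skill and Marshall interaction tags are unconnected.
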(event `self.ReceiveBeginPlay`
  (`parent.ReceiveBeginPlay`))

(event `self.ReceiveTick`
  (params (DeltaSeconds :type "Float (single-precision)"))
  (`parent.ReceiveTick` DeltaSeconds))

(fn `CleanFunction`
  (bind _returnvalue (`self.K2_GetActorLocation`))
  (bind _outhit (`KismetSystemLibrary.LineTraceSingle` _returnvalue (+ _returnvalue (* (`self.GetActorForwardVector`) (`self.Trace Distance`))) "TraceTypeQuery1"))
  (bind (_bblockinghit _binitialoverlap _time _distance _location _impactpoint _normal _impactnormal _physmat _hitactor) (`GameplayStatics.BreakHitResult` _outhit))
  (bind _output_get (set `self.Position` _location))
  (`KismetSystemLibrary.DrawDebugSphere` _output_get 10.0 12 (struct :`R` 1.0 :`G` 0.759845 :`A` 1.0) 0.333 0.01)
  (bind _asbp_test_clean (cast `/Game/Prototype/Art/Temp/Ricardo/BP_TEST_CLEAN` _hitactor))
  (`/Game/Prototype/Art/Temp/Ricardo/BP_TEST_CLEAN.Paint` _asbp_test_clean _output_get (`self.HitRadius`)))

(fn `UserConstructionScript`
  (`parent.UserConstructionScript`))