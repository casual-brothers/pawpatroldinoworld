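; Base Blueprint for a Pup character pawn, handling player icons and hand and foot print decals.
; It tags the player icon component as P1 on possession or P2 on multiplayer state changes, based on the controller.
; Four footprint events spawn fading decals at hand and foot sockets, aligned to socket yaw.
; BeginPlay sets a temporary custom depth stencil on character meshes, and Tick can print walk speed for debugging.
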(event `self.ReceivePossessed`
  (params (NewController :type "Controller Object Reference"))
  (if (not (== NewController (`PDWGameplayFunctionLibrary.GetPlayerControllerTwo`)))
    (`PDWIconComponent.OnTagAdded` (`self.BP_PlayerIconComponent`) (`self.Tag Container P1`) (`self.Added Tag P1`))))

(event `self.ReceiveBeginPlay`
  ;[1 0 0 0.5] TEMP
  (`PrimitiveComponent.SetCustomDepthStencilValue` (`self.Mesh`) 10)
  (`PrimitiveComponent.SetCustomDepthStencilValue` (`self.SK_CH_01_Skill`) 10)
  (`PrimitiveComponent.SetCustomDepthStencilValue` (`self.SM_CH_01_Hat`) 10)
  (add `PDWEventSubsytem.OnMultiplayerStateChange` (subsystem `PDWEventSubsytem`) (delegate `CustomEvent`)))

(event `CustomEvent`
  (if (== (`self.GetController`) (`PDWGameplayFunctionLibrary.GetPlayerControllerTwo`))
    (`PDWIconComponent.OnTagAdded` (`self.BP_PlayerIconComponent`) (`self.Tag Container P2`) (`self.Added Tag P2`))))

(event `self.ReceiveTick`
  (params (DeltaSeconds :type "Float (single-precision)"))
  (`parent.ReceiveTick` DeltaSeconds)
  (if (`self.bPrintSpeed`)
    (`KismetSystemLibrary.PrintString` (`KismetStringLibrary.Concat_StrStr` "Pup Speed:" (`KismetStringLibrary.Conv_DoubleToString` (`CharacterMovementComponent.MaxWalkSpeed` (`self.CharacterMovement`)))) true true (struct :`G` 1.0 :`B` 0.101638 :`A` 1.0) 0.0 "1457")))

(event `L_Hand_FootPrint`
  (params (DecalSize_Hand_l :type "Vector Structure" :default (40.0 15.0 15.0)))
  (bind _mesh (`self.Mesh`))
  (bind (_returnvalue_roll _returnvalue_pitch _returnvalue_yaw) (`KismetMathLibrary.BreakRotator` (`SceneComponent.GetSocketRotation` _mesh "l_hand_socket")))
  (bind _returnvalue (`GameplayStatics.SpawnDecalAtLocation` "/Game/Art/VFX/MaterialInstances/MI_FootPrint.MI_FootPrint" DecalSize_Hand_l (`SceneComponent.GetSocketLocation` _mesh "l_hand_socket") (`KismetMathLibrary.MakeRotator` 90.0 -90.0 _returnvalue_yaw) 12.0))
  (`DecalComponent.SetFadeOut` _returnvalue 8.0 4.0 true))

(event `R_Hand_FootPrint`
  (params (DecalSize_Hand_r :type "Vector Structure" :default (40.0 15.0 15.0)))
  (bind _mesh (`self.Mesh`))
  (bind (_returnvalue_roll _returnvalue_pitch _returnvalue_yaw) (`KismetMathLibrary.BreakRotator` (`SceneComponent.GetSocketRotation` _mesh "r_hand_socket")))
  (bind _returnvalue (`GameplayStatics.SpawnDecalAtLocation` "/Game/Art/VFX/MaterialInstances/MI_FootPrint.MI_FootPrint" DecalSize_Hand_r (`SceneComponent.GetSocketLocation` _mesh "r_hand_socket") (`KismetMathLibrary.MakeRotator` 90.0 -90.0 _returnvalue_yaw) 12.0))
  (`DecalComponent.SetFadeOut` _returnvalue 8.0 4.0 true))

(event `L_Foot_FootPrint`
  (params (DecalSize_Hand_l :type "Vector Structure" :default (40.0 10.0 15.0)))
  (bind _mesh (`self.Mesh`))
  (bind (_returnvalue_roll _returnvalue_pitch _returnvalue_yaw) (`KismetMathLibrary.BreakRotator` (`SceneComponent.GetSocketRotation` _mesh "l_foot_socket")))
  (bind _returnvalue (`GameplayStatics.SpawnDecalAtLocation` "/Game/Art/VFX/MaterialInstances/MI_FootPrint_Shoe.MI_FootPrint_Shoe" DecalSize_Hand_l (`SceneComponent.GetSocketLocation` _mesh "l_foot_socket") (`KismetMathLibrary.MakeRotator` 90.0 -90.0 _returnvalue_yaw) 12.0))
  (`DecalComponent.SetFadeOut` _returnvalue 8.0 4.0 true))

(event `R_Foot_FootPrint`
  (params (DecalSize_Foot_r :type "Vector Structure" :default (40.0 10.0 15.0)))
  (bind _mesh (`self.Mesh`))
  (bind (_returnvalue_roll _returnvalue_pitch _returnvalue_yaw) (`KismetMathLibrary.BreakRotator` (`SceneComponent.GetSocketRotation` _mesh "r_foot_socket")))
  (bind _returnvalue (`GameplayStatics.SpawnDecalAtLocation` "/Game/Art/VFX/MaterialInstances/MI_FootPrint_Shoe_r.MI_FootPrint_Shoe_r" DecalSize_Foot_r (`SceneComponent.GetSocketLocation` _mesh "r_foot_socket") (`KismetMathLibrary.MakeRotator` 90.0 -90.0 _returnvalue_yaw) 12.0))
  (`DecalComponent.SetFadeOut` _returnvalue 8.0 4.0 true))

(fn `UserConstructionScript`)