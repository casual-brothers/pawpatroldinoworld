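; Base Blueprint for Paleo Center dinosaur NPCs, handling their pen needs, interactions and minigame reactions through PDWPaleoDino events.
; Need searches claim a random matching Smart Object in the pen and run it as a gameplay interaction, retrying after failure once pen activity allows.
; Needs set icon tags and swap base or dirt dynamic materials.
; Minigame endings play happy montages, first finishing the hurt montage and restoring collision.
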(event `self.ReceiveBeginPlay`
  (bind _mesh (`self.Mesh`))
  (add `PDWInteractionReceiverComponent.OnInteractionSuccessful` (`self.BP_InteractionReceiverComponent`) (delegate `OnInteractionSuccessful_Event`))
  (bind _returnvalue (`KismetMaterialLibrary.CreateDynamicMaterialInstance` (`PrimitiveComponent.GetMaterial` _mesh 0)))
  (bind _output_get (set `self.BaseMaterial` _returnvalue))
  (bind _returnvalue_2 (`PrimitiveComponent.CreateDynamicMaterialInstance` (`self.Mesh`) 0 (`self.DirtMaterial`) "None"))
  (set `self.MID DinoDirt` _returnvalue_2)
  (`PrimitiveComponent.SetMaterial` _mesh 0 _output_get))

(event `OnInteractionSuccessful_Event`
  (params (Payload :type "PDWInteractionPayload Structure (by ref)"))
  (`PDWPaleoDinoComponent.OnInteractionSuccess` (`self.PDWPaleoDino`)))

(event `self.PDWPaleoDino.OnSearchSO`
  (params (NeedTag :type "GameplayTag Structure"))
  (bind (_returnvalue_penareacenter _returnvalue_maxmoveradius _returnvalue_sosearchbox) (break `PDWPenAreaBounds` (`PDWDinoPenArea.GetPenAreaBounds` (`PDWPaleoDinoComponent.GetPenAreaRef` (`self.PDWPaleoDino`)))))
  ; Temp, move to c++
  (bind (_outresults _returnvalue) (`SmartObjectSubsystem.FindSmartObjects_BP` (subsystem `SmartObjectSubsystem`) (make `SmartObjectRequest` _returnvalue_sosearchbox (make `SmartObjectRequestFilter` (`BlueprintGameplayTagLibrary.MakeGameplayTagContainerFromArray` (`|MakeArray` NeedTag)))) self :!label _label))
  (if _returnvalue
    (bind _returnvalue_2 (`SmartObjectBlueprintFunctionLibrary.MarkSmartObjectSlotAsClaimed` (`.SlotHandle` (break `SmartObjectRequestResult` (`|GetArrayItem` _outresults (`KismetMathLibrary.RandomIntegerInRange` 0 (- (`KismetArrayLibrary.Array_Length` _outresults) 1))))) self "High"))
    (set `self.ClaimedHandle` _returnvalue_2)
    (bind _asynctaskproxy (`AITask_UseGameplayInteraction.MoveToAndUseSmartObjectWithGameplayInteraction` (`AIBlueprintHelperLibrary.GetAIController` self) _returnvalue_2)
      (:`then`
        (set `self.CurrentGameplayInteractionTask` _asynctaskproxy))
      (:`OnSucceeded`
        (`PDWPaleoDinoComponent.OnSearchSOCompleted` (`self.PDWPaleoDino`) true))
      (:`OnFailed`
        (`KismetSystemLibrary.PrintString` "Fail!")
        (`KismetSystemLibrary.Delay` 3.0 :!label _label_2)
        (bind _returnvalue_3 (`PDWPaleoCenterSubsystem.GetDinoPenActivity` (subsystem `PDWPaleoCenterSubsystem`) (`PDWPaleoDinoComponent.GetPenTag` (`self.PDWPaleoDino`))))
        (if _returnvalue_3
          (goto _label)
          (else
            (goto _label_2))))
      (:`OnMoveToFailed`
        (`KismetSystemLibrary.PrintString` "Move To Failed")
        (goto _label_2)))
    (else
      (`PDWPaleoDinoComponent.OnSearchSOCompleted` (`self.PDWPaleoDino`) false))))

(event `self.PDWPaleoDino.OnShowNeed`
  (params (NeedTag :type "GameplayTag Structure"))
  (`self.HandleDinoNeed` NeedTag))

(event `self.PDWPaleoDino.OnShowFakeNeed`
  (params (NeedTag :type "GameplayTag Structure"))
  (`self.HandleDinoNeed` NeedTag))

(event `HandleDinoNeed`
  (params (Tag :type "GameplayTag Structure"))
  (bind _pdwtag (`self.PDWTag`))
  (bind _icontags_gameplaytags (break `GameplayTagContainer` (`PDWIconComponent.IconTags` (`self.BP_PaleocenterIconComponent_P1`))))
  (for _array_element _icontags_gameplaytags
    (`PDWTagComponent.RemoveTag` _pdwtag _array_element))
  (if (not (== Tag (struct :`TagName` "ID.DinoNeed.Happy")))
    (`PDWTagComponent.AddTag` _pdwtag Tag)))

(event `self.PDWPaleoDino.BeforeEndPlay`
  (`SmartObjectBlueprintFunctionLibrary.MarkSmartObjectSlotAsFree` (`self.ClaimedHandle`)))

(event `self.PDWPaleoDino.OnMinigameEnd`
  (params (MinigameTag :type "GameplayTag Structure"))
  (bind _returnvalue (`SkeletalMeshComponent.GetAnimInstance` (`self.Mesh`)))
  (bind _returnvalue_2 (`AnimInstance.GetCurrentActiveMontage` _returnvalue))
  (if (== MinigameTag (struct :`TagName` "ID.DinoNeed.Hurt"))
    (`PrimitiveComponent.SetCollisionEnabled` (`self.Mesh`) "QueryAndPhysics")
    (`/Engine/EditorBlueprintResources/StandardMacros.IsValid` _returnvalue_2
      (:`Is Valid`
        (`AnimInstance.Montage_JumpToSection` _returnvalue "End" _returnvalue_2)
        (add `AnimInstance.OnMontageEnded` _returnvalue (delegate `OnSadMontageEnd`))))
    (elif (== MinigameTag (struct :`TagName` "ID.DinoNeed.Dirty"))
      (bind _aspdwanim_instance (cast `PDWAnimInstance` _returnvalue))
      (`PDWAnimInstance.PlayMontageByTag` _aspdwanim_instance (struct :`TagName` "ID.Animation.Happy")))))

(event `OnSadMontageEnd`
  (params (Montage :type "AnimMontage Object Reference") (bInterrupted :type Boolean))
  (bind _returnvalue (`SkeletalMeshComponent.GetAnimInstance` (`self.Mesh`)))
  (remove `AnimInstance.OnMontageEnded` _returnvalue (delegate `OnSadMontageEnd`))
  (bind _aspdwanim_instance (cast `PDWAnimInstance` _returnvalue))
  (`PDWAnimInstance.PlayMontageByTag` _aspdwanim_instance (struct :`TagName` "ID.Animation.Happy")))

(event `self.PDWPaleoDino.OnActivateInteraction`
  (params (InteractionTag :type "GameplayTag Structure"))
  (`PDWInteractionReceiverComponent.AddStateTag` (`self.BP_InteractionReceiverComponent`) InteractionTag))

(event `self.PDWPaleoDino.OnDeactivateInteraction`
  (params (InteractionTag :type "GameplayTag Structure"))
  (`PDWInteractionReceiverComponent.AddStateTag` (`self.BP_InteractionReceiverComponent`) (`self.EmptyTag`)))

(event `StartHurtAnimation`
  (bind _aspdwanim_instance (cast `PDWAnimInstance` (`SkeletalMeshComponent.GetAnimInstance` (`self.Mesh`))))
  (`PDWAnimInstance.PlayMontageByTag` _aspdwanim_instance (struct :`TagName` "ID.DinoNeed.Hurt"))
  (`PrimitiveComponent.SetCollisionEnabled` (`self.Mesh`) "PhysicsOnly"))

(event `self.PDWPaleoDino.OnShowNeedMat`
  (params (NeedTag :type "GameplayTag Structure"))
  (bind _basematerial (`self.BaseMaterial`))
  (bind _mid_dinodirt (`self.MID DinoDirt`))
  (if (and (== NeedTag (struct :`TagName` "ID.DinoNeed.Happy")) (!= (`PrimitiveComponent.GetMaterial` (`self.Mesh`) 0) (`self.BaseMaterial`)))
    (`/Engine/EditorBlueprintResources/StandardMacros.IsValid` _basematerial
      (:`Is Valid`
        (`PrimitiveComponent.SetMaterial` (`self.Mesh`) 0 _basematerial)))
    (elif (== NeedTag (`PDWGameplayTagSettings.GetDirtyDino`))
      (`/Engine/EditorBlueprintResources/StandardMacros.IsValid` _mid_dinodirt
        (:`Is Valid`
          (`PrimitiveComponent.SetMaterial` (`self.Mesh`) 0 _mid_dinodirt))))))

(fn `UserConstructionScript`)