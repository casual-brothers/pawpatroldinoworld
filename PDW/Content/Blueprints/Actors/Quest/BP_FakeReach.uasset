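; BP_FakeReach is a quest actor whose only logic is a helper for placing it on the ground.
; SnapToGround runs a complex Visibility line trace along the actor's up axis, from slightly above to far below, and moves the actor to the impact point on a blocking hit.
; The event graph and construction script are empty, and nothing in this Blueprint calls SnapToGround.
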(event `self.ReceiveActorBeginOverlap`
  (params (OtherActor :type "Actor Object Reference")))

(fn `SnapToGround`
  (bind _outhit (`KismetSystemLibrary.LineTraceSingle` (+ (`self.K2_GetActorLocation`) (* (`self.GetActorUpVector`) 200.0)) (+ (`self.K2_GetActorLocation`) (* (`self.GetActorUpVector`) -5000.0)) "TraceTypeQuery1" true))
  (if (`GameplayStatics.BreakHitResult` _outhit)
    (`self.K2_SetActorLocation` (`.ImpactPoint` (`GameplayStatics.BreakHitResult` _outhit)))))

(fn `UserConstructionScript`)