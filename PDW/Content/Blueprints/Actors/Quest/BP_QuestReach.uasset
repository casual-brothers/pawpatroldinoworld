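; BP_QuestReach is a quest "reach this location" marker that highlights itself while it is tagged as a quest target.
; PDWTag add and remove events, plus a check on BeginPlay, toggle the HighlightReach effect and spawn an end Niagara burst on deactivation.
; Entering the FlowTriggerComponent while tagged plays the "StepCompleted" UI event.
; A SnapToGround function line-traces vertically to place the actor on the surface below.
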(event `self.ReceiveActorBeginOverlap`
  (params (OtherActor :type "Actor Object Reference")))

(event `self.ReceiveBeginPlay`
  (bind _returnvalue (`QuestSettings.GetQuestTargetTag`))
  (bind _pdwtag (`self.PDWTag`))
  (add `PDWTagComponent.OnPDWTagAdded` _pdwtag (delegate `ShowQuestIcon`))
  (add `PDWTagComponent.OnPDWTagRemoved` _pdwtag (delegate `HideQuestIcon`))
  (if (`BlueprintGameplayTagLibrary.HasTag` (`PDWTagComponent.TagContainer` _pdwtag) _returnvalue)
    (`self.ShowQuestIcon` (struct) _returnvalue)
    (else
      (`self.HideQuestIcon` (struct) _returnvalue))))

(event `ShowQuestIcon`
  (params (UpdatedContainer :type "GameplayTagContainer Structure (by ref)") (NewTagAdded :type "GameplayTag Structure (by ref)"))
  (if (`BlueprintGameplayTagLibrary.MatchesTag` NewTagAdded (`QuestSettings.GetQuestTargetTag`))
    (`ActorComponent.Activate` (`self.HighlightReach`) true)))

(event `HideQuestIcon`
  (params (UpdatedContainer :type "GameplayTagContainer Structure (by ref)") (TagRemoved :type "GameplayTag Structure (by ref)"))
  (if (`BlueprintGameplayTagLibrary.MatchesTag` TagRemoved (`QuestSettings.GetQuestTargetTag`))
    (`ActorComponent.Deactivate` (`self.HighlightReach`))
    (`NiagaraFunctionLibrary.SpawnSystemAttached` "/Game/Art/VFX/NiagaraSystem/Generic/NS_HighlightReach_End.NS_HighlightReach_End" (`self.HighlightReach`) "None" (0.0 0.0 0.0) (struct) "KeepRelativeOffset" true)))

(event `self.ReceiveEndPlay`
  (params (EndPlayReason :type "EEndPlayReason Enum" :default "Destroyed"))
  (bind _pdwtag (`self.PDWTag`))
  (remove `PDWTagComponent.OnPDWTagAdded` _pdwtag (delegate `ShowQuestIcon`))
  (remove `PDWTagComponent.OnPDWTagRemoved` _pdwtag (delegate `HideQuestIcon`)))

(event `self.FlowTriggerComponent.OnTriggerEvent`
  (params (bOverlapping :type Boolean) (OtherFlowComponent :type "FlowComponent Object Reference") (SourceFlowComponent :type "FlowComponent Object Reference"))
  (if bOverlapping
    (if (`BlueprintGameplayTagLibrary.HasTag` (`PDWTagComponent.TagContainer` (`self.PDWTag`)) (`QuestSettings.GetQuestTargetTag`))
      (`NebulaFlowAudioFunctionLibrary.PlayUIEvent` "StepCompleted"))))

(fn `SnapToGround`
  (bind _outhit (`KismetSystemLibrary.LineTraceSingle` (+ (`self.K2_GetActorLocation`) (* (`self.GetActorUpVector`) 200.0)) (+ (`self.K2_GetActorLocation`) (* (`self.GetActorUpVector`) -5000.0)) "TraceTypeQuery1" true))
  (if (`GameplayStatics.BreakHitResult` _outhit)
    (`self.K2_SetActorLocation` (`.ImpactPoint` (`GameplayStatics.BreakHitResult` _outhit)))))

(fn `UserConstructionScript`)