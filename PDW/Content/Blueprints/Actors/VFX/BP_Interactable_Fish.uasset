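; Interactable fish VFX actor that feeds the player's position to Niagara while its sphere is overlapped.
; Sphere overlaps by any valid actor set or clear an Overlap flag, and both events enable Tick, which is never disabled here.
; While the flag is set, Tick writes the first player character's location, slightly lowered, into the PlayerPosition parameter of the NPC_PlayerLocation Niagara Parameter Collection.
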(event `self.ReceiveTick`
  (params (DeltaSeconds :type "Float (single-precision)"))
  (if (`self.Overlap`)
    (bind _returnvalue (`NiagaraFunctionLibrary.GetNiagaraParameterCollection` "/Game/Art/VFX/NiagaraSystem/NPC/NPC_PlayerLocation.NPC_PlayerLocation"))
    (`NiagaraParameterCollectionInstance.SetVectorParameter` _returnvalue "PlayerPosition" (- (`self.K2_GetActorLocation` (`GameplayStatics.GetPlayerCharacter` 0)) (0.0 0.0 15.0)))))

(event `self.Sphere.OnComponentBeginOverlap`
  (params (OverlappedComponent :type "PrimitiveComponent Object Reference") (OtherActor :type "Actor Object Reference") (OtherComp :type "PrimitiveComponent Object Reference") (OtherBodyIndex :type Integer) (bFromSweep :type Boolean) (SweepResult :type "HitResult Structure (by ref)"))
  (`/Engine/EditorBlueprintResources/StandardMacros.IsValid` OtherActor
    (:`Is Valid`
      (set `self.Overlap` true)
      (`self.SetActorTickEnabled` true))))

(event `self.Sphere.OnComponentEndOverlap`
  (params (OverlappedComponent :type "PrimitiveComponent Object Reference") (OtherActor :type "Actor Object Reference") (OtherComp :type "PrimitiveComponent Object Reference") (OtherBodyIndex :type Integer))
  (`/Engine/EditorBlueprintResources/StandardMacros.IsValid` OtherActor
    (:`Is Valid`
      (set `self.Overlap` false)
      (`self.SetActorTickEnabled` true))))

(fn `UserConstructionScript`)