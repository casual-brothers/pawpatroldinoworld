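; Base actor for skill-spawned objects that deliver a skill interaction to whatever receiver they overlap.
; On overlap with a PDW interaction receiver component, it spawns a Niagara hit effect at its own location and sends a payload with its owner and the ability's skill action type.
; A Tick countdown periodically flips the collision's response on one game trace channel to Ignore and back to Overlap, resetting that overlap response.
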(event `self.ReceiveBeginPlay`
  (set `self.ResetCollisionTime` (`self.DefaultResetCollisionTime`)))

(event `self.ReceiveTick`
  (params (DeltaSeconds :type "Float (single-precision)"))
  (bind _collision (`self.Collision`))
  (bind _output_get (set `self.ResetCollisionTime` (- (`self.ResetCollisionTime`) DeltaSeconds)))
  (if (<= _output_get 0.0)
    (`PrimitiveComponent.SetCollisionResponseToChannel` _collision "ECC_GameTraceChannel5" "ECR_Ignore")
    (`PrimitiveComponent.SetCollisionResponseToChannel` _collision "ECC_GameTraceChannel5" "ECR_Overlap")
    (set `self.ResetCollisionTime` (`self.DefaultResetCollisionTime`))))

(event `self.Collision.OnComponentBeginOverlap`
  (params (OverlappedComponent :type "PrimitiveComponent Object Reference") (OtherActor :type "Actor Object Reference") (OtherComp :type "PrimitiveComponent Object Reference") (OtherBodyIndex :type Integer) (bFromSweep :type Boolean) (SweepResult :type "HitResult Structure (by ref)"))
  (`self.OnHit` OtherComp))

(fn `OnHit`
  (params (OtherComp :type "PrimitiveComponent Object Reference"))
  (bind _aspdwinteraction_receiver_component (cast `PDWInteractionReceiverComponent` OtherComp))
  (`NiagaraFunctionLibrary.SpawnSystemAtLocation` (`self.NiagaraHit`) (`self.K2_GetActorLocation`) (struct) (1.0 1.0 1.0) true true "AutoRelease")
  (`PDWInteractionReceiverComponent.ProcessInteraction` _aspdwinteraction_receiver_component (make `PDWInteractionPayload` (`self.GetOwner`) (struct) (`.SkillActionType` (break `AbilityInfo` (`self.GetAbilityInfo`))))))

(fn `UserConstructionScript`)