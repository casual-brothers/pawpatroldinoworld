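; Area actor for the Water Gun skill that leaves a temporary wet decal on the ground.
; On BeginPlay it projects the decal downward at the SceneOrizz component's location with a randomized lifespan, then sets it to fade in quickly and fade out later.
; The random branch and overlap event do nothing, and the vertical-wall decal and overlap debug print are disconnected.
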(event `self.ReceiveActorBeginOverlap`
  (params (OtherActor :type "Actor Object Reference")))

(event `self.ReceiveBeginPlay`
  (bind _returnvalue (`KismetMathLibrary.RandomFloatInRange` 100.0 100.0))
  (if (>= (`KismetMathLibrary.RandomIntegerInRange` 0 1) 1)
    _
    (else
      _))
  ;[0.003474 0.15 0 0.5] Decal On Plane
  (bind _returnvalue_2 (`GameplayStatics.SpawnDecalAtLocation` "/Game/Art/VFX/MaterialInstances/MI_WetDecal.MI_WetDecal" (`KismetMathLibrary.MakeVector` 200.0 _returnvalue _returnvalue) (`SceneComponent.K2_GetComponentLocation` (`self.Scene_Orizz`)) (`KismetMathLibrary.MakeRotator` 0.0 -90.0) (`KismetMathLibrary.RandomFloatInRange` 8.0 12.0)))
  (`DecalComponent.SetFadeIn` _returnvalue_2 0.0 0.25)
  (`DecalComponent.SetFadeOut` _returnvalue_2 6.0 4.0 true))

(fn `UserConstructionScript`)