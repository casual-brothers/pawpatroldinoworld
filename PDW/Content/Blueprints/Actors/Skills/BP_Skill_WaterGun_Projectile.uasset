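; Water Gun skill projectile that leaves a temporary wet decal in the world.
; Shortly after BeginPlay, it spawns a randomly sized decal at its current location, on a timer independent of any hit, then fades it in and later out.
; OnHit runs the parent's hit logic, then immediately stops projectile movement.
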(event `self.ReceiveBeginPlay`
  (bind _returnvalue (`KismetMathLibrary.RandomFloatInRange` 75.0 150.0))
  (`KismetSystemLibrary.Delay` 0.15)
  (bind _returnvalue_2 (`GameplayStatics.SpawnDecalAtLocation` "/Game/Materials/BaseMaterials/VFX/M_WetDecal.M_WetDecal" (`KismetMathLibrary.MakeVector` _returnvalue _returnvalue _returnvalue) (`self.K2_GetActorLocation`) (struct :`Pitch` -90.0) (`KismetMathLibrary.RandomFloatInRange` 8.0 12.0)))
  (`DecalComponent.SetFadeIn` _returnvalue_2 0.0 0.25)
  (`DecalComponent.SetFadeOut` _returnvalue_2 6.0 4.0 true))

(fn `OnHit`
  (params (OtherComp :type "PrimitiveComponent Object Reference"))
  (`parent.OnHit` OtherComp)
  (`MovementComponent.StopMovementImmediately` (`self.ProjectileMovement`)))

(fn `UserConstructionScript`)