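; Target actor for the water hose minigame, exposing its PDWDeployable as the minigame target component.
; When the minigame starts, it runs the activating behaviour on its InteractionReceiverComponent.
; Each finished behaviour sets that component's collision to none when inactive, query-only otherwise.
; RandomizeStainDecal sets a random scalar on a new dynamic stain material, but is not called or assigned back to the decal here.
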(event `self.PDWDeployable.OnMinigameStartedEvent`
  (`PDWInteractionReceiverComponent.ExecuteInteractionBehaviour` (`self.InteractionReceiverComponent`) (`self.ActivatingBehaviour`) self false false))

(event `self.InteractionReceiverComponent.OnBehaviourFinished`
  (params (Behaviour :type "PDWInteractionBehaviour Object Reference"))
  (bind _interactionreceivercomponent (`self.InteractionReceiverComponent`))
  (if (== (`PDWInteractionReceiverComponent.GetCurrentState` _interactionreceivercomponent) (struct :`TagName` "InteractionState.Inactive"))
    (`PrimitiveComponent.SetCollisionEnabled` _interactionreceivercomponent "NoCollision")
    (else
      (`PrimitiveComponent.SetCollisionEnabled` _interactionreceivercomponent "QueryOnly"))))

(fn `BP_GetMinigameTargetComponent`
  (returns (ReturnValue :type "PDWMinigameTargetComponent Object Reference"))
  (return (`self.PDWDeployable`)))

(fn `RandomizeStainDecal`
  (bind _returnvalue (`DecalComponent.GetDecalMaterial` (`self.Decal`)))
  (`/Engine/EditorBlueprintResources/StandardMacros.IsValid` _returnvalue
    (:`Is Valid`
      (bind _returnvalue_2 (`KismetMaterialLibrary.CreateDynamicMaterialInstance` _returnvalue))
      (`/Engine/EditorBlueprintResources/StandardMacros.IsValid` _returnvalue_2
        (:`Is Valid`
          (`MaterialInstanceDynamic.SetScalarParameterValueByInfo` _returnvalue_2 (make `MaterialParameterInfo` "RandomValue") (`KismetMathLibrary.RandomFloatInRange` 0.0 1.0)))))))

(fn `UserConstructionScript`
  (`parent.UserConstructionScript`))