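; Rock target actor for the drill excavation minigame, exposing its PDWDeployable as the minigame target component.
; On BeginPlay it randomly rolls its mesh in 90-degree steps for visual variety.
; Minigame start sets the mesh, unhides the actor and enables query-only targeting collision.
; When an interaction behaviour finishes in the Broken state, it reports rock removal to the PDW event subsystem and disables that collision.
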(event `self.ReceiveBeginPlay`
  (bind _staticmesh (`self.StaticMesh`))
  (bind (_returnvalue_roll _returnvalue_pitch _returnvalue_yaw) (`KismetMathLibrary.BreakRotator` (`SceneComponent.K2_GetComponentRotation` _staticmesh)))
  (`SceneComponent.K2_SetWorldRotation` _staticmesh (`KismetMathLibrary.MakeRotator` (+ _returnvalue_roll (* (`KismetMathLibrary.RandomIntegerInRange` 0 3) 90)) _returnvalue_pitch _returnvalue_yaw) false false))

(event `self.InteractionReceiverComponent.OnInteractionSuccessful`
  (params (Payload :type "PDWInteractionPayload Structure (by ref)"))
  ; Notify the Minigame Event on State Change
  (set `self.PreviousState` (`PDWInteractionReceiverComponent.GetCurrentState` (`self.InteractionReceiverComponent`))))

(event `self.InteractionReceiverComponent.OnBehaviourFinished`
  (params (Behaviour :type "PDWInteractionBehaviour Object Reference"))
  ; Notify the Minigame Event on State Change
  (if (== (`PDWInteractionReceiverComponent.GetCurrentState` (`self.InteractionReceiverComponent`)) (struct :`TagName` "InteractionState.Broken"))
    (`PDWEventSubsytem.OnRockRemovedEvent` (subsystem `PDWEventSubsytem`) self)
    (`PrimitiveComponent.SetCollisionEnabled` (`self.PDWDrillExcavationTargetingComponent`) "NoCollision")))

(event `self.PDWDeployable.OnMinigameStartedEvent`
  (`PrimitiveComponent.SetCollisionEnabled` (`self.PDWDrillExcavationTargetingComponent`) "QueryOnly")
  (`StaticMeshComponent.SetStaticMesh` (`self.StaticMesh`) (`self.Mesh01`))
  (`self.SetActorHiddenInGame` self false))

(fn `BP_GetMinigameTargetComponent`
  (returns (ReturnValue :type "PDWMinigameTargetComponent Object Reference"))
  (return (`self.PDWDeployable`)))

(fn `UserConstructionScript`)