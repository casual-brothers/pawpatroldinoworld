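; Goal actor for the Drill Excavation minigame, exposing its PDWDeployable component as the minigame target component.
; BeginPlay caches the static mesh's first material.
; When the deployable signals minigame start, it creates a dynamic instance from that cached material, sets its Color to dark blue, and resets the DrillExcavationGoalTargetingComponent.
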(event `self.ReceiveBeginPlay`
  (`parent.ReceiveBeginPlay`)
  (set `self.Storedmaterial` (`PrimitiveComponent.GetMaterial` (`self.StaticMesh`) 0)))

(event `self.PDWDeployable.OnMinigameStartedEvent`
  (bind _returnvalue (`PrimitiveComponent.CreateDynamicMaterialInstance` (`self.StaticMesh`) 0 (`self.Storedmaterial`) "None"))
  (`MaterialInstanceDynamic.SetVectorParameterValue` _returnvalue "Color" (`KismetMathLibrary.MakeColor` 0.0 0.06301 0.246201))
  (`PDWDrillExcavationTargetingComp.Reset` (`self.DrillExcavationGoalTargetingComponent`)))

(fn `BP_GetMinigameTargetComponent`
  (returns (ReturnValue :type "PDWMinigameTargetComponent Object Reference"))
  (return (`self.PDWDeployable`)))

(fn `UserConstructionScript`)