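; Roaming log actor for the Bulldozer Scoop minigame that reappears after being used.
; On BeginPlay it adds its interaction states through the PDWInteraction component and binds to that component's state-removed event.
; When states are removed, it starts a timer of random length between MinTime and MaxTime.
; When the timer fires, it re-adds the states and makes the Log visible again.
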(event `self.ReceiveBeginPlay`
  (`self.SetInteractionStates`)
  (add `PDWInteractionComponent.OnInteractionStateRemoved` (`self.PDWInteraction`) (delegate `OnStateRemoved`)))

(event `OnStateRemoved`
  (params (outTagsRemoved :type "GameplayTagContainer Structure (by ref)"))
  (`KismetSystemLibrary.K2_SetTimerDelegate` (delegate `On Time Off`) (`KismetMathLibrary.RandomFloatInRange` (`self.Min Time`) (`self.Max Time`))))

(event `On Time Off`
  (`self.SetInteractionStates`)
  (`SceneComponent.SetVisibility` (`self.Log`) true false))

(fn `SetInteractionStates`
  (`PDWInteractionComponent.AddOwnerInteractionStates` (`self.PDWInteraction`) (`self.In Container`)))

(fn `UserConstructionScript`)