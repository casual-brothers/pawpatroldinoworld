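; Dropped item in the Bulldozer Scoop minigame that penalizes a player who runs into it.
; On mesh overlap, a vehicle that is not boosting gets a timed speed debuff, and a stun Niagara effect looping for the same duration attaches to the pup.
; Regardless of boost, it asks its owning drop area to reset state, plays destroy VFX and impact force feedback, then destroys itself.
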(event `self.StaticMesh.OnComponentHit`
  (params (HitComponent :type "PrimitiveComponent Object Reference") (OtherActor :type "Actor Object Reference") (OtherComp :type "PrimitiveComponent Object Reference") (NormalImpulse :type "Vector Structure") (Hit :type "HitResult Structure (by ref)")))

(event `self.StaticMesh.OnComponentBeginOverlap`
  (params (OverlappedComponent :type "PrimitiveComponent Object Reference") (OtherActor :type "Actor Object Reference") (OtherComp :type "PrimitiveComponent Object Reference") (OtherBodyIndex :type Integer) (bFromSweep :type Boolean) (SweepResult :type "HitResult Structure (by ref)"))
  (bind _debuffduration (`self.DebuffDuration`))
  (bind _aspdwplayer_interface (cast `PDWPlayerInterface` OtherActor))
  (bind _returnvalue (`PDWPlayerInterface.GetPDWPlayerController` _aspdwplayer_interface))
  (bind _returnvalue_2 (`PDWPlayerController.GetVehicleInstance` _returnvalue))
  (bind _returnvalue_3 (`PDWPlayerController.GetPupInstance` _returnvalue))
  (if (not (`PDWVehiclePawn.GetBoosting` _returnvalue_2))
    (`PDWVehiclePawn.ApplyVehicleDebuff` _returnvalue_2 (`self.Speed Multiplier`) false _debuffduration 0.0)
    (bind _rootcomponent (`Actor.RootComponent` _returnvalue_3))
    (bind _returnvalue_4 (`NiagaraFunctionLibrary.SpawnSystemAttached` (`self.NiagaraStun`) _rootcomponent "None" (0.0 0.0 300.0) (struct) "SnapToTarget"))
    (`NiagaraComponent.SetVariableFloat` _returnvalue_4 "LoopDuration" _debuffduration)
    (`SceneComponent.K2_AttachToComponent` _returnvalue_4 _rootcomponent "None" "SnapToTarget" "SnapToTarget" "KeepRelative" true))
  (bind _asbp_minigame_bulldozer_scoop_drop_area (cast `/Game/Blueprints/Actors/MiniGames/BulldozerScoop/BP_Minigame_BulldozerScoop_DropArea` (`self.GetOwner`)))
  (`/Game/Blueprints/Actors/MiniGames/BulldozerScoop/BP_Minigame_BulldozerScoop_DropArea.RequestResetState` _asbp_minigame_bulldozer_scoop_drop_area)
  (`NiagaraFunctionLibrary.SpawnSystemAtLocation` (`self.NiagaraDestroy`) (`SceneComponent.K2_GetComponentLocation` (`self.StaticMesh`)) (`self.K2_GetActorRotation` _asbp_minigame_bulldozer_scoop_drop_area))
  (`PDWGameplayFunctionLibrary.PlayForceFeedback` (`|MakeArray` _returnvalue) (struct :`TagName` "ID.Vibration.VehicleImpact"))
  (`self.K2_DestroyActor`))

(fn `UserConstructionScript`)