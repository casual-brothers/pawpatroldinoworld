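; Scoop target actor for the bulldozer minigame, the variant without a wall.
; On BeginPlay it picks a random mesh, snaps the interaction receiver to it and drops its scene component onto the surface found by a downward trace.
; Pickup by the rubble vehicle disables physics and collision, then attaches the mesh to the scoop socket with a random rotation.
; It exposes PDWDeployable as the minigame target component; its behaviour-finished handler is empty.
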(event `self.ReceiveBeginPlay`
  (bind _itemstospawn (`self.ItemsToSpawn`))
  (bind _staticmesh (`self.StaticMesh`))
  (`StaticMeshComponent.SetStaticMesh` (`self.StaticMesh`) (`|GetArrayItem` _itemstospawn (`KismetMathLibrary.RandomIntegerInRange` 0 (`KismetArrayLibrary.Array_LastIndex` _itemstospawn))))
  (`SceneComponent.K2_AttachToComponent` (`self.BP_InteractionReceiverComponent`) _staticmesh "None" "SnapToTarget" "KeepWorld" "KeepWorld" true)
  (`SceneComponent.K2_SetRelativeRotation` _staticmesh (`KismetMathLibrary.MakeRotator` 0.0) false false)
  (bind _outhit (`KismetSystemLibrary.LineTraceSingle` (+ (`self.K2_GetActorLocation`) (* (`self.GetActorUpVector`) 200.0)) (+ (`self.K2_GetActorLocation`) (* (`self.GetActorUpVector`) -5000.0)) "TraceTypeQuery1"))
  (if (`GameplayStatics.BreakHitResult` _outhit)
    (`SceneComponent.K2_SetWorldLocation` (`self.Scene`) (`.ImpactPoint` (`GameplayStatics.BreakHitResult` _outhit)) false false)))

(event `self.BP_InteractionReceiverComponent.OnBehaviourFinished`
  (params (Behaviour :type "PDWInteractionBehaviour Object Reference")))

(fn `BP_GetMinigameTargetComponent`
  (returns (ReturnValue :type "PDWMinigameTargetComponent Object Reference"))
  (return (`self.PDWDeployable`)))

(fn `Pickup`
  (params (OtherActor :type "Actor Object Reference") (OtherComponent :type "PrimitiveComponent Object Reference"))
  (bind _staticmesh (`self.StaticMesh`))
  (bind _staticmesh_2 (`self.StaticMesh`))
  (if (== (`GameplayStatics.GetObjectClass` OtherActor) "/Game/Blueprints/Pawn/Vehicles/BP_VH_04_Rubble.BP_VH_04_Rubble_C")
    (`PrimitiveComponent.SetSimulatePhysics` _staticmesh false)
    (`PrimitiveComponent.SetCollisionEnabled` _staticmesh "NoCollision")
    (bind _returnvalue (`SceneComponent.K2_AttachToComponent` _staticmesh_2 (`|GetArrayItem` (`self.GetComponentsByTag` OtherActor "/Script/Engine.StaticMeshComponent" "ComponentTag.VehicleMesh")) "ScoopSocket" "SnapToTarget" "KeepRelative" "KeepRelative" true))
    (`SceneComponent.K2_SetWorldRotation` _staticmesh_2 (`KismetMathLibrary.RandomRotator` _returnvalue) false false)))

(fn `UserConstructionScript`)