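; Scent target actor for the SuperSmell minigame, whose interaction receiver state decides whether it reads as a right or wrong target.
; Entering its Visibility volume recolors the Niagara marker when Full; when Empty it shuts the marker off, vibrates the player's controller and spawns a one-time wrong-target effect.
; Leaving restores the default color.
; A successful Filling or Emptying hides the clue, disables receiver overlaps and reports deactivation to the event subsystem.
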(event `self.BP_InteractionReceiverComponent.OnBehaviourFinished`
  (params (Behaviour :type "PDWInteractionBehaviour Object Reference"))
  (bind _behaviouridentifier (`PDWInteractionBehaviour.BehaviourIdentifier` Behaviour))
  (if (and (`PDWInteractionBehaviour.bNotifySuccess` Behaviour) (or (== _behaviouridentifier (struct :`TagName` "InteractionBehaviour.Filling")) (== _behaviouridentifier (struct :`TagName` "InteractionBehaviour.Emptying"))))
    (`SceneComponent.SetHiddenInGame` (`self.Clue`) true true)
    (set `PrimitiveComponent.bGenerateOverlapEvents` false (`self.BP_InteractionReceiverComponent`))
    (`PDWEventSubsytem.OnTargetDeactivationEvent` (subsystem `PDWEventSubsytem`) self)))

(event `self.Visibility.OnComponentBeginOverlap`
  (params (OverlappedComponent :type "PrimitiveComponent Object Reference") (OtherActor :type "Actor Object Reference") (OtherComp :type "PrimitiveComponent Object Reference") (OtherBodyIndex :type Integer) (bFromSweep :type Boolean) (SweepResult :type "HitResult Structure (by ref)"))
  (bind _returnvalue (`PDWInteractionReceiverComponent.GetCurrentState` (`self.BP_InteractionReceiverComponent`)))
  (if (== _returnvalue (struct :`TagName` "InteractionState.Full"))
    (`self.SetNiagaraTargetColor` (`self.RightColor`))
    (elif (== _returnvalue (struct :`TagName` "InteractionState.Empty"))
      (`|ExecutionSequence`
        (:`then_0`
          (`ActorComponent.Deactivate` (`self.Niagara_Target`))
          (bind _aspawn (cast `Pawn` OtherActor))
          (bind _aspdwplayer_controller (cast `PDWPlayerController` (`Pawn.GetController` _aspawn)))
          (`PDWGameplayFunctionLibrary.PlayForceFeedback` (`|MakeArray` _aspdwplayer_controller) (struct :`TagName` "ID.Vibration.Bark")))
        (:`then_1`
          (`/Engine/EditorBlueprintResources/StandardMacros.DoOnce` false
            (:`Completed`
              (`NiagaraFunctionLibrary.SpawnSystemAtLocation` "/Game/Art/VFX/NiagaraSystem/MiniGame/NS_MG_Chase_SuperSmell_WrongTarget.NS_MG_Chase_SuperSmell_WrongTarget" (`SceneComponent.K2_GetComponentLocation` (`self.Niagara_Target`))))))))))

(event `self.Visibility.OnComponentEndOverlap`
  (params (OverlappedComponent :type "PrimitiveComponent Object Reference") (OtherActor :type "Actor Object Reference") (OtherComp :type "PrimitiveComponent Object Reference") (OtherBodyIndex :type Integer))
  (`self.SetNiagaraTargetColor` (`self.DefaultColor`)))

(event `self.K2_OnReset`
  (`parent.K2_OnReset`)
  (`KismetSystemLibrary.PrintString` "Changeee!!"))

(fn `SetNiagaraTargetColor`
  (params (NewColor :type "LinearColor Structure (by ref)"))
  (bind _niagara_target (`self.Niagara_Target`))
  (`NiagaraComponent.SetVariableLinearColor` _niagara_target "SecondaryColor" NewColor)
  (`NiagaraComponent.SetVariableLinearColor` _niagara_target "MainColor" NewColor))

(fn `UserConstructionScript`)