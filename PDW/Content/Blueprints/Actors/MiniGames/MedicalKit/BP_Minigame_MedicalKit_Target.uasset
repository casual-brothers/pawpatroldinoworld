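; Target actor for the medical kit minigame, representing one of six two-piece bone models with a targeting box.
; InitializeMesh matches the socket name against SocketPrefix plus a number to assign both bone meshes and fit the PDWTargeting box's location and extent.
; BeginPlay caches the second bone's relative transform, which the deployable's minigame-started event restores while re-enabling actor collision.
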(event `self.ReceiveBeginPlay`
  (`parent.ReceiveBeginPlay`)
  (set `self.SecondBoneTransform` (`SceneComponent.GetRelativeTransform` (`self.StaticMesh_B`))))

(event `self.PDWDeployable.OnMinigameStartedEvent`
  (`SceneComponent.K2_SetRelativeTransform` (`self.StaticMesh_B`) (`self.SecondBoneTransform`) false false)
  (`self.SetActorEnableCollision` true))

(fn `InitializeMesh`
  (params (socketName :type Name))
  (locals (SkeletonWorldZRotation :type "Float (double-precision)"))
  (bind _returnvalue (`KismetStringLibrary.Conv_NameToString` socketName))
  (bind _pdwtargeting (`self.PDWTargeting`))
  (bind _pdwtargeting_2 (`self.PDWTargeting`))
  (bind _pdwtargeting_3 (`self.PDWTargeting`))
  (bind _pdwtargeting_4 (`self.PDWTargeting`))
  (bind _pdwtargeting_5 (`self.PDWTargeting`))
  (bind _pdwtargeting_6 (`self.PDWTargeting`))
  (if (`KismetStringLibrary.StartsWith` _returnvalue (`KismetStringLibrary.Concat_StrStr` (`self.SocketPrefix`) "01"))
    (`StaticMeshComponent.SetStaticMesh` (`self.StaticMesh`) "/Game/Art/Environments/Minigames/MedicalKit/StaticMeshes/SM_Minigame_MedicalKit_Bones_01_A.SM_Minigame_MedicalKit_Bones_01_A")
    (`StaticMeshComponent.SetStaticMesh` (`self.StaticMesh_B`) "/Game/Art/Environments/Minigames/MedicalKit/StaticMeshes/SM_Minigame_MedicalKit_Bones_01_B.SM_Minigame_MedicalKit_Bones_01_B")
    (`SceneComponent.K2_SetRelativeLocation` _pdwtargeting (1.0 -22.0 -36.0) false false)
    (`BoxComponent.SetBoxExtent` _pdwtargeting (7.0 7.0 20.0) true)
    (elif (`KismetStringLibrary.StartsWith` _returnvalue (`KismetStringLibrary.Concat_StrStr` (`self.SocketPrefix`) "02"))
      (`StaticMeshComponent.SetStaticMesh` (`self.StaticMesh`) "/Game/Art/Environments/Minigames/MedicalKit/StaticMeshes/SM_Minigame_MedicalKit_Bones_02_A.SM_Minigame_MedicalKit_Bones_02_A")
      (`StaticMeshComponent.SetStaticMesh` (`self.StaticMesh_B`) "/Game/Art/Environments/Minigames/MedicalKit/StaticMeshes/SM_Minigame_MedicalKit_Bones_02_B.SM_Minigame_MedicalKit_Bones_02_B")
      (`SceneComponent.K2_SetRelativeLocation` _pdwtargeting_4 (1.5 -2.0 -31.0) false false)
      (`BoxComponent.SetBoxExtent` _pdwtargeting_4 (7.0 7.0 15.0) true)
      (elif (`KismetStringLibrary.StartsWith` _returnvalue (`KismetStringLibrary.Concat_StrStr` (`self.SocketPrefix`) "03"))
        (`StaticMeshComponent.SetStaticMesh` (`self.StaticMesh`) "/Game/Art/Environments/Minigames/MedicalKit/StaticMeshes/SM_Minigame_MedicalKit_Bones_03_A.SM_Minigame_MedicalKit_Bones_03_A")
        (`StaticMeshComponent.SetStaticMesh` (`self.StaticMesh_B`) "/Game/Art/Environments/Minigames/MedicalKit/StaticMeshes/SM_Minigame_MedicalKit_Bones_03_B.SM_Minigame_MedicalKit_Bones_03_B")
        (`SceneComponent.K2_SetRelativeLocation` _pdwtargeting_3 (1.0 0.0 -16.0) false false)
        (`BoxComponent.SetBoxExtent` _pdwtargeting_3 (5.0 5.0 10.0) true)
        (elif (`KismetStringLibrary.StartsWith` _returnvalue (`KismetStringLibrary.Concat_StrStr` (`self.SocketPrefix`) "04"))
          (`StaticMeshComponent.SetStaticMesh` (`self.StaticMesh`) "/Game/Art/Environments/Minigames/MedicalKit/StaticMeshes/SM_Minigame_MedicalKit_Bones_04_A.SM_Minigame_MedicalKit_Bones_04_A")
          (`StaticMeshComponent.SetStaticMesh` (`self.StaticMesh_B`) "/Game/Art/Environments/Minigames/MedicalKit/StaticMeshes/SM_Minigame_MedicalKit_Bones_04_B.SM_Minigame_MedicalKit_Bones_04_B")
          (`SceneComponent.K2_SetRelativeLocation` _pdwtargeting_5 (3.0 -12.0 -36.0) false false)
          (`BoxComponent.SetBoxExtent` _pdwtargeting_5 (9.0 9.0 20.0) true)
          (elif (`KismetStringLibrary.StartsWith` _returnvalue (`KismetStringLibrary.Concat_StrStr` (`self.SocketPrefix`) "05"))
            (`StaticMeshComponent.SetStaticMesh` (`self.StaticMesh`) "/Game/Art/Environments/Minigames/MedicalKit/StaticMeshes/SM_Minigame_MedicalKit_Bones_05_A.SM_Minigame_MedicalKit_Bones_05_A")
            (`StaticMeshComponent.SetStaticMesh` (`self.StaticMesh_B`) "/Game/Art/Environments/Minigames/MedicalKit/StaticMeshes/SM_Minigame_MedicalKit_Bones_05_B.SM_Minigame_MedicalKit_Bones_05_B")
            (`SceneComponent.K2_SetRelativeLocation` _pdwtargeting_6 (0.0 -10.0 -24.0) false false)
            (`BoxComponent.SetBoxExtent` _pdwtargeting_6 (7.0 7.0 15.0) true)
            (elif (`KismetStringLibrary.StartsWith` _returnvalue (`KismetStringLibrary.Concat_StrStr` (`self.SocketPrefix`) "06"))
              (`StaticMeshComponent.SetStaticMesh` (`self.StaticMesh`) "/Game/Art/Environments/Minigames/MedicalKit/StaticMeshes/SM_Minigame_MedicalKit_Bones_06_A.SM_Minigame_MedicalKit_Bones_06_A")
              (`StaticMeshComponent.SetStaticMesh` (`self.StaticMesh_B`) "/Game/Art/Environments/Minigames/MedicalKit/StaticMeshes/SM_Minigame_MedicalKit_Bones_06_B.SM_Minigame_MedicalKit_Bones_06_B")
              (`SceneComponent.K2_SetRelativeLocation` _pdwtargeting_2 (0.0 0.0 -12.0) false false)
              (`BoxComponent.SetBoxExtent` _pdwtargeting_2 (3.5 3.5 6.5) true))))))))

(fn `UserConstructionScript`
  (`parent.UserConstructionScript`))