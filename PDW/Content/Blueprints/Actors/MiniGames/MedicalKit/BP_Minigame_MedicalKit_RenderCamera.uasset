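; Render camera actor for the medical kit minigame that captures the kit's skeleton and target actors to a render target.
; BeginPlay attaches it to the minigame's tagged component at the CameraAttach socket and fills the capture's show-only list with actors found by tag.
; Captures happen on demand: once on the first Tick, then on each OnMovingMeshBehaviour event from the PDW event subsystem, which rebinds after every capture.
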(event `self.ReceiveBeginPlay`
  (`self.K2_AttachToComponent` (`|GetArrayItem` (`self.GetComponentsByTag` (`self.Minigame`) "/Script/Engine.SceneComponent" (`self.Tag`))) "CameraAttach" "SnapToTarget" "SnapToTarget" "KeepRelative")
  (bind _outactors (`GameplayStatics.GetAllActorsWithTag` (`self.MedicalKitSkeletonTag`)))
  (`KismetArrayLibrary.Array_Append` (`self.MedicalKitMesh`) _outactors)
  (bind _outactors_2 (`GameplayStatics.GetAllActorsWithTag` (`self.MedicalKitTargetTag`)))
  (`KismetArrayLibrary.Array_Append` (`self.MedicalKitMesh`) _outactors_2)
  (set `SceneCaptureComponent.ShowOnlyActors` (`self.MedicalKitMesh`) (`self.CaptureComponent2D`))
  (set `self.IsRTInitialized` false)
  (add `PDWEventSubsytem.OnMovingMeshBehaviour` (subsystem `PDWEventSubsytem`) (delegate `CustomEvent`) :!label _label))

(event `CustomEvent`
  (params (SceneComponent :type "SceneComponent Object Reference"))
  (`SceneCaptureComponent2D.CaptureScene` (`self.CaptureComponent2D`))
  (goto _label))

(event `self.ReceiveTick`
  (params (DeltaSeconds :type "Float (single-precision)"))
  (if (not (`self.IsRTInitialized`))
    (`SceneCaptureComponent2D.CaptureScene` (`self.CaptureComponent2D`))
    (set `self.IsRTInitialized` true)))

(fn `UserConstructionScript`)