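; Skeleton actor for the Medical Kit minigame that pairs its own montage with the hurt animation of a Paleo Center dino.
; On BeginPlay it looks up the dino by gameplay tag through the PDW Paleo Center subsystem and starts both animations if found.
; Otherwise it binds to the subsystem's dino load event and starts them when a dino with an exactly matching pen tag loads.
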(event `self.ReceiveBeginPlay`
  (bind _returnvalue (subsystem `PDWPaleoCenterSubsystem`))
  (bind _paleodinotosync (`self.PaleoDinoToSync`))
  (if (`BlueprintGameplayTagLibrary.IsGameplayTagValid` _paleodinotosync)
    (bind _returnvalue_2 (`PDWPaleoCenterSubsystem.GetDinoActorRef` _returnvalue _paleodinotosync))
    (bind _asbp_npc_paleo_center_base (cast `/Game/Blueprints/Pawn/NPC/PaleoCenter/BP_NPC_PaleoCenter_Base` _returnvalue_2)
      (:`then`
        (`self.StartAnimations` _asbp_npc_paleo_center_base))
      (:`CastFailed`
        (add `PDWPaleoCenterSubsystem.OnDinoLoad` _returnvalue (delegate `OnDinoLoad`))))))

(event `OnDinoLoad`
  (params (DinoRef :type "Actor Object Reference"))
  (bind _returnvalue (`self.GetComponentByClass` DinoRef "/Script/PDW.PDWPaleoDinoComponent"))
  (`/Engine/EditorBlueprintResources/StandardMacros.IsValid` _returnvalue
    (:`Is Valid`
      (if (`BlueprintGameplayTagLibrary.MatchesTag` (`self.PaleoDinoToSync`) (`PDWPaleoDinoComponent.PenTag` _returnvalue) true)
        (bind _asbp_npc_paleo_center_base (cast `/Game/Blueprints/Pawn/NPC/PaleoCenter/BP_NPC_PaleoCenter_Base` DinoRef))
        (`self.StartAnimations` _asbp_npc_paleo_center_base)))))

(event `StartAnimations`
  (params (Dino :type "/Game/Blueprints/Pawn/NPC/PaleoCenter/BP_NPC_PaleoCenter_Base Object Reference"))
  (`/Game/Blueprints/Pawn/NPC/PaleoCenter/BP_NPC_PaleoCenter_Base.StartHurtAnimation` Dino)
  (`|PlayMontage` (`self.SkeletalMesh`) (`self.AnimToSync`)))

(fn `UserConstructionScript`)