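; Endless runner minigame ramp that takes over a player in the Minigame state and carries them along a spline.
; Entering the trigger deactivates the player through PDWPlayerInterface, registers them as ramp user and enables the PDWSplineRamp component, which Tick advances by scaled delta time.
; Leaving the exit trigger reactivates the player and disables the ramp logic.
; An optional custom camera blends the view to the ramp and back.
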(event `self.ReceiveBeginPlay`)

(event `self.ReceiveTick`
  (params (DeltaSeconds :type "Float (single-precision)"))
  (`PDWSplineRampComponent.MoveOnSpline` (`self.PDWSplineRamp`) (* DeltaSeconds (`self.Speed`))))

(event `self.RampTriggerEnter.OnComponentBeginOverlap`
  (params (OverlappedComponent :type "PrimitiveComponent Object Reference") (OtherActor :type "Actor Object Reference") (OtherComp :type "PrimitiveComponent Object Reference") (OtherBodyIndex :type Integer) (bFromSweep :type Boolean) (SweepResult :type "HitResult Structure (by ref)"))
  (bind _returnvalue (`PDWGameplayFunctionLibrary.GetPlayerControllerOne`))
  (bind _pdwsplineramp (`self.PDWSplineRamp`))
  (bind _aspdwplayer_interface (cast `PDWPlayerInterface` OtherActor))
  (bind _returnvalue_2 (`PDWPlayerInterface.GetPDWPlayerState` _aspdwplayer_interface))
  (`/Engine/EditorBlueprintResources/StandardMacros.IsValid` _returnvalue_2
    (:`Is Valid`
      (if (`BlueprintGameplayTagLibrary.HasTag` (`PDWPlayerState.GetPlayerStates` _returnvalue_2) (struct :`TagName` "InteractionType.Minigame"))
        (`PDWPlayerInterface.SetActivation` _aspdwplayer_interface false)
        (`PDWSplineRampComponent.SetRampUser` _pdwsplineramp OtherActor)
        (`PDWSplineRampComponent.SetLogicEnabled` _pdwsplineramp true)
        (if (`self.UseCustomCamera`)
          (set `self.CurrentCamera` (`Controller.GetViewTarget` _returnvalue))
          (`PlayerController.SetViewTargetWithBlend` _returnvalue self 1.0 "VTBlend_Linear" 0.0 false))))))

(event `self.RampTriggerExit.OnComponentEndOverlap`
  (params (OverlappedComponent :type "PrimitiveComponent Object Reference") (OtherActor :type "Actor Object Reference") (OtherComp :type "PrimitiveComponent Object Reference") (OtherBodyIndex :type Integer))
  (bind _aspdwplayer_interface (cast `PDWPlayerInterface` OtherActor))
  (bind _returnvalue (`PDWPlayerInterface.GetPDWPlayerState` _aspdwplayer_interface))
  (`/Engine/EditorBlueprintResources/StandardMacros.IsValid` _returnvalue
    (:`Is Valid`
      (if (`BlueprintGameplayTagLibrary.HasTag` (`PDWPlayerState.GetPlayerStates` _returnvalue) (struct :`TagName` "InteractionType.Minigame"))
        (`PDWPlayerInterface.SetActivation` _aspdwplayer_interface true)
        (`PDWSplineRampComponent.SetLogicEnabled` (`self.PDWSplineRamp`) false)
        (if (`self.UseCustomCamera`)
          (`PlayerController.SetViewTargetWithBlend` (`PDWGameplayFunctionLibrary.GetPlayerControllerOne`) (`self.CurrentCamera`) 1.0 "VTBlend_Linear" 0.0 false))))))

(fn `UserConstructionScript`)