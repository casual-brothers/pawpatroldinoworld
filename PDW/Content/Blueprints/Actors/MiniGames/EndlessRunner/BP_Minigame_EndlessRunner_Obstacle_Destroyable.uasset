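; Destroyable rock obstacle for the endless runner minigame, breakable while ram mode is on.
; BeginPlay gives the rock mesh a random yaw for visual variety.
; On box overlap in ram mode, it spawns Niagara dust and a timeline drives the material's "Display Frame" to play a vertex animation texture break, clearing the overlay material.
; Without ram mode, the overlap calls OnRamModeOff instead.
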(event `self.ReceiveBeginPlay`
  (`parent.ReceiveBeginPlay`)
  (`SceneComponent.K2_SetRelativeRotation` (`self.T_VAT_RockBig_mesh`) (`KismetMathLibrary.MakeRotator` 0.0 0.0 (`KismetMathLibrary.RandomFloatInRange` 0.0 270.0)) false false))

(event `self.Box.OnComponentBeginOverlap`
  (params (OverlappedComponent :type "PrimitiveComponent Object Reference") (OtherActor :type "Actor Object Reference") (OtherComp :type "PrimitiveComponent Object Reference") (OtherBodyIndex :type Integer) (bFromSweep :type Boolean) (SweepResult :type "HitResult Structure (by ref)"))
  (if (`self.bRamModeOn`)
    (`NiagaraFunctionLibrary.SpawnSystemAtLocation` "/Game/Art/VFX/NiagaraSystem/MiniGame/NS_MG_TimmyRamRockBreak_Dust.NS_MG_TimmyRamRockBreak_Dust" (+ (`self.K2_GetActorLocation`) (0.0 0.0 222.0)))
    (bind (_direction _newtrack_0) (`Timeline|Timeline` :!via `PlayFromStart`)
      (:`Update`
        (`MeshComponent.SetScalarParameterValueOnMaterials` (`self.T_VAT_RockBig_mesh`) "Display Frame" (+ _newtrack_0 1.0))
        (`MeshComponent.SetOverlayMaterial` (`self.T_VAT_RockBig_mesh`) null)))
    (else
      (`self.OnRamModeOff` null))))

(fn `UserConstructionScript`
  (`parent.UserConstructionScript`))