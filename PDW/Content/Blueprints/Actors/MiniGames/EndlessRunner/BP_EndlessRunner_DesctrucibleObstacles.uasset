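; Destructible obstacle for the endless runner minigame, extending a parent obstacle Blueprint.
; On BeginPlay it binds to the PDW event subsystem's ram-mode start and stop events to maintain a RamMode flag.
; Overlaps run the parent logic, then check RamMode, but that branch performs no action, so no destruction is implemented here.
; The construction script removes the inherited warning and jump effect components.
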(event `self.ReceiveBeginPlay`
  (bind _returnvalue (subsystem `PDWEventSubsytem`))
  (`parent.ReceiveBeginPlay`)
  (add `PDWEventSubsytem.OnRamMode` _returnvalue (delegate `OnRamMode_Event`))
  (add `PDWEventSubsytem.OnStopRamMode` _returnvalue (delegate `OnStopRamMode_Event`)))

(event `OnRamMode_Event`
  (set `self.bRamMode` true))

(event `OnStopRamMode_Event`
  (set `self.bRamMode` false))

(event `self.ReceiveActorBeginOverlap`
  (params (OtherActor :type "Actor Object Reference"))
  (`parent.ReceiveActorBeginOverlap` OtherActor)
  (if (`self.bRamMode`)
    _))

(fn `UserConstructionScript`
  (`parent.UserConstructionScript`)
  (`ActorComponent.K2_DestroyComponent` (`self.NS_Warning_EndlessRun`))
  (`ActorComponent.K2_DestroyComponent` (`self.NS_MG_EndlessRun_Jump`)))