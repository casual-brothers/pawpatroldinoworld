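; Target actor for the endless runner minigame that is visible and collidable only while multiplayer is on.
; On BeginPlay it subscribes to multiplayer state changes through the PDW event subsystem and applies the current state.
; Each state change reapplies visibility and collision, then binds to the minigame complete-or-left event, which refreshes them again.
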(event `self.ReceiveBeginPlay`
  (add `PDWEventSubsytem.OnMultiplayerStateChange` (subsystem `PDWEventSubsytem`) (delegate `OnMultiplayerStateChange`))
  (`self.UpdateVisibilityAndCollisions`))

(event `OnMultiplayerStateChange`
  (`self.UpdateVisibilityAndCollisions`)
  (add `PDWEventSubsytem.OnMinigameCompleteOrLeft` (subsystem `PDWEventSubsytem`) (delegate `CustomEvent`)))

(event `CustomEvent`
  (params (Actor :type "Actor Object Reference"))
  (`self.UpdateVisibilityAndCollisions`))

(fn `UpdateVisibilityAndCollisions`
  (bind _returnvalue (`PDWGameplayFunctionLibrary.IsMultiplayerOn`))
  (`self.SetActorHiddenInGame` (not _returnvalue))
  (`self.SetActorEnableCollision` _returnvalue))

(fn `UserConstructionScript`)