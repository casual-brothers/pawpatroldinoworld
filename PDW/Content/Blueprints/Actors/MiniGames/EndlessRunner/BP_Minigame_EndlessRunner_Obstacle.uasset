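; Base obstacle for the endless runner minigame that reacts when something overlaps its box.
; It tracks ram mode through the PDW event subsystem and routes overlaps to OnRamModeOn, which is empty here, or OnRamModeOff, which plays Timmy's slide montage on the runner pawn.
; UseJumpableObstacleVfx selects the jump or warning effect: the construction script destroys the unused component and BeginPlay activates the other.
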(event `self.ReceiveBeginPlay`
  (add `PDWEventSubsytem.OnRamMode` (subsystem `PDWEventSubsytem`) (delegate `OnStartRamMode`))
  (add `PDWEventSubsytem.OnStopRamMode` (subsystem `PDWEventSubsytem`) (delegate `OnStopRamMode`))
  (if (`self.UseJumpableObstacle_vfx`)
    (bind _ns_mg_endlessrun_jump (`self.NS_MG_EndlessRun_Jump`)
      (:`then`
        (`ActorComponent.SetActive` _ns_mg_endlessrun_jump true false)
        (bind _ns_warning_endlessrun (`self.NS_Warning_EndlessRun`)
          (:`then`
            (`ActorComponent.SetActive` _ns_warning_endlessrun false false))
          (:`else`)))
      (:`else`))
    (else
      (bind _ns_mg_endlessrun_jump_2 (`self.NS_MG_EndlessRun_Jump`)
        (:`then`
          (`ActorComponent.SetActive` _ns_mg_endlessrun_jump_2 false false)
          (bind _ns_warning_endlessrun_2 (`self.NS_Warning_EndlessRun`)
            (:`then`
              (`ActorComponent.SetActive` _ns_warning_endlessrun_2 true false))
            (:`else`)))
        (:`else`)))))

(event `OnStartRamMode`
  (set `self.bRamModeOn` true))

(event `OnStopRamMode`
  (set `self.bRamModeOn` false))

(event `self.Box.OnComponentBeginOverlap`
  (params (OverlappedComponent :type "PrimitiveComponent Object Reference") (OtherActor :type "Actor Object Reference") (OtherComp :type "PrimitiveComponent Object Reference") (OtherBodyIndex :type Integer) (bFromSweep :type Boolean) (SweepResult :type "HitResult Structure (by ref)"))
  (if (`self.bRamModeOn`)
    (`self.OnRamModeOn` OtherActor)
    (else
      (`self.OnRamModeOff` OtherActor))))

(fn `OnRamModeOff`
  (params (`Other Actor` :type "Actor Object Reference"))
  (bind _asbp_minigame_timmy_run_pawn (cast `/Game/Blueprints/Actors/MiniGames/EndlessRunner/BP_Minigame_TimmyRun_Pawn` `Other Actor`))
  (`Character.PlayAnimMontage` _asbp_minigame_timmy_run_pawn "/Game/Art/Characters/NPC_15_Timmy/Animation/AM_CH_Timmy_Slide.AM_CH_Timmy_Slide" 1.0 "None"))

(fn `OnRamModeOn`
  (params (OtherActor :type "Actor Object Reference")))

(fn `UserConstructionScript`
  (if (`self.UseJumpableObstacle_vfx`)
    (`ActorComponent.K2_DestroyComponent` (`self.NS_Warning_EndlessRun`))
    (else
      (`ActorComponent.K2_DestroyComponent` (`self.NS_MG_EndlessRun_Jump`)))))