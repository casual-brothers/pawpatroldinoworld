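; Target actor for the vehicle claws minigame: a small trunk that a minigame-tagged vehicle can interact with.
; Box overlap by that vehicle turns on trunk physics, registers the actor as an item in the player state and adds interaction states, and leaving reverses this.
; Tick keeps InteractionZone at the trunk's XY position and plays an attached sound while the trunk moves, stopping it at rest.
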(event `self.ReceiveTick`
  (params (DeltaSeconds :type "Float (single-precision)"))
  (bind _audio (`self.Audio`))
  (bind _audio_2 (`self.Audio`))
  (bind _interactionzone (`self.InteractionZone`))
  (bind (_returnvalue_x _returnvalue_y) (`KismetMathLibrary.BreakVector` (`SceneComponent.K2_GetComponentLocation` (`self.SM_Small_Trunk`))))
  (bind (_returnvalue_x_2 _returnvalue_y_2 _returnvalue_z) (`KismetMathLibrary.BreakVector` (`SceneComponent.K2_GetComponentLocation` _interactionzone)))
  (`SceneComponent.K2_SetWorldLocation` _interactionzone (`KismetMathLibrary.MakeVector` _returnvalue_x _returnvalue_y _returnvalue_z) false false)
  (if (== (`SceneComponent.GetComponentVelocity` (`self.SM_Small_Trunk`)) (0.0 0.0 0.0) :`ErrorTolerance` 0.1)
    (`/Engine/EditorBlueprintResources/StandardMacros.IsValid` _audio
      (:`Is Valid`
        (`FMODAudioComponent.Stop` _audio_2)))
    (else
      (`/Engine/EditorBlueprintResources/StandardMacros.IsValid` _audio
        (:`Is Valid`
          (bind _returnvalue (`FMODAudioComponent.IsPlaying` _audio_2))
          (if (not _returnvalue)
            (`FMODAudioComponent.Play` _audio_2)))
        (:`Is Not Valid`
          (bind _returnvalue_2 (`FMODBlueprintStatics.PlayEventAttached` "/Game/FMOD/Events/MINI_GAME/Rocky/minigame_claws_tree.minigame_claws_tree" (`self.Root`) "None" (0.0 0.0 0.0) "KeepRelativeOffset"))
          (set `self.Audio` _returnvalue_2))))))

(event `self.Box.OnComponentBeginOverlap`
  (params (OverlappedComponent :type "PrimitiveComponent Object Reference") (OtherActor :type "Actor Object Reference") (OtherComp :type "PrimitiveComponent Object Reference") (OtherBodyIndex :type Integer) (bFromSweep :type Boolean) (SweepResult :type "HitResult Structure (by ref)"))
  (bind _aspdwvehicle_pawn (cast `PDWVehiclePawn` OtherActor))
  (bind _aspdwplayer_interface (cast `PDWPlayerInterface` OtherActor))
  (if (`BlueprintGameplayTagLibrary.HasTag` (`BlueprintGameplayTagLibrary.GetOwnedGameplayTags` _aspdwvehicle_pawn) (struct :`TagName` "InteractionType.Minigame"))
    (set `self.Other Actor` OtherActor)
    (`PrimitiveComponent.SetSimulatePhysics` (`self.SM_Small_Trunk`) true)
    (bind _returnvalue (`PDWPlayerInterface.GetPDWPlayerState` _aspdwplayer_interface))
    (`PDWPlayerState.AddItem` _returnvalue (`self.In ID`) self)
    (bind _returnvalue_2 (`PDWPlayerInterface.GetInteractionComponent` _aspdwplayer_interface))
    (`PDWInteractionComponent.AddOwnerInteractionStates` _returnvalue_2 (`self.Gameplay Tags`))))

(event `self.Box.OnComponentEndOverlap`
  (params (OverlappedComponent :type "PrimitiveComponent Object Reference") (OtherActor :type "Actor Object Reference") (OtherComp :type "PrimitiveComponent Object Reference") (OtherBodyIndex :type Integer))
  (bind _in_id (`self.In ID`))
  (bind _other_actor (`self.Other Actor`))
  (if (== OtherActor _other_actor)
    (bind _aspdwvehicle_pawn (cast `PDWVehiclePawn` _other_actor))
    (bind _aspdwplayer_interface (cast `PDWPlayerInterface` (`self.Other Actor`)))
    (if (`BlueprintGameplayTagLibrary.HasTag` (`BlueprintGameplayTagLibrary.GetOwnedGameplayTags` _aspdwvehicle_pawn) (struct :`TagName` "InteractionType.Minigame"))
      (`PrimitiveComponent.SetSimulatePhysics` (`self.SM_Small_Trunk`) false)
      (bind _returnvalue (`PDWPlayerInterface.GetPDWPlayerState` _aspdwplayer_interface))
      (bind _returnvalue_2 (`PDWPlayerState.CheckItem` _returnvalue _in_id))
      (if _returnvalue_2
        (`PDWPlayerState.GetItem` _returnvalue _in_id))
      (bind _returnvalue_3 (`PDWPlayerInterface.GetInteractionComponent` _aspdwplayer_interface))
      (`PDWInteractionComponent.RemoveinteractionStates` _returnvalue_3 (`self.Gameplay Tags`)))))

(fn `UserConstructionScript`)