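; Static target actor for the Sea Rescue minigame that controls a water ripple effect based on its interaction state.
; Events from its interaction receiver component deactivate the ripple when the target becomes interactable or is successfully interacted with, and reactivate it when it stops being interactable.
; The Blueprint has no other active logic, as BeginPlay, overlap and Tick are disabled and construction only calls the parent.
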(event `self.BP_InteractionReceiverComponent.OnBecomeInteractable`
  (params (Component :type "PDWInteractionComponent Object Reference"))
  (`ActorComponent.SetActive` (`self.NS_MG_SeaRescue_Ripple`) false false :!label _label))

(event `self.BP_InteractionReceiverComponent.OnStopBeingInteractable`
  (params (Component :type "PDWInteractionComponent Object Reference"))
  (`ActorComponent.SetActive` (`self.NS_MG_SeaRescue_Ripple`) true false))

(event `self.BP_InteractionReceiverComponent.OnInteractionSuccessful`
  (params (Payload :type "PDWInteractionPayload Structure (by ref)"))
  (goto _label))

(fn `UserConstructionScript`
  (`parent.UserConstructionScript`))