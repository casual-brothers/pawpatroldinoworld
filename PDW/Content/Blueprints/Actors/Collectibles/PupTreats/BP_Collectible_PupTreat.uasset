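; Pup treat collectible actor that handles the visual and audio feedback when it is picked up.
; Pickup start speeds the bone treat's rotation through a dynamic material, then after a delay destroys both treat Niagara components, with a validity-gated color and flare update following the destroy.
; Pickup end spawns a collect burst and plays either a ghost treat sound if already taken or the normal pickup sound.
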(event `self.BP_PickUpEnd`
  (bind _returnvalue (`self.GetTransform`))
  (`NiagaraFunctionLibrary.SpawnSystemAtLocation` "/Game/Art/VFX/NiagaraSystem/Generic/NS_Collect_Treats.NS_Collect_Treats" (`self.K2_GetActorLocation`))
  (if (`self.AlreadyTaken`)
    (`FMODBlueprintStatics.PlayEventAtLocation` (`self.GhostTreat`) _returnvalue)
    (else
      (`FMODBlueprintStatics.PlayEventAtLocation` (`self.PickUpEvent`) _returnvalue))))

(event `self.PickUpComponent.OnPickUpStart`
  (params (Instigator :type "PDWPickUpComponent Object Reference") (PlayerController :type "PDWPlayerController Object Reference"))
  (bind _collectiblemeshcomponent (`self.CollectibleMeshComponent`))
  (bind _ns_puptreat (`self.NS_PupTreat`))
  (bind _returnvalue (`PrimitiveComponent.CreateDynamicMaterialInstance` _collectiblemeshcomponent 0 (`PrimitiveComponent.GetMaterial` _collectiblemeshcomponent (`PrimitiveComponent.GetMaterialIndex` _collectiblemeshcomponent "MI_BoneTreat_Rotating")) "MI_BoneTreat_Rotating"))
  (`MaterialInstanceDynamic.SetScalarParameterValueByInfo` _returnvalue (make `MaterialParameterInfo` "RotationAngleTimeMultiplier") 2.0)
  (`KismetSystemLibrary.Delay` 1.0)
  (`ActorComponent.K2_DestroyComponent` (`self.NS_PupTreat`))
  (`ActorComponent.K2_DestroyComponent` (`self.NS_PupTreat_Glow`))
  (`/Engine/EditorBlueprintResources/StandardMacros.IsValid` (`self.NS_PupTreat_Glow`)
    (:`Is Valid`
      (`NiagaraComponent.SetVariableVec3` _ns_puptreat "Color" (1.0 1.0 1.0))
      (`NiagaraComponent.SetVariableVec3` (`self.NS_PupTreat_Glow`) "Color" (1.0 1.0 1.0))
      (`NiagaraComponent.SetVariableBool` _ns_puptreat "UseFlare" false)
      (`NiagaraComponent.SetVariableBool` (`self.NS_PupTreat_Glow`) "UseFlare" false))))

(fn `UserConstructionScript`)