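; BP_Minigame_TimmyRun is the Blueprint for the Timmy Run minigame, handling its setup.
; On the PDWMinigameConfig initialization event, it finds the BP_Minigame_TimmyRun_Pawn in the level, stores it as Timmy and unhides it.
; BeginPlay, Tick and the construction script only call their parent versions, so this graph holds no gameplay logic beyond that reveal.
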(event `self.ReceiveBeginPlay`
  (`parent.ReceiveBeginPlay`))

(event `self.ReceiveTick`
  (params (DeltaSeconds :type "Float (single-precision)"))
  (`parent.ReceiveTick` DeltaSeconds))

(event `self.PDWMinigameConfig.OnMinigameInitialization`
  (bind _returnvalue (`GameplayStatics.GetActorOfClass` "/Game/Blueprints/Actors/MiniGames/EndlessRunner/BP_Minigame_TimmyRun_Pawn.BP_Minigame_TimmyRun_Pawn_C"))
  (bind _output_get (set `self.Timmy` _returnvalue))
  (`self.SetActorHiddenInGame` _output_get false))

(fn `UserConstructionScript`
  (`parent.UserConstructionScript`))