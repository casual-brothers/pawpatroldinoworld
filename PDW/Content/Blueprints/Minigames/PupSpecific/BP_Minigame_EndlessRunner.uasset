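; Endless runner minigame actor that ties its procedural content and balloon despawning to the minigame lifecycle.
; PCG generates when PDWMinigameConfig finishes initialization, and is cleaned up on begin play, completion or leaving, along with hiding P2Mesh.
; Leaving also resets obstacles.
; The BaloonDespawn volume hides actors whose overlapping component is tagged "Baloon", disables their collision and spawns a puff Niagara effect.
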(event OnMinigameInitializationComplete(PDWMinigameConfig)
  (params (Controllers :type Array%20of%20PDW%20Player%20Controller%20Object%20References))
  (PCG|Generate (Variables|Default|GetPCG) false))

(event OnMinigameComplete(PDWMinigameConfig)
  (params (inSignature :type Mini%20Game%20Event%20Signature%20Structure%20%28by%20ref%29))
  (Class|PCGComponent|Cleanup (Variables|Default|GetPCG) true)
  (Rendering|SetVisibility (Variables|Default|GetP2Mesh) false true))

(event OnMinigameLeft(PDWMinigameConfig)
  (params (inSignature :type Mini%20Game%20Event%20Signature%20Structure%20%28by%20ref%29))
  (Class|PDWSplineActor|ResetObstacles)
  (Class|PCGComponent|Cleanup (Variables|Default|GetPCG) true)
  (Rendering|SetVisibility (Variables|Default|GetP2Mesh) false true))

(event OnComponentBeginOverlap(BaloonDespawn)
  (params (OverlappedComponent :type Primitive%20Component%20Object%20Reference) (OtherActor :type Actor%20Object%20Reference) (OtherComp :type Primitive%20Component%20Object%20Reference) (OtherBodyIndex :type Integer) (bFromSweep :type Boolean) (SweepResult :type Hit%20Result%20Structure%20%28by%20ref%29))
  (if (Components|ComponentHasTag OtherComp "Baloon")
    (Rendering|SetActorHiddenInGame OtherActor true)
    (Collision|SetActorEnableCollision OtherActor false)
    (Niagara|SpawnSystematLocation "/Game/Art/VFX/NiagaraSystem/MiniGame/NS_MG_Zuma_Puff.NS_MG_Zuma_Puff" (Transformation|GetWorldLocation OtherComp))))

(event EventBeginPlay
  (Class|PCGComponent|Cleanup (Variables|Default|GetPCG) true)
  (Rendering|SetVisibility (Variables|Default|GetP2Mesh) false true))

(event Collision|EventActorBeginOverlap
  (params (OtherActor :type Actor%20Object%20Reference)))

(event EventTick
  (params (DeltaSeconds :type Float%20%28single-precision%29)))

(fn ConstructionScript)