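; Grappling hook minigame Blueprint that highlights the minigame's target actors while it runs.
; When the minigame config finishes initializing, it turns on custom depth rendering for static meshes tagged "RenderTarget" on each target actor, and turns it off on completion or leave.
; IsTarget extends the parent check by rejecting actors whose targeting component marks them as fake targets.
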(event `self.PDWMinigameConfig.OnMinigameComplete`
  (params (inSignature :type "MiniGameEventSignature Structure (by ref)"))
  (`self.SetTargetRenderCustomDepthPass` false :!label _label))

(event `self.PDWMinigameConfig.OnMinigameLeft`
  (params (inSignature :type "MiniGameEventSignature Structure (by ref)"))
  (goto _label))

(event `self.PDWMinigameConfig.OnMinigameInitializationComplete`
  (params (Controllers :type "Array of PDWPlayerController Object Reference (by ref)"))
  (`self.SetTargetRenderCustomDepthPass` true))

(fn `IsTarget`
  (params (Target :type "Actor Object Reference (by ref)"))
  (returns (CanAdd :type Boolean))
  (return (and (not (`PDWTargetingComponent.IsFakeTarget` (`self.GetComponentByClass` Target "/Script/PDW.PDWTargetingComponent"))) (`parent.IsTarget` null))))

(fn `SetTargetRenderCustomDepthPass`
  (params (RenderCustomDepthPass :type Boolean))
  (for _array_element (`PDWMinigameConfigComponent.MinigameTargetActors` (`self.PDWMinigameConfig`))
    (`/Engine/EditorBlueprintResources/StandardMacros.IsValid` _array_element
      (:`Is Valid`
        (for _array_element_2 (`self.GetComponentsByTag` _array_element "/Script/Engine.StaticMeshComponent" "RenderTarget")
          (`/Engine/EditorBlueprintResources/StandardMacros.IsValid` _array_element_2
            (:`Is Valid`
              (`PrimitiveComponent.SetRenderCustomDepth` _array_element_2 RenderCustomDepthPass))))))))

(fn `UserConstructionScript`
  (`parent.UserConstructionScript`))