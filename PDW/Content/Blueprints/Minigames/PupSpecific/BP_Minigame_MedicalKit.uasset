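; BP_Minigame_MedicalKit is a pup-specific minigame Blueprint that scatters medical kit targets over a skeletal mesh.
; On each multiplayer state change, it takes the mesh from SkeletonActor and gathers sockets whose names match SocketPrefix.
; It then destroys old targets, spawns the configured quantity, and initializes and attaches each at a random socket, removing used sockets to avoid repeats.
; ActivateTargets is an empty stub.
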(event `self.ReceiveBeginPlay`
  (`parent.ReceiveBeginPlay`))

(event `self.OnMultiplayerStateChange`
  (`parent.OnMultiplayerStateChange`)
  (`self.InitializeTargets`))

(fn `ActivateTargets`)

(fn `CreateTargets`
  (locals (CurrentIndex :type Integer))
  (bind _minigametargetactors (`PDWMinigameConfigComponent.MinigameTargetActors` (`self.PDWMinigameConfig`)))
  (for _array_element _minigametargetactors
    (`/Engine/EditorBlueprintResources/StandardMacros.IsValid` _array_element
      (:`Is Valid`
        (`self.K2_DestroyActor` _array_element))))
  (`KismetArrayLibrary.Array_Clear` _minigametargetactors)
  (for _ (range (`self.GetTargetQuantityValue`))
    (bind _output_get (set `local.CurrentIndex` (`KismetMathLibrary.RandomIntegerInRange` 0 (- (`KismetArrayLibrary.Array_Length` (`self.AvailableSocket`)) 1))))
    (bind _returnvalue (`|SpawnActorFromClass` (`self.MedicalKit_Target_Class`) (`self.GetTransform` self) "Undefined" "MultiplyWithRoot" self null))
    (bind _output (`|GetArrayItem` (`self.AvailableSocket`) _output_get))
    (`/Game/Blueprints/Actors/MiniGames/MedicalKit/BP_Minigame_MedicalKit_Target.InitializeMesh` _returnvalue _output)
    (`self.K2_AttachToComponent` _returnvalue (`self.SkeletonMesh`) _output "SnapToTarget" "SnapToTarget" "SnapToTarget" true)
    (`KismetArrayLibrary.Array_AddUnique` (`PDWMinigameConfigComponent.MinigameTargetActors` (`self.PDWMinigameConfig`)) _returnvalue)
    (`KismetArrayLibrary.Array_Remove` (`self.AvailableSocket`) (`local.CurrentIndex`))))

(fn `GetSocketList`
  (`KismetArrayLibrary.Array_Clear` (`self.SocketList`))
  (for _index (range (`SkeletalMesh.NumSockets` (`SkeletalMeshComponent.SkeletalMeshAsset` (`self.SkeletonMesh`))))
    (bind _socketname (`SkeletalMeshSocket.SocketName` (`SkeletalMesh.GetSocketByIndex` (`SkeletalMeshComponent.SkeletalMeshAsset` (`self.SkeletonMesh`)) _index)))
    (if (`KismetStringLibrary.StartsWith` (`KismetStringLibrary.Conv_NameToString` _socketname) (`self.SocketPrefix`))
      (`KismetArrayLibrary.Array_Add` (`self.SocketList`) _socketname)))
  (set `self.AvailableSocket` (`self.SocketList`)))

(fn `InitializeTargets`
  (bind _skeletonactor (`self.SkeletonActor`))
  (`/Engine/EditorBlueprintResources/StandardMacros.IsValid` _skeletonactor
    (:`Is Valid`
      (bind _output_get (set `self.SkeletonMesh` (`self.GetComponentByClass` _skeletonactor "/Script/Engine.SkeletalMeshComponent")))
      (`/Engine/EditorBlueprintResources/StandardMacros.IsValid` _output_get
        (:`Is Valid`
          (`self.GetSocketList`)
          (`self.CreateTargets`))))))

(fn `UserConstructionScript`
  (`parent.UserConstructionScript`))