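; Pup-specific drill excavation minigame Blueprint with a moving mesh for each of two players, extending a parent minigame class.
; An animation request plays the drill animation on the requesting player's skeletal mesh unless it is already playing.
; Each moving mesh is shown only while its owning controller is active.
; AddTarget passes DrillExcavation goals to the parent and collects all other targets uniquely in RockList.
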(event `self.ReceiveBeginPlay`
  (`parent.ReceiveBeginPlay`)
  (add `self.OnAnimationRequest` (delegate `OnAnimationRequest_Event`)))

(event `OnAnimationRequest_Event` :!signature `self.OnAnimationRequest`
  (params (PlayerController :type "PDWPlayerController Object Reference"))
  (bind _skeletalmeshp1 (`self.SkeletalMeshP1`))
  (bind _skeletalmeshp2 (`self.SkeletalMeshP2`))
  (if (== PlayerController (`PDWMinigameMovingMesh.ControllerOwner` (`self.MovingMeshP1`)))
    (if (not (`SkeletalMeshComponent.IsPlaying` _skeletalmeshp1))
      (`SkeletalMeshComponent.PlayAnimation` _skeletalmeshp1 "/Game/Art/Characters/CH_04_Rubble/Animation/Backpack_Skill/AM_CH_04_Minigame_DrillExcavation.AM_CH_04_Minigame_DrillExcavation" false))
    (elif (== PlayerController (`PDWMinigameMovingMesh.ControllerOwner` (`self.MovingMeshP2`)))
      (if (not (`SkeletalMeshComponent.IsPlaying` _skeletalmeshp2))
        (`SkeletalMeshComponent.PlayAnimation` _skeletalmeshp2 "/Game/Art/Characters/CH_04_Rubble/Animation/Backpack_Skill/AM_CH_04_Minigame_DrillExcavation.AM_CH_04_Minigame_DrillExcavation" false)))))

(fn `ActivateTargets`
  (`parent.ActivateTargets`))

(fn `AddTarget`
  (params (Target :type "Actor Object Reference (by ref)"))
  (cast `/Game/Blueprints/Actors/MiniGames/DrillExcavation/BP_Minigame_DrillExcavation_Goal` Target
    (:`then`
      (`parent.AddTarget` Target))
    (:`CastFailed`
      (`KismetArrayLibrary.Array_AddUnique` (`self.RockList`) Target)))
  (return))

(fn `ShowMovingMesh`
  (params (ActiveControllers :type "Array of PDWPlayerController Object Reference (by ref)") (MovingMesh :type "PDWMinigameMovingMesh Object Reference"))
  (`SceneComponent.SetHiddenInGame` MovingMesh (== (`KismetArrayLibrary.Array_Find` ActiveControllers (`PDWMinigameMovingMesh.ControllerOwner` MovingMesh)) -1) true))

(fn `UserConstructionScript`
  (`parent.UserConstructionScript`))