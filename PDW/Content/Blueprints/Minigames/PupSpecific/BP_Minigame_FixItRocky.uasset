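; Rocky's Fix-It minigame Blueprint, a pup-specific puzzle built on puzzle piece components.
; On minigame initialization it gives each of its puzzle piece components a random yaw in quarter-turn steps.
; It listens to the PDW event subsystem and spawns a Niagara success effect at a piece whenever its possess event reports false.
; Target deactivation only prints the deactivating actor's name.
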(event `self.ReceiveBeginPlay`
  (bind _returnvalue (subsystem `PDWEventSubsytem`))
  (`parent.ReceiveBeginPlay`)
  (add `PDWEventSubsytem.OnTargetDeactivation` _returnvalue (delegate `OnTargetDeactivation_FixItRocky`))
  (add `PDWEventSubsytem.OnPuzzlePosses` _returnvalue (delegate `OnPuzzlePosses_Event`)))

(event `OnTargetDeactivation_FixItRocky`
  (params (DeactivatingActor :type "Actor Object Reference"))
  (`KismetSystemLibrary.PrintString` (`KismetSystemLibrary.GetDisplayName` DeactivatingActor)))

(event `OnPuzzlePosses_Event`
  (params (bPosses :type Boolean) (PuzzlePiece :type "SceneComponent Object Reference"))
  (if (not bPosses)
    (`NiagaraFunctionLibrary.SpawnSystemAtLocation` "/Game/Art/VFX/NiagaraSystem/Interactables/NS_MG_Fix-it_Success.NS_MG_Fix-it_Success" (+ (`SceneComponent.K2_GetComponentLocation` PuzzlePiece) (0.0 0.0 0.0)))))

(event `self.PDWMinigameConfig.OnMinigameInitialization`
  (for _array_element (`self.K2_GetComponentsByClass` self "/Script/PDW.PDWPuzzlePieceComponent")
    (`SceneComponent.K2_SetRelativeRotation` _array_element (`KismetMathLibrary.MakeRotator` 0.0 0.0 (* (`KismetMathLibrary.RandomIntegerInRange` 0 3) 90.0)) false false)))

(fn `UserConstructionScript`
  (`parent.UserConstructionScript`))