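; Base minigame actor that manages targets, quest highlight and optional vehicle resizing around a PDW minigame config.
; It overrides the success objective's target quantity for single or multiplayer, falling back to the configured default.
; It enables a random subset of deployable targets, always including any main target, and rerolls on multiplayer state changes.
; After initialization it can rescale players' vehicles, meshes and suspensions, restoring them on completion or leaving.
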(event `self.ReceiveBeginPlay`
  (bind _pdwminigameconfig (`self.PDWMinigameConfig`))
  (add `PDWMinigameConfigComponent.OnMinigameInitialization` _pdwminigameconfig (delegate `HideHighlight`))
  (add `PDWMinigameConfigComponent.OnMinigameComplete` _pdwminigameconfig (delegate `ShowHighlight`))
  (add `PDWMinigameConfigComponent.OnMinigameLeft` _pdwminigameconfig (delegate `Reactivatehighlight`))
  (`self.InitializeDefaultTargetQuantity`)
  (`self.OverrideTargetQuantity`)
  (add `PDWEventSubsytem.OnMultiplayerStateChange` (subsystem `PDWEventSubsytem`) (delegate `OnMultiplayerStateChange`))
  (`self.InitializeTargets`)
  (`self.ActivateTargets`))

(event `Reactivatehighlight`
  (params (inSignature :type "MiniGameEventSignature Structure (by ref)"))
  (`SceneComponent.SetHiddenInGame` (`self.TargetQuestHighlight`) false false))

(event `HideHighlight`
  (`SceneComponent.SetHiddenInGame` (`self.TargetQuestHighlight`) true false))

(event `OnMultiplayerStateChange`
  (`self.OverrideTargetQuantity`)
  (`self.ActivateTargets`))

(event `ShowHighlight`
  (params (inSignature :type "MiniGameEventSignature Structure (by ref)"))
  ; verificare, non dovrebbe riaccendersi
  (`SceneComponent.SetHiddenInGame` (`self.TargetQuestHighlight`) false false))

(event `self.PDWMinigameConfig.OnMinigameComplete`
  (params (inSignature :type "MiniGameEventSignature Structure (by ref)"))
  (if (!= (`self.VehicleScale`) (0.0 0.0 0.0)) :!label _label
    (`self.ResetVehicle` (`PDWGameplayFunctionLibrary.GetPlayerControllerOne`))
    (if (`PDWGameplayFunctionLibrary.IsMultiplayerOn`)
      (`self.ResetVehicle` (`PDWGameplayFunctionLibrary.GetPlayerControllerTwo`)))))

(event `self.PDWMinigameConfig.OnMinigameLeft`
  (params (inSignature :type "MiniGameEventSignature Structure (by ref)"))
  (goto _label))

(event `self.PDWMinigameConfig.OnMinigameInitializationComplete`
  (params (Controllers :type "Array of PDWPlayerController Object Reference (by ref)"))
  (if (!= (`self.VehicleScale`) (0.0 0.0 0.0))
    (`BlueprintMapLibrary.Map_Clear` (`self.Relative Location`))
    (`KismetSystemLibrary.K2_SetTimerDelegate` (delegate `CustomEvent`) 0.2)))

(event `CustomEvent`
  (bind _returnvalue (`PDWGameplayFunctionLibrary.GetPlayerControllerOne`))
  (bind _returnvalue_2 (`PDWGameplayFunctionLibrary.GetPlayerControllerTwo`))
  (bind _vehiclescale (`self.VehicleScale`))
  (`self.SaveLocation` _returnvalue)
  (`self.ResizeVehicle` _returnvalue _vehiclescale (`self.NewSkeletalRelativeLocation`))
  (if (`PDWGameplayFunctionLibrary.IsMultiplayerOn`)
    (`self.SaveLocation` _returnvalue_2)
    (`self.ResizeVehicle` _returnvalue_2 _vehiclescale (`self.NewSkeletalRelativeLocation`))))

(fn `ActivateTargets`
  (locals (TempTargetList :type "Array of Actor Object Reference") (CurrentIndex :type Integer :default 0))
  (bind _returnvalue (`self.GetTargetQuantityValue`))
  (bind _maintarget (`self.MainTarget`))
  (`self.DeactivateTargets`)
  (set `local.TempTargetList` (`self.TargetList`))
  (if (`self.HasMainTarget`)
    (`self.SetActorHiddenInGame` _maintarget false)
    (`self.SetActorEnableCollision` _maintarget true)
    (`KismetArrayLibrary.Array_RemoveItem` (`local.TempTargetList`) _maintarget))
  (for _ (range (+ (`KismetMathLibrary.SelectInt` (- _returnvalue 2) (- _returnvalue 1) (`self.HasMainTarget`)) 1))
    (bind _output_get (set `local.CurrentIndex` (`KismetMathLibrary.RandomIntegerInRange` 0 (- (`KismetArrayLibrary.Array_Length` (`local.TempTargetList`)) 1))))
    (bind _output (`|GetArrayItem` (`local.TempTargetList`) _output_get))
    (`/Engine/EditorBlueprintResources/StandardMacros.IsValid` _output
      (:`Is Valid`
        (`self.SetActorHiddenInGame` _output false)
        (`self.SetActorEnableCollision` _output true)
        (`KismetArrayLibrary.Array_Remove` (`local.TempTargetList`) (`local.CurrentIndex`))))))

(fn `AddTarget`
  (params (Target :type "Actor Object Reference (by ref)"))
  (`KismetArrayLibrary.Array_AddUnique` (`self.TargetList`) Target))

(fn `DeactivateTargets`
  (for _array_element (`self.TargetList`)
    (`self.SetActorHiddenInGame` _array_element true)
    (`self.SetActorEnableCollision` _array_element false)))

(fn `GetTargetQuantityValue`
  (returns (ReturnValue :type Byte))
  (bind _returnvalue (select `bool` (`PDWGameplayFunctionLibrary.IsMultiplayerOn`) :`false` (`self.SingleplayerTargetQuantity`) :`true` (`self.MultiplayerTargetQuantity`)))
  (return (select `bool` (> _returnvalue 0) :`false` (`self.DefaultTargetQuantity`) :`true` _returnvalue)))

(fn `HasMainTarget`
  (returns (ReturnValue :type Boolean))
  (return (`KismetSystemLibrary.IsValid` (`self.MainTarget`))))

(fn `InitializeDefaultTargetQuantity`
  (bind _returnvalue (`PDWMinigameConfigComponent.GetMinigameConfigurationData` (`self.PDWMinigameConfig`)))
  (set `self.DefaultTargetQuantity` (`PDWQuantityConditionCheck.TargetQuantity` (`BlueprintMapLibrary.Map_Find` (`PDWMinigameConfigData.MiniGameObjectiveConfig` _returnvalue) (`self.MinigameSuccessGameplayTag`)))))

(fn `InitializeTargets`
  (for _array_element (`PDWMinigameConfigComponent.MinigameTargetActors` (`self.PDWMinigameConfig`))
    (if (`self.IsTarget` _array_element)
      (`self.AddTarget` _array_element)))
  (if (`self.HasMainTarget`)
    (`KismetArrayLibrary.Array_AddUnique` (`self.TargetList`) (`self.MainTarget`))))

(fn `IsTarget`
  (params (Target :type "Actor Object Reference (by ref)"))
  (returns (CanAdd :type Boolean))
  (`/Engine/EditorBlueprintResources/StandardMacros.IsValid` Target
    (:`Is Valid`
      (return (`KismetSystemLibrary.IsValid` (`self.GetComponentByClass` Target "/Script/PDW.PDWDeployableComponent"))))
    (:`Is Not Valid`
      (return false))))

(fn `OverrideTargetQuantity`
  (bind _returnvalue (`PDWMinigameConfigComponent.GetMinigameConfigurationData` (`self.PDWMinigameConfig`)))
  (set `PDWQuantityConditionCheck.TargetQuantity` (`self.GetTargetQuantityValue`) (`BlueprintMapLibrary.Map_Find` (`PDWMinigameConfigData.MiniGameObjectiveConfig` _returnvalue) (`self.MinigameSuccessGameplayTag`))))

(fn `ResetVehicle`
  (params (`Player Controller` :type "PDWPlayerController Object Reference"))
  (bind _returnvalue (`PDWPlayerController.GetVehicleInstance` `Player Controller`))
  (`self.ResizeVehicle` `Player Controller` (1.0 1.0 1.0) (`BlueprintMapLibrary.Map_Find` (`self.Relative Location`) (`|GetArrayItem` (`self.GetComponentsByTag` _returnvalue "/Script/Engine.SkeletalMeshComponent" "ComponentTag.VehicleMesh"))))
  (`PDWVehiclePawn.ResetSuspensionsLenght` _returnvalue))

(fn `ResizeVehicle`
  (params (`Player Controller` :type "PDWPlayerController Object Reference") (NewScale :type "Vector Structure") (NewRelativeLocation :type "Vector Structure"))
  (bind _returnvalue (`PDWPlayerController.GetVehicleInstance` `Player Controller`))
  (`SceneComponent.SetWorldScale3D` (`Actor.RootComponent` _returnvalue) NewScale)
  (`SceneComponent.K2_SetRelativeLocation` (`|GetArrayItem` (`self.GetComponentsByTag` _returnvalue "/Script/Engine.SkeletalMeshComponent" "ComponentTag.VehicleMesh")) NewRelativeLocation false false)
  (`PDWVehiclePawn.OverrideSuspensionsLenght` _returnvalue (* (`PDWVehiclePawn.GetSuspensionsLenght` _returnvalue) (.z NewScale))))

(fn `SaveLocation`
  (params (`Player Controller` :type "PDWPlayerController Object Reference"))
  (bind _returnvalue (`PDWPlayerController.GetVehicleInstance` `Player Controller`))
  (bind _output (`|GetArrayItem` (`self.GetComponentsByTag` _returnvalue "/Script/Engine.SkeletalMeshComponent" "ComponentTag.VehicleMesh")))
  (`BlueprintMapLibrary.Map_Add` (`self.Relative Location`) _output (`SceneComponent.RelativeLocation` _output)))

(fn `UserConstructionScript`)