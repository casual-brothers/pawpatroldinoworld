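; Dino nest minigame actor that displays its collected egg count and marks itself as a quest target.
; Egg-collected events from the nest handler drive a Quantity parameter on the nest's dynamic material.
; Quest-target tag changes on PDWTag activate or deactivate the highlight, with the initial state checked on BeginPlay.
; The nest-full event unhides that highlight.
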(event `self.ReceiveBeginPlay`
  (bind _returnvalue (`QuestSettings.GetQuestTargetTag`))
  (bind _nest (`self.Nest`))
  (bind _material_slot_name (`self.Material Slot Name`))
  (bind _pdwtag (`self.PDWTag`))
  (bind _returnvalue_2 (`PrimitiveComponent.CreateDynamicMaterialInstance` (`self.Nest`) (`PrimitiveComponent.GetMaterialIndex` _nest _material_slot_name) (`PrimitiveComponent.GetMaterialByName` _nest _material_slot_name) "None"))
  (set `self.Nest MID` _returnvalue_2)
  (add `PDWTagComponent.OnPDWTagAdded` _pdwtag (delegate `ShowQuestIcon`))
  (add `PDWTagComponent.OnPDWTagRemoved` _pdwtag (delegate `HideQuestIcon`))
  (if (`BlueprintGameplayTagLibrary.HasTag` (`PDWTagComponent.TagContainer` _pdwtag) _returnvalue)
    (`self.ShowQuestIcon` (struct) _returnvalue)
    (else
      (`self.HideQuestIcon` (struct) _returnvalue))))

(event `ShowQuestIcon`
  (params (UpdatedContainer :type "GameplayTagContainer Structure (by ref)") (NewTagAdded :type "GameplayTag Structure (by ref)"))
  (if (`BlueprintGameplayTagLibrary.MatchesTag` NewTagAdded (`QuestSettings.GetQuestTargetTag`))
    (`ActorComponent.Activate` (`self.TargetQuestHighlight`) true)))

(event `self.PDWDinoNestHandler.OnNestEggCollected`
  (params (TotalEggs :type Integer))
  (bind _output_get (set `self.Total Eggs` TotalEggs))
  (`self.DrawEggCount` _output_get))

(event `HideQuestIcon`
  (params (UpdatedContainer :type "GameplayTagContainer Structure (by ref)") (TagRemoved :type "GameplayTag Structure (by ref)"))
  (if (`BlueprintGameplayTagLibrary.MatchesTag` TagRemoved (`QuestSettings.GetQuestTargetTag`))
    (`ActorComponent.Deactivate` (`self.TargetQuestHighlight`))))

(event `DrawEggCount`
  (params (`Total Eggs` :type Integer))
  (`MaterialInstanceDynamic.SetScalarParameterValue` (`self.Nest MID`) "Quantity" (* `Total Eggs` 0.2)))

(event `self.ReceiveEndPlay`
  (params (EndPlayReason :type "EEndPlayReason Enum" :default "Destroyed"))
  (bind _pdwtag (`self.PDWTag`))
  (remove `PDWTagComponent.OnPDWTagAdded` _pdwtag (delegate `ShowQuestIcon`))
  (remove `PDWTagComponent.OnPDWTagRemoved` _pdwtag (delegate `HideQuestIcon`)))

(event `self.PDWDinoNestHandler.OnNestFull`
  (params (Source :type "Actor Object Reference"))
  (`SceneComponent.SetHiddenInGame` (`self.TargetQuestHighlight`) false false))

(fn `UserConstructionScript`)