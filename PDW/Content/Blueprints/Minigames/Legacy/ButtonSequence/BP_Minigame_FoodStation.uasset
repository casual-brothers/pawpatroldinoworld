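; Food station actor in the legacy ButtonSequence minigame folder that registers as a Smart Object while it holds food.
; Its food station handler drives Smart Object registration; the use event processes an interaction for the user, empties the food and hides the mesh.
; Quest-target tag changes toggle a highlight and set the interaction receiver's active or inactive state.
; The minigame completion handler is empty.
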(event `self.PDWFoodStationHandler.OnInit`
  (`self.HandleSmartObjectActivity`))

(event `self.ReceiveBeginPlay`
  (bind _returnvalue (`QuestSettings.GetQuestTargetTag`))
  (bind _pdwtag (`self.PDWTag`))
  (`parent.ReceiveBeginPlay`)
  (add `SmartObjectComponent.OnSmartObjectEvent` (`self.SmartObject`) (delegate `OnSOEvent`))
  (add `PDWFoodStationHandler.OnSmartObjectUpdate` (`self.PDWFoodStationHandler`) (delegate `OnSOUpdate`))
  (`self.HandleSmartObjectActivity`)
  (add `PDWTagComponent.OnPDWTagAdded` _pdwtag (delegate `ActivateInteraction`))
  (add `PDWTagComponent.OnPDWTagRemoved` _pdwtag (delegate `RemoveInteraction`))
  (if (`BlueprintGameplayTagLibrary.HasTag` (`PDWTagComponent.TagContainer` _pdwtag) _returnvalue)
    (`self.ActivateInteraction` (struct) _returnvalue)
    (else
      (`self.RemoveInteraction` (struct) _returnvalue))))

(event `OnSOUpdate`
  (params (IsActive :type Boolean))
  (`SmartObjectBlueprintFunctionLibrary.AddOrRemoveSmartObject` self IsActive)
  (`SceneComponent.SetVisibility` (`self.FoodMesh`) true false))

(event `ActivateInteraction`
  (params (UpdatedContainer :type "GameplayTagContainer Structure (by ref)") (NewTagAdded :type "GameplayTag Structure (by ref)"))
  (if (`BlueprintGameplayTagLibrary.MatchesTag` NewTagAdded (`QuestSettings.GetQuestTargetTag`))
    (`ActorComponent.Activate` (`self.TargetQuestHighlight`) true)
    (`PDWInteractionReceiverComponent.AddStateTag` (`self.InteractionReceiver`) (`self.ActiveTag`))))

(event `OnSOEvent`
  (params (EventData :type "SmartObjectEventData Structure (by ref)") (Interactor :type "Actor Object Reference"))
  (switch `ESmartObjectChangeReason` EventData_Reason
    (:`OnEvent`
      (if (== (`PDWGameplayTagSettings.GetSOUseEvent`) EventData_Tag)
        (`PDWInteractionReceiverComponent.ProcessInteraction` (`self.InteractionReceiver`) (make `PDWInteractionPayload` Interactor (struct) (`BlueprintGameplayTagLibrary.MakeGameplayTagContainerFromArray` (`|MakeArray` (`self.Behaviour Identifier`)))))
        (`PDWFoodStationHandler.SetCurrentStationFood` (`self.PDWFoodStationHandler`) 0.0)
        (`SceneComponent.SetVisibility` (`self.FoodMesh`) false false)))
    (:`OnReleased`
      (`self.HandleSmartObjectActivity`))))

(event `RemoveInteraction`
  (params (UpdatedContainer :type "GameplayTagContainer Structure (by ref)") (TagRemoved :type "GameplayTag Structure (by ref)"))
  (if (`BlueprintGameplayTagLibrary.MatchesTag` TagRemoved (`QuestSettings.GetQuestTargetTag`))
    (`ActorComponent.Deactivate` (`self.TargetQuestHighlight`))
    (`PDWInteractionReceiverComponent.AddStateTag` (`self.InteractionReceiver`) (`self.InactiveTag`))))

(event `self.ReceiveEndPlay`
  (params (EndPlayReason :type "EEndPlayReason Enum" :default "Destroyed"))
  (bind _pdwtag (`self.PDWTag`))
  (remove `PDWTagComponent.OnPDWTagAdded` _pdwtag (delegate `ActivateInteraction`))
  (remove `PDWTagComponent.OnPDWTagRemoved` _pdwtag (delegate `RemoveInteraction`)))

(event `HandleSmartObjectActivity`
  (`SmartObjectBlueprintFunctionLibrary.AddOrRemoveSmartObject` self (not (<= (`PDWFoodStationHandler.GetCurrentStationFood` (`self.PDWFoodStationHandler`)) 0))))

(fn `HandleMinigameCompleted`)

(fn `UserConstructionScript`
  (`parent.UserConstructionScript`))