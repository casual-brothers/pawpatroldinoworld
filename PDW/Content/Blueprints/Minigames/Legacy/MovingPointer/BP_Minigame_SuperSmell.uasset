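; Super Smell minigame Blueprint, in which characters sniff out clues for a smell target shown on the HUD.
; On start, it slows characters into a sniff animation and reveals targets in random order as right or capped-chance wrong clues, optionally hinted.
; NextStep scales the clue Niagara effect with progress and reveals the clue mesh at the target count.
; Completing or leaving restores characters and deactivates targets, which can come from actor spawners.
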(event `self.ReceiveBeginPlay`
  (`parent.ReceiveBeginPlay`))

(event `self.PDWMinigameConfig.OnMinigameComplete`
  (params (inSignature :type "MiniGameEventSignature Structure (by ref)"))
  (`self.ResetCharacterSpeedAndAnimation` :!label _label)
  (`self.DeactivateTargets`)
  (set `self.CurrentStep` 0))

(event `self.PDWMinigameConfig.OnMinigameLeft`
  (params (inSignature :type "MiniGameEventSignature Structure (by ref)"))
  (goto _label))

(event `self.PDWMinigameConfig.OnMinigameInitializationComplete`
  (params (Controllers :type "Array of PDWPlayerController Object Reference (by ref)"))
  (bind _returnvalue (`PDWMinigameConfigComponent.GetMinigameFlowComponent` (`self.PDWMinigameConfig`)))
  (`PDWHUDSubsystem.ShowSmellTarget` (subsystem `PDWHUDSubsystem`) (`FlowComponent.IdentityTags` _returnvalue))
  (`self.ActivateClues`)
  (`KismetSystemLibrary.Delay` 0.5)
  (`self.SetCharacterSpeedAndAnimation` Controllers))

(event `self.BP_OnHintTriggered`
  (set `self.HintRequested` true))

(fn `ActivateClues`
  (locals (CurrentIndex :type Integer) (WrongClueBehaviour :type "GameplayTag Structure" :default (struct :`TagName` "InteractionBehaviour.EmptyingStart")) (RightClueBehaviour :type "GameplayTag Structure" :default (struct :`TagName` "InteractionBehaviour.FillingStart")) (LastIndex :type Integer) (WrongCluesMax :type Integer) (TempTargetActors :type "Array of Actor Object Reference"))
  (bind _wrongcluebehaviour (`local.WrongClueBehaviour`))
  (bind _returnvalue (`KismetArrayLibrary.Array_Length` (`local.TempTargetActors`)))
  (bind _output (`|GetArrayItem` (`local.TempTargetActors`) (`local.CurrentIndex`)))
  (bind _returnvalue_2 (`self.GetComponentByClass` _output "/Script/PDW.PDWInteractionReceiverComponent"))
  (bind _output_2 (`|GetArrayItem` (`self.GetComponentsByTag` _output "/Script/Engine.SceneComponent" (`self.SceneComponentTag`))))
  (bind _returnvalue_3 (select `bool` (or (> (`KismetMathLibrary.RandomFloat`) (`self.WrongClueChance`)) (<= (`local.WrongCluesMax`) 0)) :`false` _wrongcluebehaviour :`true` (`local.RightClueBehaviour`)))
  (set `local.TempTargetActors` (`self.TargetList`))
  (set `local.LastIndex` (- _returnvalue 1))
  (set `local.WrongCluesMax` (`KismetMathLibrary.Min` (- _returnvalue (`self.GetTargetQuantityValue`)) (/ _returnvalue 2)))
  (for _ (range (+ (`local.LastIndex`) 1))
    (set `local.CurrentIndex` (`KismetMathLibrary.RandomIntegerInRange` 0 (- _returnvalue 1)))
    (if (`self.HintRequested`)
      (bind _returnvalue_4 (`PDWMinigameConfigComponent.GetMinigameConfigurationData` (`self.PDWMinigameConfig`)))
      (`PDWEventSubsytem.OnShowHintEvent` (subsystem `PDWEventSubsytem`) _output_2 (`PDWMinigameConfigData.MiniGameIdentifierTag` _returnvalue_4)))
    (`SceneComponent.SetHiddenInGame` _output_2 false true)
    (`PrimitiveComponent.SetCollisionEnabled` _returnvalue_2 "QueryOnly")
    (if (== _wrongcluebehaviour _returnvalue_3)
      (`/Engine/EditorBlueprintResources/StandardMacros.DecrementInt` (`local.WrongCluesMax`)
        (:`  `
          _)))
    (`PDWInteractionReceiverComponent.ExecuteInteractionBehaviour` _returnvalue_2 _returnvalue_3 self false false)
    (`KismetArrayLibrary.Array_Remove` (`local.TempTargetActors`) (`local.CurrentIndex`)))
  (if (`self.HintRequested`)
    (set `self.HintRequested` false))
  (return))

(fn `ActivateTargets`)

(fn `AddTarget`
  (params (Target :type "Actor Object Reference (by ref)"))
  (bind _asnebula_tool_moving_actors_spawner (cast `NebulaToolMovingActorsSpawner` Target)
    (:`then`
      (for _array_element (`NebulaToolMovingActorsSpawner.GetSpawnedActorList` _asnebula_tool_moving_actors_spawner)
        (`parent.AddTarget` _array_element)))
    (:`CastFailed`
      (`parent.AddTarget` Target)))
  (return))

(fn `CurrentStepValue`
  (params (Value :type "Float (double-precision)" :default 0.0))
  (returns (ReturnValue :type "Float (double-precision)"))
  (return (* (/ Value (`self.GetTargetQuantityValue`)) (`self.CurrentStep`))))

(fn `DeactivateTargets`
  (for _array_element (`self.TargetList`)
    (`PDWEventSubsytem.OnTargetDeactivationEvent` (subsystem `PDWEventSubsytem`) _array_element)
    (`SceneComponent.SetHiddenInGame` (`self.GetComponentsByTag` _array_element "/Script/Engine.SceneComponent" (`self.SceneComponentTag`)) true true)
    (`PrimitiveComponent.SetCollisionEnabled` (`self.GetComponentByClass` "/Script/PDW.PDWInteractionReceiverComponent") "NoCollision"))
  (return))

(fn `IsTarget`
  (params (Target :type "Actor Object Reference (by ref)"))
  (returns (CanAdd :type Boolean))
  (if (not (`parent.IsTarget` null))
    (cast `NebulaToolMovingActorsSpawner` Target
      (:`then`
        _)
      (:`CastFailed`
        (return true))))
  (return true))

(fn `NextStep`
  (bind _clueniagara (`self.ClueNiagara`))
  (`/Engine/EditorBlueprintResources/StandardMacros.IncrementInt` (`self.CurrentStep`)
    (:`  `
      (`ActorComponent.SetActive` _clueniagara true false)
      (`NiagaraComponent.SetVariableFloat` _clueniagara "Dissolve" (`self.CurrentStepValue` (`self.Dissolve`)))
      (`NiagaraComponent.SetVariableFloat` _clueniagara "SpawnRate" (`self.CurrentStepValue` (`self.SpawnRate`)))
      (`SceneComponent.SetHiddenInGame` (`self.ClueMesh`) (< (`self.CurrentStep`) (`self.GetTargetQuantityValue`)) false))))

(fn `ResetCharacterSpeedAndAnimation`
  (bind _defaultmaxspeed (`self.DefaultMaxSpeed`))
  (bind _keys (`BlueprintMapLibrary.Map_Keys` _defaultmaxspeed))
  (for _array_element _keys
    (set `CharacterMovementComponent.MaxWalkSpeed` (`BlueprintMapLibrary.Map_Find` _defaultmaxspeed _array_element) (`Character.CharacterMovement` _array_element))
    (bind _aspdwanim_instance (cast `PDWAnimInstance` (`SkeletalMeshComponent.GetAnimInstance` (`Character.Mesh` _array_element))))
    (`PDWAnimInstance.SetAnimationState` _aspdwanim_instance "Walking")))

(fn `SetCharacterSpeedAndAnimation`
  (params (Controllers :type "Array of PDWPlayerController Object Reference"))
  (for _array_element Controllers
    (bind _aspdwcharacter (cast `PDWCharacter` (`Controller.K2_GetPawn` _array_element)))
    (bind _charactermovement (`Character.CharacterMovement` _aspdwcharacter))
    (`BlueprintMapLibrary.Map_Add` (`self.DefaultMaxSpeed`) _aspdwcharacter (`CharacterMovementComponent.MaxWalkSpeed` _charactermovement))
    (set `CharacterMovementComponent.MaxWalkSpeed` (`self.SniffingWalkSpeed`) _charactermovement)
    (bind _aspdwanim_instance (cast `PDWAnimInstance` (`SkeletalMeshComponent.GetAnimInstance` (`Character.Mesh` _aspdwcharacter))))
    (`PDWAnimInstance.SetAnimationState` _aspdwanim_instance "Sniff")))

(fn `UserConstructionScript`
  (`parent.UserConstructionScript`))