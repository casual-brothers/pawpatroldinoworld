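; Vehicle claws minigame Blueprint that lights up one target actor at a time for the player to hit.
; On initialization it copies the configured targets, then on each success deactivates the current one and draws the next, in order or at random, without repeats.
; Activation shows Niagara effects and enables query collision on components tagged InteractableArea, skipping targets without a tagged box.
; Completion hides the effects on all targets.
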(event `self.PDWMinigameConfig.OnMinigameInitializationComplete`
  (params (Controllers :type "Array of PDWPlayerController Object Reference (by ref)"))
  (set `self.TempMinigameTargetActors` (`PDWMinigameConfigComponent.MinigameTargetActors` (`self.PDWMinigameConfig`)))
  (`self.ActivateNextTarget`))

(event `self.PDWMinigameConfig.OnMinigameComplete`
  (params (inSignature :type "MiniGameEventSignature Structure (by ref)"))
  (for _array_element (`PDWMinigameConfigComponent.MinigameTargetActors` (`self.PDWMinigameConfig`))
    (for _array_element_2 (`self.GetComponentsByTag` _array_element "/Script/Niagara.NiagaraComponent" "InteractableArea")
      (`SceneComponent.SetHiddenInGame` _array_element_2 true false))))

(event `self.PDWMinigameConfig.OnNotifySuccessFromMinigame`
  (params (inEvent :type "InteractionEventSignature Structure (by ref)"))
  (`self.DeactivateCurrentTarget`)
  (`self.ActivateNextTarget`))

(fn `ActivateNextTarget`
  (bind _currenttarget (`self.CurrentTarget`))
  (bind _tempminigametargetactors (`self.TempMinigameTargetActors`))
  (bind _returnvalue (`KismetArrayLibrary.Array_Length` _tempminigametargetactors))
  (bind _returnvalue_2 (`self.GetComponentsByTag` _currenttarget "/Script/Engine.BoxComponent" "InteractableArea"))
  (if (> _returnvalue 0)
    (if (not (`self.TargetsInOrder`))
      (set `self.CurrentIndex_0` (`KismetMathLibrary.RandomIntegerInRange` 0 (- _returnvalue 1))))
    (set `self.CurrentTarget` (`|GetArrayItem` _tempminigametargetactors (`self.CurrentIndex_0`)))
    (`KismetArrayLibrary.Array_Remove` (`self.TempMinigameTargetActors`) (`self.CurrentIndex_0`))
    (if (> (`KismetArrayLibrary.Array_Length` _returnvalue_2) 0)
      (for _array_element (`self.GetComponentsByTag` _currenttarget "/Script/Niagara.NiagaraComponent" "InteractableArea")
        (`SceneComponent.SetHiddenInGame` _array_element false false))
      (for _array_element_2 _returnvalue_2
        (`PrimitiveComponent.SetCollisionEnabled` _array_element_2 "QueryOnly"))
      (else
        (`self.ActivateNextTarget`)))))

(fn `DeactivateCurrentTarget`
  (bind _currenttarget (`self.CurrentTarget`))
  (bind _returnvalue (`self.GetComponentsByTag` _currenttarget "/Script/Engine.BoxComponent" "InteractableArea"))
  (`/Engine/EditorBlueprintResources/StandardMacros.IsValid` _currenttarget
    (:`Is Valid`
      (if (> (`KismetArrayLibrary.Array_Length` _returnvalue) 0)
        (for _array_element (`self.GetComponentsByTag` _currenttarget "/Script/Niagara.NiagaraComponent" "InteractableArea")
          (`SceneComponent.SetHiddenInGame` _array_element true false))
        (for _array_element_2 _returnvalue
          (`PrimitiveComponent.SetCollisionEnabled` _array_element_2 "NoCollision"))
        (else
          (`self.ActivateNextTarget`))))))

(fn `UserConstructionScript`
  (`parent.UserConstructionScript`))