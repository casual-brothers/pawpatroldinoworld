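; Water hose minigame that places stain targets on a Paleo Center dinosaur, apparently for cleaning.
; With a valid dino tag, parent BeginPlay waits until the matching dinosaur is found or loaded.
; Target initialization, rerun on multiplayer state changes, respawns randomized stain actors on distinct random prefix-filtered mesh sockets.
; The dinosaur mesh blocks GameTraceChannel6 once minigame initialization completes and ignores it on completion or leave.
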(event `self.ReceiveTick`
  (params (DeltaSeconds :type "Float (single-precision)"))
  (`parent.ReceiveTick` DeltaSeconds))

(event `self.ReceiveBeginPlay`
  (bind _returnvalue (subsystem `PDWPaleoCenterSubsystem`))
  (bind _paleodinotosync (`self.PaleoDinoToSync`))
  (if (`BlueprintGameplayTagLibrary.IsGameplayTagValid` _paleodinotosync)
    (bind _returnvalue_2 (`PDWPaleoCenterSubsystem.GetDinoActorRef` _returnvalue _paleodinotosync))
    (bind _asbp_npc_paleo_center_base (cast `/Game/Blueprints/Pawn/NPC/PaleoCenter/BP_NPC_PaleoCenter_Base` _returnvalue_2)
      (:`then`
        (set `self.DinosaurActor` _asbp_npc_paleo_center_base)
        (`parent.ReceiveBeginPlay`))
      (:`CastFailed`
        (add `PDWPaleoCenterSubsystem.OnDinoLoad` _returnvalue (delegate `OnDinoLoad`))))
    (else
      (`parent.ReceiveBeginPlay`))))

(event `OnDinoLoad`
  (params (DinoRef :type "Actor Object Reference"))
  (bind _returnvalue (`self.GetComponentByClass` DinoRef "/Script/PDW.PDWPaleoDinoComponent"))
  (`/Engine/EditorBlueprintResources/StandardMacros.IsValid` _returnvalue
    (:`Is Valid`
      (if (`BlueprintGameplayTagLibrary.MatchesTag` (`self.PaleoDinoToSync`) (`PDWPaleoDinoComponent.PenTag` _returnvalue) true)
        (bind _asbp_npc_paleo_center_base (cast `/Game/Blueprints/Pawn/NPC/PaleoCenter/BP_NPC_PaleoCenter_Base` DinoRef))
        (set `self.DinosaurActor` _asbp_npc_paleo_center_base)
        (`parent.ReceiveBeginPlay`)))))

(event `self.OnMultiplayerStateChange`
  (`parent.OnMultiplayerStateChange`)
  (`self.InitializeTargets`))

(event `self.PDWMinigameConfig.OnMinigameComplete`
  (params (inSignature :type "MiniGameEventSignature Structure (by ref)"))
  (bind _dinosauractor (`self.DinosaurActor`))
  (`/Engine/EditorBlueprintResources/StandardMacros.IsValid` _dinosauractor :!label _label
    (:`Is Valid`
      (`PrimitiveComponent.SetCollisionResponseToChannel` (`self.GetComponentByClass` _dinosauractor "/Script/Engine.SkeletalMeshComponent") "ECC_GameTraceChannel6" "ECR_Ignore"))))

(event `self.PDWMinigameConfig.OnMinigameLeft`
  (params (inSignature :type "MiniGameEventSignature Structure (by ref)"))
  (goto _label))

(event `self.PDWMinigameConfig.OnMinigameInitializationComplete`
  (params (Controllers :type "Array of PDWPlayerController Object Reference (by ref)"))
  (bind _dinosauractor (`self.DinosaurActor`))
  (`/Engine/EditorBlueprintResources/StandardMacros.IsValid` _dinosauractor
    (:`Is Valid`
      (`PrimitiveComponent.SetCollisionResponseToChannel` (`self.GetComponentByClass` _dinosauractor "/Script/Engine.SkeletalMeshComponent") "ECC_GameTraceChannel6" "ECR_Block"))))

(fn `ActivateTargets`)

(fn `CreateTargets`
  (bind _minigametargetactors (`PDWMinigameConfigComponent.MinigameTargetActors` (`self.PDWMinigameConfig`)))
  (for _array_element _minigametargetactors
    (`/Engine/EditorBlueprintResources/StandardMacros.IsValid` _array_element
      (:`Is Valid`
        (`self.K2_DestroyActor` _array_element))))
  (`KismetArrayLibrary.Array_Clear` _minigametargetactors)
  (for _ (range (`self.GetTargetQuantityValue`))
    (bind _output_get (set `self.CurrentIndex_0` (`KismetMathLibrary.RandomIntegerInRange` 0 (- (`KismetArrayLibrary.Array_Length` (`self.AvailableSocket`)) 1))))
    (bind _returnvalue (`|SpawnActorFromClass` (`self.WaterHose_Target_Class`) (`self.GetTransform` self) "Undefined" "MultiplyWithRoot" self null))
    (`/Game/Blueprints/Actors/MiniGames/WaterHose/BP_Minigame_WaterHose_Target.RandomizeStainDecal` _returnvalue)
    (`self.K2_AttachToComponent` _returnvalue (`self.DinosaurMesh`) (`|GetArrayItem` (`self.AvailableSocket`) _output_get) "SnapToTarget" "SnapToTarget" "SnapToTarget" true)
    (`KismetArrayLibrary.Array_AddUnique` (`PDWMinigameConfigComponent.MinigameTargetActors` (`self.PDWMinigameConfig`)) _returnvalue)
    (`KismetArrayLibrary.Array_Remove` (`self.AvailableSocket`) (`self.CurrentIndex_0`))))

(fn `GetSocketList`
  (`KismetArrayLibrary.Array_Clear` (`self.SocketList`))
  (for _index (range (`SkeletalMesh.NumSockets` (`SkeletalMeshComponent.SkeletalMeshAsset` (`self.DinosaurMesh`))))
    (bind _socketname (`SkeletalMeshSocket.SocketName` (`SkeletalMesh.GetSocketByIndex` (`SkeletalMeshComponent.SkeletalMeshAsset` (`self.DinosaurMesh`)) _index)))
    (if (`KismetStringLibrary.StartsWith` (`KismetStringLibrary.Conv_NameToString` _socketname) (`self.In Prefix`))
      (`KismetArrayLibrary.Array_Add` (`self.SocketList`) _socketname)))
  (set `self.AvailableSocket` (`self.SocketList`)))

(fn `InitializeTargets`
  (bind _dinosauractor (`self.DinosaurActor`))
  (`/Engine/EditorBlueprintResources/StandardMacros.IsValid` _dinosauractor
    (:`Is Valid`
      (bind _output_get (set `self.DinosaurMesh` (`self.GetComponentByClass` _dinosauractor "/Script/Engine.SkeletalMeshComponent")))
      (`/Engine/EditorBlueprintResources/StandardMacros.IsValid` _output_get
        (:`Is Valid`
          (`self.GetSocketList`)
          (`self.CreateTargets`))))))

(fn `UserConstructionScript`
  (`parent.UserConstructionScript`))